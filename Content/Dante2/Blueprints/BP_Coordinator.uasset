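; Coordinator actor that controls when and where the Ambassador enemy appears as the player dives between levels.
; On game start it indexes all room volumes, binds to the pawn's dive event and rolls a random Ambassador dive level.
; Each dive removes any existing Ambassador; level 0 rerolls, the chosen level spawns immediately, and others spawn after a timer.
; Spawns land on navmesh in a random room other than the player's, with dispatchers announcing spawn and removal.
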(event Custom|RemoveAmbassador
  ;[1 1 1] Remove Ambassador
  (Utilities|FlowControl|Delay 0.2)
  (Actor|DestroyActor (Variables|Default|GetAmbassadorReference))
  (Default|CallAmbassadorRemoved))

(event Custom|SpawnAmbassador
  ;[1 1 1] Spawn Ambassador
  (bind _output_get (Variables|Default|SetRoomsTemp (Variables|Default|GetRooms)))
  (Utilities|Array|RemoveIndex _output_get (Variables|/Game/Dante/Blueprint/BP_DantePawn.BP_DantePawn_C|GetCurrentRoom (Variables|Default|GetAs%20BP%20Dante%20Pawn)))
  (bind _randomlocation (Class|NavigationSystemV1|GetRandomLocationinNavigableRadius (Transformation|GetActorLocation (.OutItem (Utilities|Array|Random (Variables|Default|GetRoomsTemp)))) 1e+02 0 0))
  (bind _returnvalue (Game|SpawnActorfromClass "/Game/XanWorld/BP_BaseCharacter.BP_BaseCharacter_C" (Math|Transform|MakeTransform _randomlocation "0, 0, 0" "1.000000,1.000000,1.000000") "Undefined" "MultiplyWithRoot" 0 0))
  (bind _output_get_2 (Variables|Default|SetAmbassadorReference _returnvalue))
  (Variables|/Game/XanWorld/BP_BaseCharacter.BP_BaseCharacter_C|SetCoordinatorReference _output_get_2 self)
  (Default|InitializeBaseCharacter _output_get_2 "/Game/XanWorld/DataAssets/DA_DanteProtoEnemy_A.DA_DanteProtoEnemy_A")
  (Default|CallAmbassadorSpawned))

(event Custom|OnDive_Event
  (params (DiveLevel :type Integer))
  (bind _ambassadortimerhandle (Variables|Default|GetAmbassadorTimerHandle))
  ;[1 1 1] Player ref + OnDive event
  (if (Utilities|IsValid (Variables|Default|GetAmbassadorReference))
    (CallFunction|RemoveAmbassador))
  (if (Utilities|Time|IsValidTimerHandle _ambassadortimerhandle)
    (Utilities|Time|ClearandInvalidateTimerbyHandle _ambassadortimerhandle))
  (if (== DiveLevel 0)
    (CallFunction|SelectRandomDiveLevel)
    (elif (== DiveLevel (Variables|Default|GetAmbassadorDiveLevel))
      (CallFunction|SpawnAmbassador)
      (else
        (CallFunction|SpawnViaTimer)))))

(event Custom|SpawnViaTimer
  ;[1 1 1] Spawn via timer
  (bind _returnvalue (Utilities|Time|SetTimerbyEvent (delegate Custom|AmbassadorTimer) (Variables|Default|GetTimerBeforeSpawing)))
  (Variables|Default|SetAmbassadorTimerHandle _returnvalue))

(event Custom|AmbassadorTimer
  ;[1 1 1] Spawn via timer
  (Utilities|Time|ClearandInvalidateTimerbyHandle (Variables|Default|GetAmbassadorTimerHandle))
  (CallFunction|SpawnAmbassador))

(event Custom|SelectRandomDiveLevel
  ;[1 1 1] Select Starting Dive Level
  (Variables|Default|SetAmbassadorDiveLevel (Math|Random|RandomIntegerinRange 1 (Utilities|Array|LastIndex (Variables|/Game/Dante/Blueprint/BP_DanteGameMode.BP_DanteGameMode_C|GetLevels (Variables|Default|GetAs%20BP%20Dante%20Game%20Mode))))))

(event Custom|GameStarted_Event
  ;[1 1 1] GameMode Ref
  (Utilities|FlowControl|Sequence
    (:then_1
      ;[1 1 1] Rooms Ref
      (bind _outactors (Actor|GetAllActorsOfClass "/Game/Dante2/Blueprints/BP_RoomVolume.BP_RoomVolume_C"))
      (bind _output_get (Variables|Default|SetRooms _outactors))
      (for (_array_element _array_index) _output_get
        (Variables|/Game/Dante2/Blueprints/BP_RoomVolume.BP_RoomVolume_C|SetRoomIndex _array_element _array_index)))
    (:then_2
      ;[1 1 1] Player ref + OnDive event
      (bind _asbp_dante_pawn (Utilities|Casting|CastToBP_DantePawn (Game|Player|GetPlayerPawn 0)))
      (bind _output_get_2 (Variables|Default|SetAs%20BP%20Dante%20Pawn _asbp_dante_pawn))
      (EventDispatchers|AssignOnDive _output_get_2 (delegate Custom|OnDive_Event)))
    (:then_3
      ;[1 1 1] Select Starting Dive Level
      (Variables|Default|SetAmbassadorDiveLevel (Math|Random|RandomIntegerinRange 1 (Utilities|Array|LastIndex (Variables|/Game/Dante/Blueprint/BP_DanteGameMode.BP_DanteGameMode_C|GetLevels (Variables|Default|GetAs%20BP%20Dante%20Game%20Mode))))))))

(event Custom|DestroyAmbassador
  (Utilities|FlowControl|Delay 0.2)
  (Actor|DestroyActor (Variables|Default|GetAmbassadorReference))
  (Utilities|Time|ClearandInvalidateTimerbyHandle (Variables|Default|GetAmbassadorTimerHandle)))

(event EventBeginPlay
  ;[1 1 1] GameMode Ref
  (bind _asbp_dante_game_mode (Utilities|Casting|CastToBP_DanteGameMode (Game|GetGameMode)))
  (bind _output_get (Variables|Default|SetAs%20BP%20Dante%20Game%20Mode _asbp_dante_game_mode))
  (EventDispatchers|AssignGameStarted _output_get (delegate Custom|GameStarted_Event)))

(event EventTick
  (params (DeltaSeconds :type Float%20%28single-precision%29)))

(fn ConstructionScript)