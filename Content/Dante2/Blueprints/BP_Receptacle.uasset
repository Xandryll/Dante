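; BP_Receptacle is an actor with three switchable features: a Tracker, a Finder and a FlameShield, each shown or hidden by an activation event.
; Looping timers drive dynamic material parameters from clamped distance mappings.
; The Tracker reflects Ambassador-to-Coordinator proximity, starting and stopping on the Coordinator's spawn and removal events.
; While active, the Finder reflects the receptacle's proximity to the nearest clue in the game mode's CluesList.
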(event Custom|GetClosestClue
  (bind _as_bp_dante_game_mode (Variables|Default|GetAs%20BP%20Dante%20Game%20Mode))
  (bind _clueslist (Variables|/Game/Dante/Blueprint/BP_DanteGameMode.BP_DanteGameMode_C|GetCluesList _as_bp_dante_game_mode))
  (Variables|Default|SetClosestClueTemp (Utilities|Array|Get(acopy) _clueslist))
  (for _index (range 1 (Utilities|Array|LastIndex _clueslist))
    (if (< (Math|Vector|Distance(Vector) (Transformation|GetActorLocation (Utilities|Array|Get(acopy) _clueslist _index)) (Transformation|GetActorLocation)) (Math|Vector|Distance(Vector) (Transformation|GetActorLocation (Variables|Default|GetClosestClueTemp)) (Transformation|GetActorLocation)))
      (Variables|Default|SetClosestClueTemp (Utilities|Array|Get(acopy) _clueslist _index))))
  (Variables|Default|SetClosestClue (Variables|Default|GetClosestClueTemp))
  (Variables|Default|SetClosestClueTemp 0))

(event Custom|AmbassadorRemoved_Event
  (Rendering|Material|SetScalarParameterValue (Variables|Default|GetTrackerMaterial) "Tracker_Activation" 1.0 :!class /Script/Engine.MaterialInstanceDynamic)
  (Utilities|Time|ClearandInvalidateTimerbyHandle (Variables|Default|GetTrackerTimerHandle)))

(event Custom|FinderTimer
  (CallFunction|GetClosestClue)
  (Rendering|Material|SetScalarParameterValue (Variables|Default|GetFinderMaterial) "Finder_Transition" (Math|Float|MapRangeClamped (Math|Vector|Distance(Vector) (Transformation|GetActorLocation (Variables|Default|GetClosestClue)) (Transformation|GetActorLocation)) 1.5e+03 2e+02 0.0 1.0) :!class /Script/Engine.MaterialInstanceDynamic))

(event Custom|AmbassadorSpawned_Event
  (Rendering|Material|SetScalarParameterValue (Variables|Default|GetTrackerMaterial) "Tracker_Activation" 0.0 :!class /Script/Engine.MaterialInstanceDynamic)
  (bind _returnvalue (Utilities|Time|SetTimerbyEvent (delegate Custom|TrackerTimer) 0.1 true))
  (Variables|Default|SetTrackerTimerHandle _returnvalue))

(event Custom|TrackerTimer
  (bind _coordinatorreference (Variables|Default|GetCoordinatorReference))
  (bind _returnvalue (Transformation|GetActorLocation _coordinatorreference))
  (bind _ambassadorreference (Variables|/Game/Dante2/Blueprints/BP_Coordinator.BP_Coordinator_C|GetAmbassadorReference _coordinatorreference))
  (bind _returnvalue_2 (Transformation|GetActorLocation _ambassadorreference))
  (bind _returnvalue_3 (Math|Vector|Distance(Vector) _returnvalue_2 _returnvalue))
  (Rendering|Material|SetScalarParameterValue (Variables|Default|GetTrackerMaterial) "Tracker_Transition" (Math|Float|SelectFloat 0.0 (Math|Float|MapRangeClamped _returnvalue_3 5e+03 1.5e+03 0.0 1.0) (> _returnvalue_3 5e+03)) :!class /Script/Engine.MaterialInstanceDynamic))

(event Custom|ActivateShield
  (params (IsActive :type Boolean))
  (Development|SetHiddeninGame (Variables|Default|GetFlameShield) (not IsActive) false)
  (Variables|Default|SetActiveShield IsActive))

(event Custom|ActivateTracker
  (params (IsActive :type Boolean))
  (Development|SetHiddeninGame (Variables|Default|GetTracker) (not IsActive) false)
  (Variables|Default|SetActiveTracker IsActive))

(event Custom|ActivateFinder
  (params (IsActive :type Boolean))
  (Development|SetHiddeninGame (Variables|Default|GetFinder) (not IsActive) false)
  (bind _output_get (Variables|Default|SetActiveFinder IsActive))
  (if _output_get
    (bind _returnvalue (Utilities|Time|SetTimerbyEvent (delegate Custom|FinderTimer) 1.0 true))
    (Variables|Default|SetFinderTimerHandle _returnvalue)
    (else
      (Utilities|Time|ClearandInvalidateTimerbyHandle (Variables|Default|GetFinderTimerHandle)))))

(event EventBeginPlay
  (bind _tracker (Variables|Default|GetTracker))
  (bind _finder (Variables|Default|GetFinder))
  (Utilities|FlowControl|Sequence
    (:then_0
      (bind _returnvalue (Rendering|Material|CreateDynamicMaterialInstance _tracker 0 "/Game/Dante2/M_Tracker_Inst.M_Tracker_Inst" "None" :!class /Script/Engine.PrimitiveComponent))
      (bind _output_get (Variables|Default|SetTrackerMaterial _returnvalue))
      (Rendering|Material|SetMaterial _tracker 0 _output_get)
      (Rendering|Material|SetScalarParameterValue _returnvalue "Tracker_Transition" 0.0 :!class /Script/Engine.MaterialInstanceDynamic)
      (Rendering|Material|SetScalarParameterValue _returnvalue "Tracker_Activation" 1.0 :!class /Script/Engine.MaterialInstanceDynamic))
    (:then_1
      (bind _returnvalue_2 (Rendering|Material|CreateDynamicMaterialInstance _finder 0 "/Game/Dante2/M_Finder_Inst.M_Finder_Inst" "None" :!class /Script/Engine.PrimitiveComponent))
      (bind _output_get_2 (Variables|Default|SetFinderMaterial _returnvalue_2))
      (Rendering|Material|SetMaterial _finder 0 _output_get_2)
      (Rendering|Material|SetScalarParameterValue _output_get_2 "Finder_Transition" 0.0 :!class /Script/Engine.MaterialInstanceDynamic))
    (:then_2
      (bind _outactors (Actor|GetAllActorsOfClass "/Game/Dante2/Blueprints/BP_Coordinator.BP_Coordinator_C"))
      (Variables|Default|SetCoordinatorReference (Utilities|Array|Get(acopy) _outactors))
      (EventDispatchers|AssignAmbassadorRemoved (Variables|Default|GetCoordinatorReference) (delegate Custom|AmbassadorRemoved_Event))
      (EventDispatchers|AssignAmbassadorSpawned (Variables|Default|GetCoordinatorReference) (delegate Custom|AmbassadorSpawned_Event))
      (bind _asbp_dante_game_mode (Utilities|Casting|CastToBP_DanteGameMode (Game|GetGameMode)))
      (Variables|Default|SetAs%20BP%20Dante%20Game%20Mode _asbp_dante_game_mode))))

(event Collision|EventActorBeginOverlap
  (params (OtherActor :type Actor%20Object%20Reference)))

(fn ConstructionScript)