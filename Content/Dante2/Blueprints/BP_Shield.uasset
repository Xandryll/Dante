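; BP_Shield is a shield item actor that can be detached from its holder and dropped into the world.
; On BeginPlay it enters a default state with a query-only Box and a mesh without collision or physics.
; ReleaseItem detaches it, unhides the mesh and lets it simulate physics, then restores that state after a short delay.
; Interact is empty, and a chain that would hide and disable the item is left unconnected.
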(event Custom|DefaultState
  (bind _staticmesh (Variables|Default|GetStaticMesh))
  (Collision|SetCollisionEnabled (Variables|Default|GetBox) "QueryOnly")
  (Collision|SetCollisionEnabled _staticmesh "NoCollision")
  (Physics|SetSimulatePhysics _staticmesh false))

(event EventBeginPlay
  (|CallParentFunction)
  (CallFunction|DefaultState))

(event Collision|EventActorBeginOverlap
  (params (OtherActor :type Actor%20Object%20Reference))
  (|CallParentFunction OtherActor) ; This node is disabled and will not be called.\nDrag off pins to build functionality.
)

(event EventTick
  (params (DeltaSeconds :type Float%20%28single-precision%29))
  (|CallParentFunction DeltaSeconds) ; This node is disabled and will not be called.\nDrag off pins to build functionality.
)

(event EventInteract)

(event EventReleaseItem
  (bind _staticmesh (Variables|Default|GetStaticMesh))
  (Transformation|DetachFromActor "KeepWorld" "KeepWorld" "KeepWorld")
  (Development|SetHiddeninGame _staticmesh false false)
  (Collision|SetCollisionEnabled _staticmesh "QueryAndPhysics")
  (Physics|SetSimulatePhysics _staticmesh true)
  (Utilities|FlowControl|Delay 2.0)
  (CallFunction|DefaultState))

(fn ConstructionScript
  (|CallParentFunction))