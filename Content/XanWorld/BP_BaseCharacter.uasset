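; Base AI enemy character that copies patrol, investigation, attack and movement tuning from a data asset, then starts its StateTree.
; AI perception tracks seen player pawns and closets, setting a target location for sighted or heard actors.
; Non-sight stimuli, or losing the player unless seen hiding, start timed investigation.
; A line-of-sight check on the player's hide event records the witnessed hiding spot, and taunts use a timed cooldown.
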(event OnTargetPerceptionUpdated(AIPerception)
  (params (Actor :type Actor%20Object%20Reference) (Stimulus :type AI%20Stimulus%20Structure))
  (bind _bsuccessfullysensed (Utilities|Struct|BreakAIStimulus Stimulus))
  (bind _returnvalue (Utilities|GetClass Actor))
  (bind _seenhidingspots (Variables|Perception|GetSeenHidingSpots))
  (bind _taunttimerhandle (Variables|Attack|GetTauntTimerHandle))
  (bind _seenactors (Variables|Perception|GetSeenActors))
  (bind _heardactors (Variables|Perception|GetHeardActors))
  ;[1 1 1] PerceptionSystem
  (bind _returnvalue_2 (Class|AIPerceptionSystem|GetSenseClassforStimulus Stimulus))
  (if (== _returnvalue_2 "/Script/AIModule.AISense_Sight")
    (if (or (== _returnvalue "/Game/Dante/Blueprint/BP_DantePawn.BP_DantePawn_C") (== _returnvalue "/Game/XanWorld/HideNSeek/BP_HideNSeekPAwn.BP_HideNSeekPAwn_C"))
      (if _bsuccessfullysensed
        (if (Utilities|Time|IsValidTimerHandle _taunttimerhandle)
          (Utilities|Time|ClearandInvalidateTimerbyHandle _taunttimerhandle)
          (CallFunction|PerformTaunt))
        (Utilities|Array|AddUnique _seenactors Actor)
        (Variables|Perception|SetTargetLocation (Transformation|GetActorLocation (Utilities|Array|Get(acopy) _seenactors)))
        (elif (Variables|Perception|GetSeenBeforeHide)
          (Utilities|Array|RemoveItem _seenactors Actor)
          (else
            (Utilities|Array|RemoveItem _seenactors Actor)
            (Utilities|Array|AddUnique _heardactors Actor :!label _label)
            (Variables|Perception|SetTargetLocation (Transformation|GetActorLocation (Utilities|Array|Get(acopy) _heardactors)))
            (if (Utilities|Time|IsValidTimerHandle (Variables|Perception|GetPerceptionTimerHandle))
              (Utilities|Time|ClearandInvalidateTimerbyHandle (Variables|Perception|GetPerceptionTimerHandle)))
            (bind _returnvalue_3 (Utilities|Time|SetTimerbyEvent (delegate Custom|StopInvestigating) (Variables|Investigation|GetInvestigation_TimeBeforeResumePatrol)))
            (Variables|Perception|SetPerceptionTimerHandle _returnvalue_3))))
      (elif (== _returnvalue "/Game/Dante/Blueprint/Items/BP_HidingCloset.BP_HidingCloset_C")
        (if _bsuccessfullysensed
          (Utilities|Array|AddUnique _seenhidingspots Actor)
          (else
            (Utilities|Array|RemoveItem _seenhidingspots Actor)))))
    (else
      (goto _label))))

(event Custom|InitializeBaseCharacter
  (params (DA%20to%20Spawn :type PDA%20X%20Enemy%20Object%20Reference))
  ;[1 1 1] Initialize
  (bind _output_get (Variables|Default|SetDA DA%20to%20Spawn))
  (Variables|Patrol|SetPatrol_ChangeRouteAfterComplete (.patrol_changerouteaftercomplete (Variables|/Game/XanWorld/DataAssets/PDA_xEnemy.PDA_xEnemy_C|GetxEnemyConfiguration _output_get)))
  (Variables|Patrol|SetPatrol_RouteRepetition (.patrol_routerepetition (Variables|/Game/XanWorld/DataAssets/PDA_xEnemy.PDA_xEnemy_C|GetxEnemyConfiguration _output_get)))
  (Variables|Patrol|SetPatrol_WaypointWaitTime (.patrol_waypointwaittime (Variables|/Game/XanWorld/DataAssets/PDA_xEnemy.PDA_xEnemy_C|GetxEnemyConfiguration _output_get)))
  (Variables|Investigation|SetInvestigation_TimeBeforeResumePatrol (.investigation_timebeforeresumepatrol (Variables|/Game/XanWorld/DataAssets/PDA_xEnemy.PDA_xEnemy_C|GetxEnemyConfiguration _output_get)))
  (Variables|Investigation|SetInvestigation_HidingSpotChance (.investigation_hidingspotchance (Variables|/Game/XanWorld/DataAssets/PDA_xEnemy.PDA_xEnemy_C|GetxEnemyConfiguration _output_get)))
  (Variables|Investigation|SetInvestigation_WaypointWaitTime (.investigation_waypointwaittime (Variables|/Game/XanWorld/DataAssets/PDA_xEnemy.PDA_xEnemy_C|GetxEnemyConfiguration _output_get)))
  (Variables|Attack|SetAttack_TimeBetweenAttacks (.attack_timebetweenattacks (Variables|/Game/XanWorld/DataAssets/PDA_xEnemy.PDA_xEnemy_C|GetxEnemyConfiguration _output_get)))
  (bind _output_get_2 (Variables|Movement|SetMovement_Speed (.movement_speed (Variables|/Game/XanWorld/DataAssets/PDA_xEnemy.PDA_xEnemy_C|GetxEnemyConfiguration _output_get))))
  (Variables|/Script/Engine.CharacterMovementComponent|SetMaxWalkSpeed (Variables|Character|GetCharacterMovement) _output_get_2)
  (Variables|Default|SetRoomsToExploreBeforeDiving 10)
  (bind _asbp_dante_pawn (Utilities|Casting|CastToBP_DantePawn (Game|Player|GetPlayerPawn 0)))
  (bind _output_get_3 (Variables|References|SetPlayerReference _asbp_dante_pawn))
  (EventDispatchers|BindEventtoOnHide _output_get_3 (delegate Custom|CheckLOSBeforeHide))
  (AI|Logic|StartLogic (Variables|Default|GetStateTree)))

(event Custom|CheckLOSBeforeHide
  (bind _playerreference (Variables|References|GetPlayerReference))
  (bind _currenthidingspot (Variables|/Game/Dante/Blueprint/BP_DantePawn.BP_DantePawn_C|GetCurrentHidingSpot _playerreference))
  ;[1 1 1] Check LOS event
  (bind _output_get (Variables|Perception|SetSeenBeforeHide (Controller|LineOfSightTo (AI|GetAIController self) _playerreference "0, 0, 0" false)))
  (if _output_get
    (Variables|Perception|SetTargetHidingSpot (Transformation|GetWorldLocation (Variables|/Game/Dante/Blueprint/Items/BP_HidingCloset.BP_HidingCloset_C|GetExitDirection _currenthidingspot)))
    (Variables|Perception|SetTargetHidingSpotRef _currenthidingspot)))

(event Custom|StopInvestigating
  ;[1 1 1] PerceptionSystem
  (Utilities|Array|Clear (Variables|Perception|GetHeardActors))
  (Variables|Perception|SetTargetLocation "0, 0, 0"))

(event Custom|PerformTaunt
  ;[1 1 1] Taunt
  (Variables|Attack|SetTauntPerformedRecently true)
  (bind _returnvalue (Utilities|Time|SetTimerbyEvent (delegate Custom|ReleaseTaunt) 1e+01))
  (Variables|Attack|SetTauntTimerHandle _returnvalue))

(event Custom|ReleaseTaunt
  ;[1 1 1] Taunt
  (Utilities|Time|ClearandInvalidateTimerbyHandle (Variables|Attack|GetTauntTimerHandle))
  (Variables|Attack|SetTauntPerformedRecently false))

(fn ConstructionScript)