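; Corridor actor that secretly rotates and shifts around the player, toggling between its start transform and a 90-degree turned, offset one.
; Side triggers shut any open linked smart door, then PawnPivot records the player's transform, so the pawn is repositioned to match the moved corridor.
; Each flip swaps which door is locked, while exit triggers re-arm the side triggers through collision toggles.
; TriggerDoor slowly creaks the side A door open.
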(event OnComponentBeginOverlap(SideA_Trigger)
  (params (OverlappedComponent :type Primitive%20Component%20Object%20Reference) (OtherActor :type Actor%20Object%20Reference) (OtherComp :type Primitive%20Component%20Object%20Reference) (OtherBodyIndex :type Integer) (bFromSweep :type Boolean) (SweepResult :type Hit%20Result%20Structure%20%28by%20ref%29))
  (bind _sidea_bpdoor (Variables|Default|GetSideA_BPDoor))
  (if (== (Utilities|GetClass OtherActor) "/Game/Dante/Blueprint/BP_DantePawn.BP_DantePawn_C")
    (if (Variables|/Game/Dante/Blueprint/Items/BP_Door.BP_Door_C|GetDoorOpen _sidea_bpdoor)
      (Default|ForceChangeState _sidea_bpdoor false 1.0 true "/Game/Dante/Audio/closedoor.closedoor"))
    (CallFunction|RotateCorridor)))

(event OnComponentBeginOverlap(SideB_Trigger)
  (params (OverlappedComponent :type Primitive%20Component%20Object%20Reference) (OtherActor :type Actor%20Object%20Reference) (OtherComp :type Primitive%20Component%20Object%20Reference) (OtherBodyIndex :type Integer) (bFromSweep :type Boolean) (SweepResult :type Hit%20Result%20Structure%20%28by%20ref%29))
  (bind _sideb_bpdoor (Variables|Default|GetSideB_BPDoor))
  (if (== (Utilities|GetClass OtherActor) "/Game/Dante/Blueprint/BP_DantePawn.BP_DantePawn_C")
    (if (Variables|/Game/Dante/Blueprint/Items/BP_Door.BP_Door_C|GetDoorOpen _sideb_bpdoor)
      (Default|ForceChangeState _sideb_bpdoor false 1.0 true "/Game/Dante/Audio/closedoor.closedoor"))
    (CallFunction|RotateCorridor)))

(event OnComponentBeginOverlap(SideB_TriggerExit)
  (params (OverlappedComponent :type Primitive%20Component%20Object%20Reference) (OtherActor :type Actor%20Object%20Reference) (OtherComp :type Primitive%20Component%20Object%20Reference) (OtherBodyIndex :type Integer) (bFromSweep :type Boolean) (SweepResult :type Hit%20Result%20Structure%20%28by%20ref%29))
  (Collision|SetCollisionEnabled (Variables|Default|GetSideB_Trigger) "QueryOnly")
  (Collision|SetCollisionEnabled (Variables|Default|GetSideA_TriggerExit) "QueryOnly")
  (Collision|SetCollisionEnabled (Variables|Default|GetSideB_TriggerExit) "NoCollision"))

(event OnComponentBeginOverlap(SideA_TriggerExit)
  (params (OverlappedComponent :type Primitive%20Component%20Object%20Reference) (OtherActor :type Actor%20Object%20Reference) (OtherComp :type Primitive%20Component%20Object%20Reference) (OtherBodyIndex :type Integer) (bFromSweep :type Boolean) (SweepResult :type Hit%20Result%20Structure%20%28by%20ref%29))
  (Collision|SetCollisionEnabled (Variables|Default|GetSideA_Trigger) "QueryOnly")
  (Collision|SetCollisionEnabled (Variables|Default|GetSideB_TriggerExit) "QueryOnly")
  (Collision|SetCollisionEnabled (Variables|Default|GetSideA_TriggerExit) "NoCollision"))

(event Custom|RotateCorridor
  (bind _returnvalue (Game|Player|GetPlayerPawn 0))
  (bind _returnvalue_2 (Game|GetPlayerController 0))
  (bind _returnvalue_3 (Game|Player|GetPlayerPawn 0))
  (bind _starttransform (Variables|Default|GetStartTransform))
  (bind _pawnpivot (Variables|Default|GetPawnPivot))
  (bind _returnvalue_4 (Transformation|GetActorLocation _returnvalue))
  (bind _returnvalue_5 (Transformation|GetWorldTransform _pawnpivot))
  (Transformation|SetWorldTransform (Variables|Default|GetPawnPivot) (Transformation|GetActorTransform _returnvalue_3) false false)
  (if (Variables|Default|GetNormalState)
    (Variables|Default|SetNormalState false)
    (Collision|SetCollisionEnabled (Variables|Default|GetSideA_Trigger) "NoCollision")
    (Collision|SetCollisionEnabled (Variables|Default|GetSideB_TriggerExit) "QueryOnly")
    (Input|DisableInput _returnvalue_3 _returnvalue_2)
    (Utilities|FlowControl|Sequence
      (:then_0
        (Transformation|SetActorTransform (Math|Transform|MakeTransform (.location _starttransform) (Math|Rotator|CombineRotators (.rotation _starttransform) "0.000000,-90.000000,0.000000") (.scale _starttransform)))
        (Transformation|AddActorLocalOffset "0.000000,400.000000,0.000000" false false))
      (:then_1
        (Transformation|SetActorTransform _returnvalue (Math|Transform|MakeTransform (Math|Vector|MakeVector (.x (.location _returnvalue_5)) (.y (.location _returnvalue_5)) (.z _returnvalue_4)) (.rotation _returnvalue_5) "1.000000,1.000000,1.000000"))
        (Input|EnableInput _returnvalue_3 _returnvalue_2)
        (Variables|/Game/Dante/Blueprint/Items/BP_Door.BP_Door_C|SetLocked (Variables|Default|GetSideA_BPDoor) true)
        (Variables|/Game/Dante/Blueprint/Items/BP_Door.BP_Door_C|SetLocked (Variables|Default|GetSideB_BPDoor) false)))
    (else
      (Variables|Default|SetNormalState true)
      (Collision|SetCollisionEnabled (Variables|Default|GetSideB_Trigger) "NoCollision")
      (Collision|SetCollisionEnabled (Variables|Default|GetSideA_TriggerExit) "QueryOnly")
      (Input|DisableInput _returnvalue_2)
      (Transformation|SetActorTransform (Variables|Default|GetStartTransform))
      (Transformation|SetActorTransform _returnvalue (Math|Transform|MakeTransform (Math|Vector|MakeVector (.x (.location _returnvalue_5)) (.y (.location _returnvalue_5)) (.z _returnvalue_4)) (.rotation _returnvalue_5) "1.000000,1.000000,1.000000"))
      (Input|EnableInput _returnvalue_3 _returnvalue_2)
      (Variables|/Game/Dante/Blueprint/Items/BP_Door.BP_Door_C|SetLocked (Variables|Default|GetSideA_BPDoor) false)
      (Variables|/Game/Dante/Blueprint/Items/BP_Door.BP_Door_C|SetLocked (Variables|Default|GetSideB_BPDoor) true))))

(event Custom|TriggerDoor
  (Default|ForceChangeState (Variables|Default|GetSideA_BPDoor) true 0.3 true "/Game/Dante/Blueprint/Audio/wooden-door-creaking.wooden-door-creaking"))

(event EventBeginPlay
  (Variables|Default|SetStartTransform (Transformation|GetActorTransform))
  (bind _asbp_smart_link_door (Utilities|Casting|CastToBP_SmartLink_Door (Variables|/Script/Engine.ChildActorComponent|GetChildActor (Variables|Default|GetSideA_Door))))
  (Variables|Default|SetSideA_BPDoor (Variables|/Game/Dante/Blueprint/Items/BP_SmartLink_Door.BP_SmartLink_Door_C|GetAs%20BP%20Door _asbp_smart_link_door))
  (bind _asbp_smart_link_door_2 (Utilities|Casting|CastToBP_SmartLink_Door (Variables|/Script/Engine.ChildActorComponent|GetChildActor (Variables|Default|GetSideB_Door))))
  (Variables|Default|SetSideB_BPDoor (Variables|/Game/Dante/Blueprint/Items/BP_SmartLink_Door.BP_SmartLink_Door_C|GetAs%20BP%20Door _asbp_smart_link_door_2)))

(fn ConstructionScript)