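; BP_Log is an interactable log prop that starts with a noise-animated dynamic material and reacts to being uncovered and looked at.
; RemoveCover destroys the cover, reveals the log with a sound, then binds visibility and query collision to the game mode's dive level 1.
; The first LookatObject while the pawn is aiming stops the noise animation, fades its scale to zero and fires a Narrator event.
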(event Custom|ChangeLevel
  (bind _as_bp_dante_game_mode (Variables|Default|GetAs%20BP%20Dante%20Game%20Mode))
  (bind _dive_level (Variables|/Game/Dante/Blueprint/BP_DanteGameMode.BP_DanteGameMode_C|GetDive_Level _as_bp_dante_game_mode))
  (bind _returnvalue (== _dive_level 1))
  (Rendering|SetVisibility (Variables|Default|GetLog) _returnvalue false)
  (Collision|SetCollisionEnabled (Variables|Default|GetBox) (select _returnvalue "QueryOnly" "NoCollision")))

(event Custom|RemoveCover
  (Components|DestroyComponent (Variables|Default|GetCover))
  (Rendering|SetVisibility (Variables|Default|GetLog) true false)
  (Collision|SetCollisionEnabled (Variables|Default|GetBox) "QueryOnly")
  (EventDispatchers|BindEventtoDiveChangeLevel (Variables|Default|GetAs%20BP%20Dante%20Game%20Mode) (delegate Custom|ChangeLevel))
  (Audio|PlaySoundatLocation "/Game/Dante/Audio/clothes-drop-2.clothes-drop-2" (Transformation|GetWorldLocation (Variables|Default|GetLog)) "0, 0, 0" 1.0 1.0 0.0 0 0 0 0))

(event EventBeginPlay
  (bind _log (Variables|Default|GetLog))
  (bind _asbp_dante_game_mode (Utilities|Casting|CastToBP_DanteGameMode (Game|GetGameMode)))
  (Variables|Default|SetAs%20BP%20Dante%20Game%20Mode _asbp_dante_game_mode)
  (bind _returnvalue (Rendering|Material|CreateDynamicMaterialInstance _log 0 "/Game/XanWorld/ProtoType/Proxy/MI_Log.MI_Log" "None" :!class /Script/Engine.PrimitiveComponent))
  (Rendering|Material|SetMaterial _log 0 _returnvalue)
  (Variables|Default|SetMI _returnvalue)
  (Rendering|Material|SetScalarParameterValue (Variables|Default|GetMI) "Scale" (Variables|Default|GetNoiseScale) :!class /Script/Engine.MaterialInstanceDynamic)
  (bind _newtrack_0 (Timeline|Timeline PlayFromStart)
    (:Update
      (Rendering|Material|SetScalarParameterValue (Variables|Default|GetMI) "Noise" _newtrack_0 :!class /Script/Engine.MaterialInstanceDynamic))))

(event Collision|EventActorBeginOverlap
  (params (OtherActor :type Actor%20Object%20Reference)))

(event EventTick
  (params (DeltaSeconds :type Float%20%28single-precision%29)))

(event EventLookatObject
  (if (Variables|/Game/Dante/Blueprint/BP_DantePawn.BP_DantePawn_C|GetAiming (Variables|/Game/Dante/Blueprint/BP_DanteGameMode.BP_DanteGameMode_C|GetAs%20BP%20Dante%20Pawn (Variables|Default|GetAs%20BP%20Dante%20Game%20Mode)))
    (if (not (Variables|Default|GetTriggered))
      (Variables|Default|SetTriggered true)
      (Utilities|FlowControl|Sequence
        (:then_0
          (bind _newtrack_0 (Timeline|Timeline Stop)
            (:Update
              (Rendering|Material|SetScalarParameterValue (Variables|Default|GetMI) "Noise" _newtrack_0 :!class /Script/Engine.MaterialInstanceDynamic))))
        (:then_1
          (bind _newtrack_0_2 (Timeline|Timeline_0 PlayFromStart)
            (:Update
              (Rendering|Material|SetScalarParameterValue (Variables|Default|GetMI) "Scale" (Math|Float|Lerp (Variables|Default|GetNoiseScale) 0.0 _newtrack_0_2) :!class /Script/Engine.MaterialInstanceDynamic))
            (:Finished
              (Development|PrintString "Hello"))))
        (:then_2
          (Default|TriggerEvent (Variables|/Game/Dante/Blueprint/BP_DanteGameMode.BP_DanteGameMode_C|GetNarrator (Variables|Default|GetAs%20BP%20Dante%20Game%20Mode)) 2))))))

(fn ConstructionScript)