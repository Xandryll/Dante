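; BP_TriggerAreas is a level trigger that fires event 0 on a referenced narrator once BP_DantePawn has visited three areas or a fallback timer runs out.
; Each of three box overlaps sets its own area flag, and when all three are set the timer is cleared.
; Both paths then trigger the narrator and disable collision on all three boxes so overlaps stop.
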(event OnComponentBeginOverlap(Box)
  (params (OverlappedComponent :type Primitive%20Component%20Object%20Reference) (OtherActor :type Actor%20Object%20Reference) (OtherComp :type Primitive%20Component%20Object%20Reference) (OtherBodyIndex :type Integer) (bFromSweep :type Boolean) (SweepResult :type Hit%20Result%20Structure%20%28by%20ref%29))
  (if (== (Utilities|GetClass OtherActor) "/Game/Dante/Blueprint/BP_DantePawn.BP_DantePawn_C")
    (Variables|Default|SetArea0 true)
    (if (Math|Boolean|ANDBoolean (Variables|Default|GetArea0) (Variables|Default|GetArea1) (Variables|Default|GetArea2))
      (Utilities|Time|ClearandInvalidateTimerbyHandle (Variables|Default|GetTimerHandle))
      (Default|TriggerEvent (Variables|Default|GetNarratorReference))
      (Collision|SetCollisionEnabled (Variables|Default|GetBox1) "NoCollision"))))

(event OnComponentBeginOverlap(Box1)
  (params (OverlappedComponent :type Primitive%20Component%20Object%20Reference) (OtherActor :type Actor%20Object%20Reference) (OtherComp :type Primitive%20Component%20Object%20Reference) (OtherBodyIndex :type Integer) (bFromSweep :type Boolean) (SweepResult :type Hit%20Result%20Structure%20%28by%20ref%29))
  (if (== (Utilities|GetClass OtherActor) "/Game/Dante/Blueprint/BP_DantePawn.BP_DantePawn_C")
    (Variables|Default|SetArea1 true)
    (if (Math|Boolean|ANDBoolean (Variables|Default|GetArea0) (Variables|Default|GetArea1) (Variables|Default|GetArea2))
      (Utilities|Time|ClearandInvalidateTimerbyHandle (Variables|Default|GetTimerHandle))
      (Default|TriggerEvent (Variables|Default|GetNarratorReference))
      (Collision|SetCollisionEnabled (Variables|Default|GetBox1) "NoCollision"))))

(event OnComponentBeginOverlap(Box2)
  (params (OverlappedComponent :type Primitive%20Component%20Object%20Reference) (OtherActor :type Actor%20Object%20Reference) (OtherComp :type Primitive%20Component%20Object%20Reference) (OtherBodyIndex :type Integer) (bFromSweep :type Boolean) (SweepResult :type Hit%20Result%20Structure%20%28by%20ref%29))
  (if (== (Utilities|GetClass OtherActor) "/Game/Dante/Blueprint/BP_DantePawn.BP_DantePawn_C")
    (Variables|Default|SetArea2 true)
    (if (Math|Boolean|ANDBoolean (Variables|Default|GetArea0) (Variables|Default|GetArea1) (Variables|Default|GetArea2))
      (Utilities|Time|ClearandInvalidateTimerbyHandle (Variables|Default|GetTimerHandle))
      (Default|TriggerEvent (Variables|Default|GetNarratorReference))
      (Collision|SetCollisionEnabled (Variables|Default|GetBox1) "NoCollision"))))

(event Custom|TimerTrigger
  (Default|TriggerEvent (Variables|Default|GetNarratorReference))
  (Collision|SetCollisionEnabled (Variables|Default|GetBox1) "NoCollision"))

(event EventBeginPlay
  (bind _returnvalue (Utilities|Time|SetTimerbyEvent (delegate Custom|TimerTrigger) (Variables|Default|GetFallbackTimerDuration)))
  (Variables|Default|SetTimerHandle _returnvalue))

(event Collision|EventActorBeginOverlap
  (params (OtherActor :type Actor%20Object%20Reference)))

(event EventTick
  (params (DeltaSeconds :type Float%20%28single-precision%29)))

(fn ConstructionScript)