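; BP_CircleAreas is a prototype actor that picks player, circle and enemy locations among five area components: a center and four diagonal corners.
; BeginPlay gathers the components, and Checkdistances appends each one's distance to the player pawn into an array.
; The nearest index becomes PlayerLocation and the farthest CircleLocation.
; Both indices are removed sequentially from AvailableLocations, and EnemyLocation is drawn randomly from the remainder.
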(event Custom|Check%20distances
  (bind _distances (Variables|Default|GetDistances))
  (bind _availablelocations (Variables|Default|GetAvailableLocations))
  (for _array_element (Variables|Default|GetComponents)
    (Utilities|Array|Add _distances (Math|Vector|Distance(Vector) (Transformation|GetWorldLocation _array_element) (Transformation|GetActorLocation (Game|Player|GetPlayerPawn 0)))))
  (bind _output_get (Variables|Default|SetPlayerLocation (.IndexOfMinValue (Math|Float|MinOfFloatArray _distances))))
  (bind _output_get_2 (Variables|Default|SetCircleLocation (.IndexOfMaxValue (Math|Float|MaxOfFloatArray _distances))))
  (Utilities|Array|RemoveIndex _availablelocations _output_get)
  (Utilities|Array|RemoveIndex _availablelocations _output_get_2)
  (Variables|Default|SetEnemyLocation (.OutItem (Utilities|Array|Random _availablelocations))))

(event EventBeginPlay
  (bind _components (Variables|Default|GetComponents))
  (Utilities|Array|Add _components (Variables|Default|GetC))
  (Utilities|Array|Add _components (Variables|Default|GetNW))
  (Utilities|Array|Add _components (Variables|Default|GetNE))
  (Utilities|Array|Add _components (Variables|Default|GetSE))
  (Utilities|Array|Add _components (Variables|Default|GetSW)))

(event Collision|EventActorBeginOverlap
  (params (OtherActor :type Actor%20Object%20Reference)))

(event EventTick
  (params (DeltaSeconds :type Float%20%28single-precision%29)))

(fn ConstructionScript)