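; BP_WindowTable is a prototype interactive window-table prop that triggers narrator events when the Dante pawn approaches and aims at it.
; Activate animates the cover's dynamic material noise and enables query collision on LookBox, as does the first player overlap, which fires a one-shot narrator event.
; LookatObject, while the pawn aims from inside the area, fires a second one-shot event and fades the noise scale to zero by timeline.
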(event OnComponentBeginOverlap(OverlapBox)
  (params (OverlappedComponent :type Primitive%20Component%20Object%20Reference) (OtherActor :type Actor%20Object%20Reference) (OtherComp :type Primitive%20Component%20Object%20Reference) (OtherBodyIndex :type Integer) (bFromSweep :type Boolean) (SweepResult :type Hit%20Result%20Structure%20%28by%20ref%29))
  (if (== (Utilities|GetClass OtherActor) "/Game/Dante/Blueprint/BP_DantePawn.BP_DantePawn_C")
    (Variables|Default|SetPlayerInArea OtherActor)
    (if (not (Variables|Default|GetTriggeredOverlap))
      (Variables|Default|SetTriggeredOverlap true)
      (Default|TriggerEvent (Variables|/Game/Dante/Blueprint/BP_DanteGameMode.BP_DanteGameMode_C|GetNarrator (Variables|Default|GetAs%20BP%20Dante%20Game%20Mode)) 3)
      (Collision|SetCollisionEnabled (Variables|Default|GetLookBox) "QueryOnly"))))

(event OnComponentEndOverlap(OverlapBox)
  (params (OverlappedComponent :type Primitive%20Component%20Object%20Reference) (OtherActor :type Actor%20Object%20Reference) (OtherComp :type Primitive%20Component%20Object%20Reference) (OtherBodyIndex :type Integer))
  (if (== (Utilities|GetClass OtherActor) "/Game/Dante/Blueprint/BP_DantePawn.BP_DantePawn_C")
    (Variables|Default|SetPlayerInArea 0)))

(event Custom|Activate
  (bind _mi (Variables|Default|GetMI))
  (Rendering|Material|SetScalarParameterValue _mi "Scale" (Variables|Default|GetNoiseScale) :!class /Script/Engine.MaterialInstanceDynamic)
  (Rendering|Material|SetScalarParameterValue _mi "Noise" 1e+01 :!class /Script/Engine.MaterialInstanceDynamic)
  (Collision|SetCollisionEnabled (Variables|Default|GetLookBox) "QueryOnly")
  (bind _newtrack_0 (Timeline|Timeline PlayFromStart)
    (:Update
      (Rendering|Material|SetScalarParameterValue (Variables|Default|GetMI) "Noise" _newtrack_0 :!class /Script/Engine.MaterialInstanceDynamic))))

(event EventBeginPlay
  (bind _asbp_dante_game_mode (Utilities|Casting|CastToBP_DanteGameMode (Game|GetGameMode)))
  (Variables|Default|SetAs%20BP%20Dante%20Game%20Mode _asbp_dante_game_mode)
  (bind _returnvalue (Rendering|Material|CreateDynamicMaterialInstance (Variables|Default|GetCover) 0 "/Game/XanWorld/ProtoType/Proxy/MI_WindowTable.MI_WindowTable" "None" :!class /Script/Engine.PrimitiveComponent))
  (Variables|Default|SetMI _returnvalue))

(event EventLookatObject
  (if (and (Variables|/Game/Dante/Blueprint/BP_DantePawn.BP_DantePawn_C|GetAiming (Variables|/Game/Dante/Blueprint/BP_DanteGameMode.BP_DanteGameMode_C|GetAs%20BP%20Dante%20Pawn (Variables|Default|GetAs%20BP%20Dante%20Game%20Mode))) (Utilities|IsValid (Variables|Default|GetPlayerInArea)))
    (if (not (Variables|Default|GetTriggeredLook))
      (Variables|Default|SetTriggeredLook true)
      (Utilities|FlowControl|Sequence
        (:then_1
          (bind _newtrack_0 (Timeline|Timeline_0 PlayFromStart)
            (:Update
              (Rendering|Material|SetScalarParameterValue (Variables|Default|GetMI) "Scale" (Math|Float|Lerp (Variables|Default|GetNoiseScale) 0.0 _newtrack_0) :!class /Script/Engine.MaterialInstanceDynamic))
            (:Finished
              (Development|PrintString "Hello"))))
        (:then_2
          (Default|TriggerEvent (Variables|/Game/Dante/Blueprint/BP_DanteGameMode.BP_DanteGameMode_C|GetNarrator (Variables|Default|GetAs%20BP%20Dante%20Game%20Mode)) 4))))))

(fn ConstructionScript)