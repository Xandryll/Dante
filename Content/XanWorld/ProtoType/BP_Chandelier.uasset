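; BP_Chandelier is an interactive chandelier that swings with a squeak and reacts to being looked at according to the game mode's DiveLevel.
; A looping timeline drives pivot pitch; StopSwing silences the sound and lets the current cycle finish.
; LookatObject fires once per level: at 0 it moves NPivot along a spline (apparently a newspaper), at 1 it triggers a narrator event and stops the swing.
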(event Custom|StopSwing
  (Variables|Default|SetSwingStop true)
  (Audio|Components|Audio|Stop (Variables|Default|GetSound)))

(event Custom|SwingChandelier
  (bind _returnvalue (Audio|SpawnSoundatLocation "/Game/Dante/Audio/MetalSqueak.MetalSqueak" (Transformation|GetActorLocation) "0, 0, 0" 1.0 1.0 0.0 0 0))
  (Variables|Default|SetSound _returnvalue)
  (bind _newtrack_0 (Timeline|Timeline PlayFromStart)
    (:Update
      (Transformation|SetRelativeRotation (Variables|Default|GetPivot) (Math|Rotator|MakeRotator 0.0 (* _newtrack_0 3e+01) 0.0) false false))
    (:Finished
      (if (Variables|Default|GetSwingStop)
        (Utilities|FlowControl|Sequence
          (:then_0
            (Timeline|Timeline Stop))
          (:then_1
            (Timeline|Timeline SetNewTime)))
        (else
          (Timeline|Timeline PlayFromStart))))))

(event EventLookatObject
  (switch int (Variables|/Game/Dante/Blueprint/BP_DanteGameMode.BP_DanteGameMode_C|GetDive_Level (Variables|Default|GetAs%20BP%20Dante%20Game%20Mode))
    (:0
      (if (not (Variables|Default|GetTriggered_NewsPaper))
        (Variables|Default|SetTriggered_NewsPaper true)
        (bind _newtrack_0 (Timeline|Timeline_0 PlayFromStart)
          (:Update
            (Transformation|SetRelativeTransform (Variables|Default|GetNPivot) (Spline|GetTransformatTime (Variables|Default|GetSpline) _newtrack_0 "Local" false false) false false)))))
    (:1
      (if (not (Variables|Default|GetTriggered_Cover))
        (Variables|Default|SetTriggered_Cover true)
        (Default|TriggerEvent (Variables|/Game/Dante/Blueprint/BP_DanteGameMode.BP_DanteGameMode_C|GetNarrator (Variables|Default|GetAs%20BP%20Dante%20Game%20Mode)) 1)
        (CallFunction|StopSwing)))))

(event EventBeginPlay
  (bind _asbp_dante_game_mode (Utilities|Casting|CastToBP_DanteGameMode (Game|GetGameMode)))
  (Variables|Default|SetAs%20BP%20Dante%20Game%20Mode _asbp_dante_game_mode)
  (bind _asbp_dante_pawn (Utilities|Casting|CastToBP_DantePawn (Game|Player|GetPlayerPawn 0))))

(fn ConstructionScript)