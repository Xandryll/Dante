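; BP_Curtains is a pair of curtains that open when something overlaps their box trigger.
; CloseCurtains enables query-only collision on the box and plays a timeline that widens two cube meshes along Y with a sound.
; Overlap calls OpenCurtains, which disables the trigger and reverses the same timeline with the same sound.
; When that reverse finishes, it triggers event 5 on the Dante game mode's Narrator.
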(event OnComponentBeginOverlap(Box)
  (params (OverlappedComponent :type Primitive%20Component%20Object%20Reference) (OtherActor :type Actor%20Object%20Reference) (OtherComp :type Primitive%20Component%20Object%20Reference) (OtherBodyIndex :type Integer) (bFromSweep :type Boolean) (SweepResult :type Hit%20Result%20Structure%20%28by%20ref%29))
  (CallFunction|OpenCurtains))

(event Custom|OpenCurtains
  (Collision|SetCollisionEnabled (Variables|Default|GetBox) "NoCollision")
  (Audio|PlaySoundatLocation "/Game/Dante/Audio/OpeningCurtain.OpeningCurtain" (Transformation|GetActorLocation) "0, 0, 0" 1e+01 1.0 0.0 0 0 0 0)
  (bind (_direction _newtrack_0) (Timeline|Timeline ReverseFromEnd)
    (:Update
      (Transformation|SetRelativeScale3D (Variables|Default|GetSM_Cube) (Math|Vector|MakeVector 0.05 (Math|Float|MapRangeClamped _newtrack_0 0.0 1.0 0.25 1.66) 3.317099))
      (Transformation|SetRelativeScale3D (Variables|Default|GetSM_Cube1) (Math|Vector|MakeVector 0.05 (Math|Float|MapRangeClamped _newtrack_0 0.0 1.0 0.25 1.66) 3.317099)))
    (:Finished
      (if (Utilities|Enum|Equal(Enum) _direction "Backward")
        (Default|TriggerEvent (Variables|/Game/Dante/Blueprint/BP_DanteGameMode.BP_DanteGameMode_C|GetNarrator (Variables|Default|GetAs%20BP%20Dante%20Game%20Mode)) 5)))))

(event Custom|CloseCurtains
  (Collision|SetCollisionEnabled (Variables|Default|GetBox) "QueryOnly")
  (Audio|PlaySoundatLocation "/Game/Dante/Audio/OpeningCurtain.OpeningCurtain" (Transformation|GetActorLocation) "0, 0, 0" 1e+01 1.0 0.0 0 0 0 0)
  (bind (_direction _newtrack_0) (Timeline|Timeline PlayFromStart)
    (:Update
      (Transformation|SetRelativeScale3D (Variables|Default|GetSM_Cube) (Math|Vector|MakeVector 0.05 (Math|Float|MapRangeClamped _newtrack_0 0.0 1.0 0.25 1.66) 3.317099))
      (Transformation|SetRelativeScale3D (Variables|Default|GetSM_Cube1) (Math|Vector|MakeVector 0.05 (Math|Float|MapRangeClamped _newtrack_0 0.0 1.0 0.25 1.66) 3.317099)))
    (:Finished
      (if (Utilities|Enum|Equal(Enum) _direction "Backward")
        (Default|TriggerEvent (Variables|/Game/Dante/Blueprint/BP_DanteGameMode.BP_DanteGameMode_C|GetNarrator (Variables|Default|GetAs%20BP%20Dante%20Game%20Mode)) 5)))))

(event EventBeginPlay
  (bind _asbp_dante_game_mode (Utilities|Casting|CastToBP_DanteGameMode (Game|GetGameMode)))
  (Variables|Default|SetAs%20BP%20Dante%20Game%20Mode _asbp_dante_game_mode))

(fn ConstructionScript)