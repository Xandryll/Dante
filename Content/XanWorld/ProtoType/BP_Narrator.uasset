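; BP_Narrator is the scripted-sequence director for the Dante prototype level, driving prop and audio beats and reacting to player dives.
; Triggerevent selects numbered beats that play the radio, animate props or bind one-shot OnDive reactions, with step 5 restoring the main dive handler.
; That handler hides level props at dive level 2, then spawns circle props and an enemy, with a special first-visit setup and later placement via CircleAreas.
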(event Custom|Trigger%20event
  (params (Step :type Integer))
  (bind _windowtablereference (Variables|Default|GetWindowTableReference))
  (bind _debug (Variables|Default|GetDebug))
  (bind _debug_2 (Variables|Default|GetDebug))
  (switch int Step
    (:0
      (Development|PrintString "Radio Enabled" _debug_2 _debug_2)
      (Default|Play (Variables|Default|GetWindowTableReference))
      (EventDispatchers|BindEventtoOnDive (Variables|Default|GetAs%20BP%20Dante%20Pawn) (delegate Custom|DisableRadio))
      (Utilities|FlowControl|Delay (Variables|Default|GetDelay_FromRadioToChandelier))
      (Default|SwingChandelier (Variables|Default|GetChandelierReference))
      (Development|PrintString "Chandelier moves" _debug _debug))
    (:1
      (Default|RemoveCover (Variables|Default|GetLogReference)))
    (:2
      (EventDispatchers|BindEventtoOnDive (Variables|Default|GetAs%20BP%20Dante%20Pawn) (delegate Custom|RemoveCovers)))
    (:3
      (Default|Play _windowtablereference))
    (:4
      (Default|StopSound _windowtablereference)
      (Default|Playloop _windowtablereference)
      (Utilities|FlowControl|Delay (Variables|Default|GetDelay_FromRadioLoopToWindowCurtains))
      (Default|CloseCurtains (Variables|Default|GetCuratinsReference)))
    (:5
      (EventDispatchers|BindEventtoOnDive (Variables|Default|GetAs%20BP%20Dante%20Pawn) (delegate Custom|CustomEvent)))))

(event Custom|PlayerDived)

(event Custom|RemoveCovers
  (params (DiveLevel :type Integer))
  (for _array_element (Variables|Default|GetCoverObject)
    (Default|RemoveCovers _array_element))
  (EventDispatchers|UnbindallEventsfromOnDive (Variables|Default|GetAs%20BP%20Dante%20Pawn))
  (Default|Activate (Variables|Default|GetWindowTableReference))
  (Audio|PlaySound2D "/Game/Dante/Audio/clothes-drop-2.clothes-drop-2" 1.0 1.0 0.0 0 0))

(event Custom|DisableRadio
  (params (DiveLevel :type Integer))
  (bind _debug (Variables|Default|GetDebug))
  (Development|PrintString "Radio Disabled" _debug _debug)
  (EventDispatchers|UnbindallEventsfromOnDive (Variables|Default|GetAs%20BP%20Dante%20Pawn))
  (Default|StopSound (Variables|Default|GetWindowTableReference)))

(event Custom|CustomEvent
  (params (DiveLevel :type Integer))
  (bind _windowtablereference (Variables|Default|GetWindowTableReference))
  (bind _circleareasreference (Variables|Default|GetCircleAreasReference))
  (if (Utilities|IsValid (Variables|/Game/XanWorld/ProtoType/BP_WindowTable.BP_WindowTable_C|GetCurrentAudio _windowtablereference))
    (Default|StopSound _windowtablereference))
  (if (Utilities|IsValid (Variables|Default|GetCircleProps))
    (Actor|DestroyActor (Variables|Default|GetCircleProps)))
  (if (== (Variables|/Game/Dante/Blueprint/BP_DanteGameMode.BP_DanteGameMode_C|GetDive_Level (Variables|Default|GetAs%20BP%20Dante%20Game%20Mode)) 2)
    (CallFunction|HideLevelProps)
    (if (Variables|Default|GetCircleFirstActivation)
      (Variables|Default|SetCircleFirstActivation false)
      (bind _returnvalue (Game|SpawnActorfromClass "/Game/XanWorld/ProtoType/BP_CircleProps.BP_CircleProps_C" (Math|Transform|MakeTransform (- (.location (Variables|/Game/Dante/Blueprint/BP_DantePawn.BP_DantePawn_C|GetDiveLocation (Variables|Default|GetAs%20BP%20Dante%20Pawn))) "0.000000,0.000000,96.000000") "0, 0, 0" "1.000000,1.000000,1.000000") "AlwaysSpawn" "MultiplyWithRoot" 0 0))
      (Variables|Default|SetCircleProps _returnvalue)
      (for _array_element (Variables|Default|GetCorridorsReference)
        (Default|TriggerDoor _array_element))
      (Default|StartCradleSwing (Variables|Default|GetLogReference))
      (Utilities|FlowControl|Delay 0.0)
      (bind _returnvalue_2 (Game|SpawnActorfromClass "/Game/XanWorld/BP_xSpawner.BP_xSpawner_C" (Math|Transform|MakeTransform "3000.000000,0.000000,50.000000" "0, 0, 0" "1.000000,1.000000,1.000000") "Undefined" "MultiplyWithRoot" 0 0))
      (Default|ActivateSpawner _returnvalue_2 "/Game/XanWorld/DataAssets/DA_DanteProtoEnemy_A.DA_DanteProtoEnemy_A" 1)
      (EventDispatchers|BindEventtoOnDive (Variables|Default|GetAs%20BP%20Dante%20Pawn) (delegate Custom|DestroyEnemy))
      (else
        (Default|CheckDistances _circleareasreference)
        (bind _returnvalue_3 (Game|SpawnActorfromClass "/Game/XanWorld/ProtoType/BP_CircleProps.BP_CircleProps_C" (Math|Transform|MakeTransform (Transformation|GetWorldLocation (Utilities|Array|Get(acopy) (Variables|/Game/XanWorld/ProtoType/BP_CircleAreas.BP_CircleAreas_C|GetComponents _circleareasreference) (Variables|/Game/XanWorld/ProtoType/BP_CircleAreas.BP_CircleAreas_C|GetCircleLocation _circleareasreference))) "0, 0, 0" "1.000000,1.000000,1.000000") "AlwaysSpawn" "MultiplyWithRoot" 0 0))
        (bind _output_get (Variables|Default|SetCircleProps _returnvalue_3))
        (Rendering|SetVisibility (Variables|/Game/XanWorld/ProtoType/BP_CircleProps.BP_CircleProps_C|GetLog _output_get) true false)
        (bind _returnvalue_4 (Game|SpawnActorfromClass "/Game/XanWorld/BP_xSpawner.BP_xSpawner_C" (Math|Transform|MakeTransform (Transformation|GetWorldLocation (Utilities|Array|Get(acopy) (Variables|/Game/XanWorld/ProtoType/BP_CircleAreas.BP_CircleAreas_C|GetComponents _circleareasreference) (Variables|/Game/XanWorld/ProtoType/BP_CircleAreas.BP_CircleAreas_C|GetEnemyLocation _circleareasreference))) "0, 0, 0" "1.000000,1.000000,1.000000") "Undefined" "MultiplyWithRoot" 0 0))
        (Default|ActivateSpawner _returnvalue_4 "/Game/XanWorld/DataAssets/DA_DanteProtoEnemy_A.DA_DanteProtoEnemy_A" 1)))
    (else
      (CallFunction|ShowLevelProps))))

(event Custom|HideLevelProps
  (for _array_element (Variables|Default|GetLevelActors)
    (Rendering|SetActorHiddenInGame _array_element true)
    (Collision|SetActorEnableCollision _array_element false)))

(event Custom|ShowLevelProps
  (for _array_element (Variables|Default|GetLevelActors)
    (Rendering|SetActorHiddenInGame _array_element false)
    (Collision|SetActorEnableCollision _array_element true)))

(event Custom|DestroyEnemy
  (params (DiveLevel :type Integer))
  (Actor|DestroyActor (Utilities|Array|Get(acopy) (Variables|/Game/XanWorld/BP_xSpawner.BP_xSpawner_C|GetEnemies (stale Custom|CustomEvent _returnvalue_2)))))

(event EventBeginPlay
  (bind _levelactors (Variables|Default|GetLevelActors))
  (bind _asbp_dante_pawn (Utilities|Casting|CastToBP_DantePawn (Game|Player|GetPlayerPawn 0)))
  (Variables|Default|SetAs%20BP%20Dante%20Pawn _asbp_dante_pawn)
  (bind _outactors (Actor|GetAllActorsOfClass "/Game/XanWorld/ProtoType/Proxy/BP_CoverObject.BP_CoverObject_C"))
  (Variables|Default|SetCoverObject _outactors)
  (bind _asbp_dante_game_mode (Utilities|Casting|CastToBP_DanteGameMode (Game|GetGameMode)))
  (Variables|Default|SetAs%20BP%20Dante%20Game%20Mode _asbp_dante_game_mode)
  (Utilities|Array|Add _levelactors (Variables|Default|GetLogReference))
  (Utilities|Array|Add _levelactors (Variables|Default|GetWindowTableReference))
  (Utilities|Array|Add _levelactors (Variables|Default|GetCuratinsReference))
  (Utilities|Array|AppendArray _levelactors (Variables|Default|GetCoverObject))
  (bind _outactors_2 (Actor|GetAllActorsOfClass "/Game/XanWorld/ProtoType/BP_DynamicCorridor.BP_DynamicCorridor_C"))
  (Variables|Default|SetCorridorsReference _outactors_2)
  (EventDispatchers|BindEventtoOnDive (Variables|Default|GetAs%20BP%20Dante%20Pawn) (delegate Custom|CustomEvent)))

(event Collision|EventActorBeginOverlap
  (params (OtherActor :type Actor%20Object%20Reference)))

(event EventTick
  (params (DeltaSeconds :type Float%20%28single-precision%29)))

(fn ConstructionScript)