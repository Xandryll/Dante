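; BP_Compass is a Hide 'n' Seek actor that points toward the game mode's current objective.
; BeginPlay caches BP_HideNSeekGameMode, and each Tick reads its CurrentObjective when valid.
; A LookAt from the Direction component yields a yaw, applied as world rotation to both Direction and Compass with pitch and roll zeroed.
; Alternative look-at rotation nodes remain in the graph but are not executed.
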(event EventBeginPlay
  (bind _asbp_hide_nseek_game_mode (Utilities|Casting|CastToBP_HideNSeekGameMode (Game|GetGameMode)))
  (Variables|Default|SetAs%20BP%20Hide%20NSeek%20Game%20Mode _asbp_hide_nseek_game_mode))

(event Collision|EventActorBeginOverlap
  (params (OtherActor :type Actor%20Object%20Reference)))

(event EventTick
  (params (DeltaSeconds :type Float%20%28single-precision%29))
  (bind _as_bp_hide_nseek_game_mode (Variables|Default|GetAs%20BP%20Hide%20NSeek%20Game%20Mode))
  (bind _direction (Variables|Default|GetDirection))
  (bind _currentobjective (Variables|/Game/XanWorld/HideNSeek/BP_HideNSeekGameMode.BP_HideNSeekGameMode_C|GetCurrentObjective _as_bp_hide_nseek_game_mode))
  (if (Utilities|IsValid _currentobjective)
    (Transformation|SetWorldRotation _direction (Math|Rotator|MakeRotator 0.0 0.0 (.yaw (.rotation (Class|KismetAnimationLibrary|Lookat (Transformation|GetWorldTransform _direction) (Transformation|GetActorLocation _currentobjective) "1.000000,0.000000,0.000000" false "0, 0, 0" 0.0)))) false false)))

(fn ConstructionScript)