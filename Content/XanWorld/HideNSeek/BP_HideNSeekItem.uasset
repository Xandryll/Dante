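; BP_HideNSeekItem is a collectible for the HideNSeek mode that is visible and collectible only while being looked at.
; Activate enables LookBox for queries, and each LookatObject call shows Sphere, enables Overlap and restarts a 0.1-second timer that hides both again.
; Overlap by BP_HideNSeekPAwn or BP_DantePawn calls ItemGatered on BP_HideNSeekGameMode, then Reset hides the item and disables its collision.
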(event OnComponentBeginOverlap(Overlap)
  (params (OverlappedComponent :type Primitive%20Component%20Object%20Reference) (OtherActor :type Actor%20Object%20Reference) (OtherComp :type Primitive%20Component%20Object%20Reference) (OtherBodyIndex :type Integer) (bFromSweep :type Boolean) (SweepResult :type Hit%20Result%20Structure%20%28by%20ref%29))
  (bind _returnvalue (Utilities|GetClass OtherActor))
  (if (or (== _returnvalue "/Game/XanWorld/HideNSeek/BP_HideNSeekPAwn.BP_HideNSeekPAwn_C") (== _returnvalue "/Game/Dante/Blueprint/BP_DantePawn.BP_DantePawn_C"))
    (bind _asbp_hide_nseek_game_mode (Utilities|Casting|CastToBP_HideNSeekGameMode (Game|GetGameMode)))
    (Default|ItemGatered _asbp_hide_nseek_game_mode)
    (CallFunction|Reset)))

(event Custom|Activate
  (Collision|SetCollisionEnabled (Variables|Default|GetLookBox) "QueryOnly"))

(event Custom|Reset
  (Rendering|SetVisibility (Variables|Default|GetSphere) false false)
  (Collision|SetCollisionEnabled (Variables|Default|GetLookBox) "NoCollision"))

(event Custom|CustomEvent
  (Collision|SetCollisionEnabled (Variables|Default|GetOverlap) "NoCollision")
  (Rendering|SetVisibility (Variables|Default|GetSphere) false false))

(event EventBeginPlay)

(event Collision|EventActorBeginOverlap
  (params (OtherActor :type Actor%20Object%20Reference)))

(event EventTick
  (params (DeltaSeconds :type Float%20%28single-precision%29)))

(event EventLookatObject
  (Collision|SetCollisionEnabled (Variables|Default|GetOverlap) "QueryOnly")
  (Rendering|SetVisibility (Variables|Default|GetSphere) true false)
  (if (Utilities|Time|IsValidTimerHandle (Variables|Default|GetVisibilityTimer))
    (Utilities|Time|ClearandInvalidateTimerbyHandle (Variables|Default|GetVisibilityTimer)))
  (bind _returnvalue (Utilities|Time|SetTimerbyEvent (delegate Custom|CustomEvent) 0.1))
  (Variables|Default|SetVisibilityTimer _returnvalue))

(fn ConstructionScript)