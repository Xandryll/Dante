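; Game mode for Hide N Seek that runs the start screen, music, item objectives and rising enemy difficulty.
; Initialize removes the start HUD, activates the enemy spawners and picks a random item objective, re-rolling whenever one is gathered.
; A per-second survival timer maps elapsed time to faster enemy movement and shorter waypoint waits.
; Another looping timer picks a random level light and modulates its intensity through a Timeline, then restores it.
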(event Custom|SurvivedTimer
  (bind _output_get (Variables|Default|SetSurvivedTime (+ (Variables|Default|GetSurvivedTime) 1.0)))
  (for _array_element (Variables|Default|GetSpawnerReference)
    (for _array_element_2 (Variables|/Game/XanWorld/BP_xSpawner.BP_xSpawner_C|GetEnemies _array_element)
      (Variables|/Script/Engine.CharacterMovementComponent|SetMaxWalkSpeed (Variables|/Script/Engine.Character|GetCharacterMovement _array_element_2) (Math|Float|MapRangeClamped (Math|Conversions|ToFloat(Integer) (/ _output_get 20)) 0.0 1e+01 2e+02 8e+02))
      (Variables|/Game/XanWorld/BP_BaseCharacter.BP_BaseCharacter_C|SetInvestigation_WaypointWaitTime _array_element_2 (Math|Float|MapRangeClamped (Math|Conversions|ToFloat(Integer) (/ _output_get 20)) 0.0 1e+01 5.0 2.0))
      (Variables|/Game/XanWorld/BP_BaseCharacter.BP_BaseCharacter_C|SetPatrol_WaypointWaitTime _array_element_2 (Math|Float|MapRangeClamped (Math|Conversions|ToFloat(Integer) (/ _output_get 20)) 0.0 1e+01 5.0 2.0)))))

(event Custom|ItemGatered
  (Math|Integer|IncrementInt (Variables|Default|GetItemsGathered)
    (:%20%20
      (CallFunction|SetNextObjective))))

(event Custom|SetNextObjective
  (bind _output_get (Variables|Default|SetCurrentObjective (.OutItem (Utilities|Array|Random (Variables|Default|GetObjectives)))))
  (Default|Activate _output_get))

(event Custom|LightTimer
  (bind _output_get (Variables|Default|SetLight%20Component (Variables|/Script/Engine.Light|GetLightComponent (.OutItem (Utilities|Array|Random (Variables|Default|GetLevelLights))))))
  (Variables|Default|SetIntensity (Variables|/Script/Engine.LightComponentBase|GetIntensity _output_get))
  (bind _newtrack_0 (Timeline|Timeline PlayFromStart)
    (:Update
      (Rendering|Components|Light|SetIntensity (Variables|Default|GetLight%20Component) (* _newtrack_0 (Variables|Default|GetIntensity))))
    (:Finished
      (Rendering|Components|Light|SetIntensity (Variables|Default|GetLight%20Component) (Variables|Default|GetIntensity))
      (Timeline|Timeline SetNewTime))))

(event Custom|Initialize
  (Widget|RemovefromParent (stale EventBeginPlay _returnvalue))
  (Utilities|Time|SetTimerbyEvent (delegate Custom|SurvivedTimer) 1.0 true)
  (bind _outactors (Actor|GetAllActorsOfClass "/Game/XanWorld/HideNSeek/BP_HideNSeekItem.BP_HideNSeekItem_C"))
  (Variables|Default|SetObjectives _outactors)
  (CallFunction|SetNextObjective)
  (bind _outactors_2 (Actor|GetAllActorsOfClass "/Script/Engine.Light"))
  (Variables|Default|SetLevelLights _outactors_2)
  (Utilities|Time|SetTimerbyEvent (delegate Custom|LightTimer) 5.0 true)
  (bind _outactors_3 (Actor|GetAllActorsOfClass "/Game/XanWorld/BP_xSpawner.BP_xSpawner_C"))
  (bind _output_get (Variables|Default|SetSpawnerReference _outactors_3))
  (Utilities|Casting|CastToBP_HideNSeekPAwn (Game|Player|GetPlayerPawn 0))
  (for _array_element _output_get
    (Default|ActivateSpawner _array_element)))

(event EventBeginPlay
  (bind _returnvalue (UserInterface|CreateWidget "/Game/XanWorld/Hud/HUD_StartGame.HUD_StartGame_C"))
  (UserInterface|Viewport|AddtoViewport _returnvalue 0)
  (Audio|PlaySound2D "/Game/Dante/Blueprint/Audio/creepySewers.creepySewers" 0.8 1.0 0.0 0 0))

(event EventTick
  (params (DeltaSeconds :type Float%20%28single-precision%29)))

(fn ConstructionScript
  (|CallParentFunction))