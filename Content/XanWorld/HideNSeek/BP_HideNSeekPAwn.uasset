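; BP_HideNSeekPAwn is the player pawn for the HideNSeek mode, adding light flicker and death handling to its parent.
; A randomly re-armed timer plays a timeline that modulates inner and outer light intensities, then restores them.
; KillActor unregisters the pawn from AI perception, disables input, shows the death screen and a score from items gathered over survival time, then reloads the level after a delay.
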(event Custom|CustomEvent
  (Variables|Default|SetIntensityInner (Variables|/Script/Engine.LightComponentBase|GetIntensity (Variables|Default|GetInnerLight)))
  (Variables|Default|SetIntensityOuter (Variables|/Script/Engine.LightComponentBase|GetIntensity (Variables|Default|GetOuterLight)))
  (bind _newtrack_0 (Timeline|Timeline_1 PlayFromStart)
    (:Update
      (Rendering|Components|Light|SetIntensity (Variables|Default|GetInnerLight) (* _newtrack_0 (Variables|Default|GetIntensityInner)))
      (Rendering|Components|Light|SetIntensity (Variables|Default|GetOuterLight) (* _newtrack_0 (Variables|Default|GetIntensityOuter))))
    (:Finished
      (Rendering|Components|Light|SetIntensity (Variables|Default|GetInnerLight) (Variables|Default|GetIntensityInner))
      (Rendering|Components|Light|SetIntensity (Variables|Default|GetOuterLight) (Variables|Default|GetIntensityOuter))
      (Utilities|FlowControl|Sequence
        (:then_0
          (Timeline|Timeline_1 SetNewTime))
        (:then_1
          (CallFunction|LightTimer))))))

(event Custom|LightTimer
  (Utilities|Time|SetTimerbyEvent (delegate Custom|CustomEvent) (Math|Random|RandomFloatinRange 1e+01 3e+01)))

(event EventBeginPlay
  (|CallParentFunction)
  (CallFunction|LightTimer))

(event Collision|EventActorBeginOverlap
  (params (OtherActor :type Actor%20Object%20Reference)))

(event EventTick
  (params (DeltaSeconds :type Float%20%28single-precision%29))
  (|CallParentFunction DeltaSeconds) ; This node is disabled and will not be called.\nDrag off pins to build functionality.
)

(event EventKillActor
  (params (DeathByEnemy :type Boolean))
  (bind _as_bp_dante_game_mode (Variables|Default|GetAs%20BP%20Dante%20Game%20Mode))
  (bind _wb_hud (Variables|Default|GetWB_Hud))
  ;[1 1 1] Death
  (Default|CallOnDie)
  (Class|AIPerceptionStimuliSourceComponent|UnregisterfromPerceptionSystem (Variables|Default|GetAIPerceptionStimuliSource))
  (Variables|/Game/Dante/Blueprint/BP_DanteGameMode.BP_DanteGameMode_C|SetPlayerDead _as_bp_dante_game_mode true)
  (Class|Image|SetOpacity (Variables|/Game/Dante/Blueprint/HUD/WB_Hud.WB_Hud_C|GetDieScreen _wb_hud) 1.0)
  (Input|DisableInput (Game|GetPlayerController 0))
  (bind _asbp_hide_nseek_game_mode (Utilities|Casting|CastToBP_HideNSeekGameMode (Game|GetGameMode)))
  (Default|ShowMessage _wb_hud (Utilities|String|Append "FINAL SCORE ----> " (Utilities|String|ToString(Float) (* (/ (Variables|/Game/XanWorld/HideNSeek/BP_HideNSeekGameMode.BP_HideNSeekGameMode_C|GetItemsGathered _asbp_hide_nseek_game_mode) (Variables|/Game/XanWorld/HideNSeek/BP_HideNSeekGameMode.BP_HideNSeekGameMode_C|GetSurvivedTime _asbp_hide_nseek_game_mode)) 1e+04))) true)
  (Utilities|FlowControl|Delay 1e+01)
  (Game|OpenLevel(byName) "HideNSeek")
  (Variables|/Game/Dante/Blueprint/BP_DanteGameMode.BP_DanteGameMode_C|SetPlayerDead _as_bp_dante_game_mode false))

(event Input|KeyboardEvents|E
  (params (Key :type Key%20Structure))
  (:Pressed
    (if true
      _)))

(fn ConstructionScript
  (|CallParentFunction))