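; Enemy spawner that places BP_BaseCharacter enemies at random reachable points around its volume, either on BeginPlay or via ActivateSpawner, and assigns each a patrol route.
; It gathers BP_PatrolRoutes from allowed groups and ranks them by navmesh path length, giving enemies routes from that ordered list.
; It tracks active versus available routes, supporting single random swaps, mass reassignment by distance from a point, and closest-route lookup.
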(event Custom|ActivateSpawner
  (params (DA%20to%20Spawn :type PDA%20X%20Enemy%20Object%20Reference) (EnemiesToSpawn :type Integer))
  (bind _orderedroutes (CallFunction|OrderRoutesbyDistance (Transformation|GetActorLocation self) (Variables|Default|GetRoutes)))
  (Variables|Default|SetAvailableRoutes _orderedroutes)
  (bind _spawnedenemies (CallFunction|SpawnEnemies (Math|Integer|SelectInt (Variables|Setup|GetEnemiesToSpawn) EnemiesToSpawn (Variables|Setup|GetAutoSpawn))))
  (Variables|Default|SetActiveEnemies _spawnedenemies)
  (for (_array_element _array_index) (Variables|Default|GetAvailableRoutes)
    (Variables|/Game/Dante/Blueprint/NavSystem/BP_PatrolRoute.BP_PatrolRoute_C|SetRouteIndex _array_element _array_index))
  (for (_array_element_2 _array_index_2) (Variables|Default|GetActiveEnemies)
    (Variables|/Game/XanWorld/BP_BaseCharacter.BP_BaseCharacter_C|SetPatrol_CurrentRoute _array_element_2 (Utilities|Array|Get(acopy) (Variables|Default|GetAvailableRoutes) _array_index_2))
    (Variables|/Game/XanWorld/BP_BaseCharacter.BP_BaseCharacter_C|SetSpawnerReference _array_element_2 self)
    (Utilities|Array|Add (Variables|Default|GetActiveRoutes) (Utilities|Array|Get(acopy) (Variables|Default|GetAvailableRoutes) _array_index_2))
    (Utilities|Array|RemoveItem (Variables|Default|GetAvailableRoutes) (Utilities|Array|Get(acopy) (Variables|Default|GetAvailableRoutes) _array_index_2))
    (Default|Initialize _array_element_2 (select (Variables|Setup|GetAutoSpawn) (Variables|Setup|GetAutoSpawnxEnemyConfiguration) DA%20to%20Spawn))))

(event Custom|SingleSelectNewRoute
  (params (Enemy :type BP%20Base%20Character%20Object%20Reference))
  (bind _availableroutes (Variables|Default|GetAvailableRoutes))
  (bind _activeroutes (Variables|Default|GetActiveRoutes))
  (bind _output_get (Variables|Default|SetNextRoute (Utilities|Array|Get(acopy) _availableroutes (Math|Random|RandomIntegerinRange 0 (Utilities|Array|LastIndex _availableroutes)))))
  (Utilities|Array|RemoveItem _availableroutes _output_get)
  (Utilities|Array|RemoveItem _activeroutes (Variables|/Game/XanWorld/BP_BaseCharacter.BP_BaseCharacter_C|GetPatrol_CurrentRoute Enemy))
  (Utilities|Array|Add _activeroutes _output_get)
  (Utilities|Array|Add _availableroutes (Variables|/Game/XanWorld/BP_BaseCharacter.BP_BaseCharacter_C|GetPatrol_CurrentRoute Enemy))
  (Variables|/Game/XanWorld/BP_BaseCharacter.BP_BaseCharacter_C|SetPatrol_CurrentRoute Enemy _output_get))

(event Custom|MassSelectNewRoute
  (params (Origin%20Location :type Vector%20%28by%20ref%29))
  (bind _orderedroutes (CallFunction|OrderRoutesbyDistance Origin%20Location (Variables|Default|GetRoutes)))
  (Variables|Default|SetActiveRoutes _orderedroutes)
  (for (_array_element _array_index) (Variables|Default|GetActiveEnemies)
    (Variables|/Game/XanWorld/BP_BaseCharacter.BP_BaseCharacter_C|SetPatrol_CurrentRoute _array_element (Utilities|Array|Get(acopy) (Variables|Default|GetActiveRoutes) _array_index)))
  (Utilities|Array|Resize (Variables|Default|GetActiveRoutes) (+ _array_index 1)))

(event Custom|RequestClosestRoute
  (params (Origin%20Location :type Vector%20%28by%20ref%29))
  (bind _closest_route (CallFunction|GetClosestRoute Origin%20Location (Variables|Default|GetRoutes)))
  (Variables|Default|SetTempClosestRoute _closest_route))

(event EventBeginPlay
  (CallFunction|GetRoutesViaGroup)
  (if (Variables|Setup|GetAutoSpawn)
    (bind _orderedroutes (CallFunction|OrderRoutesbyDistance (Transformation|GetActorLocation self) (Variables|Default|GetRoutes)))
    (Variables|Default|SetAvailableRoutes _orderedroutes)
    (bind _spawnedenemies (CallFunction|SpawnEnemies (Math|Integer|SelectInt (Variables|Setup|GetEnemiesToSpawn) (stale Custom|ActivateSpawner EnemiesToSpawn) (Variables|Setup|GetAutoSpawn))))
    (Variables|Default|SetActiveEnemies _spawnedenemies)
    (for (_array_element _array_index) (Variables|Default|GetAvailableRoutes)
      (Variables|/Game/Dante/Blueprint/NavSystem/BP_PatrolRoute.BP_PatrolRoute_C|SetRouteIndex _array_element _array_index))
    (for (_array_element_2 _array_index_2) (Variables|Default|GetActiveEnemies)
      (Variables|/Game/XanWorld/BP_BaseCharacter.BP_BaseCharacter_C|SetPatrol_CurrentRoute _array_element_2 (Utilities|Array|Get(acopy) (Variables|Default|GetAvailableRoutes) _array_index_2))
      (Variables|/Game/XanWorld/BP_BaseCharacter.BP_BaseCharacter_C|SetSpawnerReference _array_element_2 self)
      (Utilities|Array|Add (Variables|Default|GetActiveRoutes) (Utilities|Array|Get(acopy) (Variables|Default|GetAvailableRoutes) _array_index_2))
      (Utilities|Array|RemoveItem (Variables|Default|GetAvailableRoutes) (Utilities|Array|Get(acopy) (Variables|Default|GetAvailableRoutes) _array_index_2))
      (Default|Initialize _array_element_2 (select (Variables|Setup|GetAutoSpawn) (Variables|Setup|GetAutoSpawnxEnemyConfiguration) (stale Custom|ActivateSpawner DA%20to%20Spawn))))))

(event Collision|EventActorBeginOverlap
  (params (OtherActor :type Actor%20Object%20Reference)))

(fn ConstructionScript)

(fn OrderRoutesbyDistance
  (params (Origin%20Location :type Vector%20%28by%20ref%29) (TempRoutes :type Array%20of%20BP%20Patrol%20Route%20Object%20References))
  (bind _tempdistances (Variables|Default|GetTempDistances))
  (bind (_indexofminvalue _minvalue) (Math|Float|MinOfFloatArray _tempdistances))
  (Variables|Default|SetTempRoutes TempRoutes)
  (Utilities|Array|Clear (Variables|Default|GetOrderedRoutes))
  (Utilities|Array|Clear (Variables|Default|GetOrderedRoutesDistances))
  (Utilities|Array|Clear (Variables|Default|GetTempDistances))
  (for _array_element TempRoutes
    (bind _returnvalue (Class|NavigationSystemV1|FindPathtoLocationSynchronously Origin%20Location (Transformation|GetActorLocation _array_element) 0 0))
    (Utilities|Array|Add (Variables|Default|GetTempDistances) (Class|NavigationPath|GetPathLength _returnvalue)))
  (while (> (Utilities|Array|Length _tempdistances) 0)
    (Utilities|Array|Add (Variables|Default|GetOrderedRoutesDistances) _minvalue)
    (Utilities|Array|Add (Variables|Default|GetOrderedRoutes) (Utilities|Array|Get(acopy) (Variables|Default|GetTempRoutes) _indexofminvalue))
    (Utilities|Array|RemoveIndex (Variables|Default|GetTempRoutes) _indexofminvalue)
    (Utilities|Array|RemoveIndex (Variables|Default|GetTempDistances) _indexofminvalue))
  (return (Variables|Default|GetOrderedRoutes)))

(fn SpawnEnemies
  (params (EnemiesToSpawn :type Integer))
  (bind _enemies (Variables|Default|GetEnemies))
  (bind _volume (Variables|Default|GetVolume))
  (bind (_origin _boxextent _sphereradius) (Collision|GetComponentBounds _volume))
  (for _index (range 1 EnemiesToSpawn)
    (bind _returnvalue (Game|SpawnActorfromClass "/Game/XanWorld/BP_BaseCharacter.BP_BaseCharacter_C" (Math|Conversions|ToTransform(Vector) (+ (.RandomLocation (AI|Navigation|GetRandomReachablePointinRadius _origin _sphereradius 0 0)) "0.000000,0.000000,100.000000")) "AdjustIfPossibleButAlwaysSpawn" "MultiplyWithRoot" 0 0))
    (Utilities|Array|Add _enemies _returnvalue)
    (Variables|/Game/XanWorld/BP_BaseCharacter.BP_BaseCharacter_C|SetSpawnerReference _returnvalue self))
  (return _enemies))

(fn GetRoutesViaGroup
  (bind _routes (Variables|Default|GetRoutes))
  (Utilities|Array|Clear _routes)
  (bind _outactors (Actor|GetAllActorsOfClass "/Game/Dante/Blueprint/NavSystem/BP_PatrolRoute.BP_PatrolRoute_C"))
  (for _array_element _outactors
    (if (!= (Utilities|Array|FindItem (Variables|Default|GetAvailable%20Routes%20Groups) (Variables|/Game/Dante/Blueprint/NavSystem/BP_PatrolRoute.BP_PatrolRoute_C|GetRouteGroup _array_element)) -1)
      (Utilities|Array|Add _routes _array_element)))
  (return))

(fn GetClosestRoute
  (params (Origin%20Location :type Vector%20%28by%20ref%29) (Routes :type Array%20of%20BP%20Patrol%20Route%20Object%20References))
  (bind _tempdistances (Variables|Default|GetTempDistances))
  (bind (_indexofminvalue _minvalue) (Math|Float|MinOfFloatArray _tempdistances))
  (Variables|Default|SetTempRoutes Routes)
  (Utilities|Array|Clear (Variables|Default|GetOrderedRoutes))
  (Utilities|Array|Clear (Variables|Default|GetOrderedRoutesDistances))
  (Utilities|Array|Clear (Variables|Default|GetTempDistances))
  (for _array_element Routes
    (bind _returnvalue (Class|NavigationSystemV1|FindPathtoLocationSynchronously Origin%20Location (Transformation|GetActorLocation _array_element) 0 0))
    (Utilities|Array|Add (Variables|Default|GetTempDistances) (Class|NavigationPath|GetPathLength _returnvalue)))
  (while (> (Utilities|Array|Length _tempdistances) 0)
    (Utilities|Array|Add (Variables|Default|GetOrderedRoutesDistances) _minvalue)
    (Utilities|Array|Add (Variables|Default|GetOrderedRoutes) (Utilities|Array|Get(acopy) (Variables|Default|GetTempRoutes) _indexofminvalue))
    (Utilities|Array|RemoveIndex (Variables|Default|GetTempRoutes) _indexofminvalue)
    (Utilities|Array|RemoveIndex (Variables|Default|GetTempDistances) _indexofminvalue))
  (return (Utilities|Array|Get(acopy) (Variables|Default|GetOrderedRoutes))))