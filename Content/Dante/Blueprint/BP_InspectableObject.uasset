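; BP_InspectableObject is an inspectable object with a two-stage activation sequence, apparently a jewel box.
; ActivateArea switches on the selected area and moves mesh parts by instant, non-swept local offsets.
; Area A shifts the cylinder and box cube, disables its own collision and enables B's query-and-probe collision.
; Area B then slides the cube much further and disables its own collision.
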(event Custom|Activate%20Area
  (params (Selection :type String))
  (switch string Selection
    (:A
      (Transformation|AddLocalOffset (Variables|Default|GetCylinder3) "0.000000,0.000000,5.000000" false false)
      (Collision|SetCollisionEnabled (Variables|Default|GetA) "NoCollision")
      (Transformation|AddLocalOffset (Variables|Default|GetJewelBox_Cube_001) "0.000000,10.000000,5.000000" false false)
      (Collision|SetCollisionEnabled (Variables|Default|GetB) "QueryAndProbe"))
    (:B
      (Transformation|AddLocalOffset (Variables|Default|GetJewelBox_Cube_001) "0.000000,140.000000,0.000000" false false)
      (Collision|SetCollisionEnabled (Variables|Default|GetB) "NoCollision"))))

(event EventBeginPlay)

(event Collision|EventActorBeginOverlap
  (params (OtherActor :type Actor%20Object%20Reference)))

(event EventTick
  (params (DeltaSeconds :type Float%20%28single-precision%29)))

(fn ConstructionScript)