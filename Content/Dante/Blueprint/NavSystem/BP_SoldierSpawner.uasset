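; Soldier spawner that populates its volume with BP_Enemy soldiers on BeginPlay and hands each one a patrol route.
; It ranks every BP_PatrolRoute in the level by synchronous navmesh path length, using a repeated-minimum sort, and pairs soldiers with routes by index.
; Soldiers spawn at random reachable points within the volume's bounding radius and keep a reference to the spawner.
; UpdateRoutes re-ranks the routes from a given origin and reassigns them.
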(event Custom|ActivateSpawner
  (bind _orderedroutes (CallFunction|OrderRoutesbyDistance (Transformation|GetActorLocation self)))
  (Variables|Default|SetCurrentRoutes _orderedroutes)
  (bind _soldiers (CallFunction|SpawnSoldiers))
  (Variables|Default|SetActiveSoldiers _soldiers)
  (for (_array_element _array_index) (Variables|Default|GetCurrentRoutes)
    (Variables|/Game/Dante/Blueprint/NavSystem/BP_PatrolRoute.BP_PatrolRoute_C|SetRouteIndex _array_element _array_index))
  (for (_array_element_2 _array_index_2) (Variables|Default|GetActiveSoldiers)
    (Default|Initialize _array_element_2 (Utilities|Array|Get(acopy) (Variables|Default|GetCurrentRoutes) _array_index_2))))

(event Custom|UpdateRoutes
  (params (Origin%20Location :type Vector%20%28by%20ref%29))
  (bind _orderedroutes (CallFunction|OrderRoutesbyDistance Origin%20Location))
  (Variables|Default|SetCurrentRoutes _orderedroutes)
  (for (_array_element _array_index) (Variables|Default|GetActiveSoldiers)
    (Default|UpdateRoute _array_element (Utilities|Array|Get(acopy) (Variables|Default|GetCurrentRoutes) _array_index))))

(event EventBeginPlay
  (CallFunction|ActivateSpawner))

(event Collision|EventActorBeginOverlap
  (params (OtherActor :type Actor%20Object%20Reference)))

(event EventTick
  (params (DeltaSeconds :type Float%20%28single-precision%29)))

(fn ConstructionScript)

(fn OrderRoutesbyDistance
  (params (Origin%20Location :type Vector%20%28by%20ref%29))
  (bind _tempdistances (Variables|Default|GetTempDistances))
  (bind (_indexofminvalue _minvalue) (Math|Float|MinOfFloatArray _tempdistances))
  (Utilities|Array|Clear (Variables|Default|GetOrderedRoutes))
  (Utilities|Array|Clear (Variables|Default|GetTempRoutes))
  (Utilities|Array|Clear (Variables|Default|GetOrderedRoutesDistances))
  (Utilities|Array|Clear (Variables|Default|GetTempDistances))
  (bind _outactors (Actor|GetAllActorsOfClass "/Game/Dante/Blueprint/NavSystem/BP_PatrolRoute.BP_PatrolRoute_C"))
  (bind _output_get (Variables|Default|SetTempRoutes _outactors))
  (for _array_element _output_get
    (bind _returnvalue (Class|NavigationSystemV1|FindPathtoLocationSynchronously Origin%20Location (Transformation|GetActorLocation _array_element) 0 0))
    (Utilities|Array|Add (Variables|Default|GetTempDistances) (Class|NavigationPath|GetPathLength _returnvalue)))
  (while (> (Utilities|Array|Length _tempdistances) 0)
    (Utilities|Array|Add (Variables|Default|GetOrderedRoutesDistances) _minvalue)
    (Utilities|Array|Add (Variables|Default|GetOrderedRoutes) (Utilities|Array|Get(acopy) (Variables|Default|GetTempRoutes) _indexofminvalue))
    (Utilities|Array|RemoveIndex (Variables|Default|GetTempRoutes) _indexofminvalue)
    (Utilities|Array|RemoveIndex (Variables|Default|GetTempDistances) _indexofminvalue))
  (return (Variables|Default|GetOrderedRoutes)))

(fn SpawnSoldiers
  (bind _soldiers (Variables|Default|GetSoldiers))
  (bind _volume (Variables|Default|GetVolume))
  (bind (_origin _boxextent _sphereradius) (Collision|GetComponentBounds _volume))
  (for _index (range 1 (Variables|Default|GetSoldiersToSpawn))
    (bind _returnvalue (Game|SpawnActorfromClass "/Game/Dante/Blueprint/BP_Enemy.BP_Enemy_C" (Math|Conversions|ToTransform(Vector) (+ (.RandomLocation (AI|Navigation|GetRandomReachablePointinRadius _origin _sphereradius 0 0)) "0.000000,0.000000,100.000000")) "AdjustIfPossibleButAlwaysSpawn" "MultiplyWithRoot" 0 0))
    (Variables|/Game/Dante/Blueprint/BP_Enemy.BP_Enemy_C|SetEnemyDA _returnvalue "/Game/Dante/Blueprint/PDAs/DataAssets/DA_Soldier.DA_Soldier")
    (Variables|/Script/Engine.Pawn|SetAIControllerClass _returnvalue "/Script/AIModule.AIController")
    (Variables|/Game/Dante/Blueprint/BP_Enemy.BP_Enemy_C|SetSpawned _returnvalue true)
    (Utilities|Array|Add _soldiers _returnvalue)
    (Variables|/Game/Dante/Blueprint/BP_Enemy.BP_Enemy_C|SetSpawnerOwner _returnvalue self))
  (return _soldiers))