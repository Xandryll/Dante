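; BP_BaseItem is a base interactable item that appears only at a matching dive level and destroys itself on Interact.
; On BeginPlay and ChangeLevel it compares the game mode's DiveLevel with VisibleInLevel, toggling visibility and collision on the mesh and box.
; Box overlaps with the player pawn send in-range and out-of-range messages, passing the item plus its PDAItem name and interaction string on entry.
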(event OnComponentBeginOverlap(Box)
  (params (OverlappedComponent :type Primitive%20Component%20Object%20Reference) (OtherActor :type Actor%20Object%20Reference) (OtherComp :type Primitive%20Component%20Object%20Reference) (OtherBodyIndex :type Integer) (bFromSweep :type Boolean) (SweepResult :type Hit%20Result%20Structure%20%28by%20ref%29))
  (bind _as_bp_dante_pawn (Variables|Default|GetAs%20BP%20Dante%20Pawn))
  (bind _pda_item (Variables|Default|GetPDA_Item))
  ;[1 1 1] Overlap system
  (if (== OtherActor _as_bp_dante_pawn)
    (Class|BPIDante|IteminRange(Message) _as_bp_dante_pawn self (Variables|/Game/Dante/Blueprint/PDAs/PDA_Items.PDA_Items_C|GetInteractionString _pda_item) (Variables|/Game/Dante/Blueprint/PDAs/PDA_Items.PDA_Items_C|GetName _pda_item))))

(event OnComponentEndOverlap(Box)
  (params (OverlappedComponent :type Primitive%20Component%20Object%20Reference) (OtherActor :type Actor%20Object%20Reference) (OtherComp :type Primitive%20Component%20Object%20Reference) (OtherBodyIndex :type Integer))
  (bind _as_bp_dante_pawn (Variables|Default|GetAs%20BP%20Dante%20Pawn))
  ;[1 1 1] Overlap system
  (if (== OtherActor _as_bp_dante_pawn)
    (Class|BPIDante|ItemOutOfRange(Message) _as_bp_dante_pawn)))

(event Custom|ChangeLevel
  (bind _self self)
  (bind _staticmesh (Variables|Default|GetStaticMesh))
  (if (== (Variables|/Game/Dante/Blueprint/BP_DanteGameMode.BP_DanteGameMode_C|GetDive_Level (Variables|Default|GetAs%20BP%20Dante%20Game%20Mode)) (Variables|Default|GetVisible%20in%20level))
    (Rendering|SetActorHiddenInGame _self false)
    (Collision|SetCollisionEnabled _staticmesh "QueryAndPhysics")
    (else
      (Rendering|SetActorHiddenInGame _self true)
      (Collision|SetCollisionEnabled _staticmesh "NoCollision"))))

(event EventBeginPlay
  (bind _self self)
  (bind _staticmesh (Variables|Default|GetStaticMesh))
  (bind _asbp_dante_game_mode (Utilities|Casting|CastToBP_DanteGameMode (Game|GetGameMode)))
  (Variables|Default|SetAs%20BP%20Dante%20Game%20Mode _asbp_dante_game_mode)
  (bind _asbp_dante_pawn (Utilities|Casting|CastToBP_DantePawn (Game|Player|GetPlayerPawn 0)))
  (Variables|Default|SetAs%20BP%20Dante%20Pawn _asbp_dante_pawn)
  (if (== (Variables|/Game/Dante/Blueprint/BP_DanteGameMode.BP_DanteGameMode_C|GetDive_Level (Variables|Default|GetAs%20BP%20Dante%20Game%20Mode)) (Variables|Default|GetVisible%20in%20level))
    (Rendering|SetActorHiddenInGame _self false)
    (Collision|SetCollisionEnabled _staticmesh "QueryAndPhysics")
    (else
      (Rendering|SetActorHiddenInGame _self true)
      (Collision|SetCollisionEnabled _staticmesh "NoCollision"))))

(event Collision|EventActorBeginOverlap
  (params (OtherActor :type Actor%20Object%20Reference)))

(event EventTick
  (params (DeltaSeconds :type Float%20%28single-precision%29)))

(event EventInteract
  (Actor|DestroyActor))

(fn ConstructionScript)

(fn IteminRange
  (params (Item :type BP%20Base%20Item%20Object%20Reference) (InteractionString :type String) (Name :type String)))