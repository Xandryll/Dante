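; Hiding closet that lets the Dante pawn hide from AI perception.
; Box overlap reports the closet and its PDA text to the pawn as an interactable.
; Interact switches the view to the closet and, unless the pawn is spotted, unregisters its perception stimuli and teleports it to a safe zone.
; F or Exit returns the pawn to ExitDirection and re-registers stimuli; a second F handler also re-possesses it.
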(event OnComponentEndOverlap(Box)
  (params (OverlappedComponent :type Primitive%20Component%20Object%20Reference) (OtherActor :type Actor%20Object%20Reference) (OtherComp :type Primitive%20Component%20Object%20Reference) (OtherBodyIndex :type Integer))
  ;[1 1 1] Show Interaction Logic
  (Default|ItemOutOfRange (Variables|Default|GetAs%20BP%20Dante%20Pawn)))

(event OnComponentBeginOverlap(Box)
  (params (OverlappedComponent :type Primitive%20Component%20Object%20Reference) (OtherActor :type Actor%20Object%20Reference) (OtherComp :type Primitive%20Component%20Object%20Reference) (OtherBodyIndex :type Integer) (bFromSweep :type Boolean) (SweepResult :type Hit%20Result%20Structure%20%28by%20ref%29))
  (bind _pda_item (Variables|Default|GetPDA_Item))
  ;[1 1 1] Show Interaction Logic
  (Default|IteminRange (Variables|Default|GetAs%20BP%20Dante%20Pawn) self (Variables|/Game/Dante/Blueprint/PDAs/PDA_Items.PDA_Items_C|GetInteractionString _pda_item) (Variables|/Game/Dante/Blueprint/PDAs/PDA_Items.PDA_Items_C|GetName _pda_item)))

(event Custom|Exit
  (bind _as_bp_dante_pawn (Variables|Default|GetAs%20BP%20Dante%20Pawn))
  ;[0 0.6928 1] Interaction Logic
  ;;[1 1 1] Exit Hiding Place
  (Variables|/Game/Dante/Blueprint/BP_DantePawn.BP_DantePawn_C|SetIsHiding _as_bp_dante_pawn false)
  (Transformation|Teleport _as_bp_dante_pawn (Transformation|GetWorldLocation (Variables|Default|GetExitDirection)) (Transformation|GetWorldRotation (Variables|Default|GetDefaultSceneRoot)))
  (Class|AIPerceptionStimuliSourceComponent|RegisterwithPerceptionSystem (Variables|/Game/Dante/Blueprint/BP_DantePawn.BP_DantePawn_C|GetAIPerceptionStimuliSource _as_bp_dante_pawn))
  (Game|Player|SetViewTargetwithBlend (Game|GetPlayerController 0) _as_bp_dante_pawn 0.0 "VTBlend_Linear" 0.0 false)
  (Variables|/Game/Dante/Blueprint/BP_DantePawn.BP_DantePawn_C|SetCurrentHidingSpot _as_bp_dante_pawn 0))

(event EventBeginPlay
  (|CallParentFunction) ; This node is disabled and will not be called.\nDrag off pins to build functionality.
)

(event Collision|EventActorBeginOverlap
  (params (OtherActor :type Actor%20Object%20Reference))
  (|CallParentFunction OtherActor) ; This node is disabled and will not be called.\nDrag off pins to build functionality.
)

(event EventTick
  (params (DeltaSeconds :type Float%20%28single-precision%29))
  (|CallParentFunction DeltaSeconds) ; This node is disabled and will not be called.\nDrag off pins to build functionality.
)

(event EventInteract
  (bind _self self)
  (bind _as_bp_dante_pawn (Variables|Default|GetAs%20BP%20Dante%20Pawn))
  ;[0 0.6928 1] Interaction Logic
  ;;[1 1 1] Enter Hiding Place
  (Variables|/Game/Dante/Blueprint/BP_DantePawn.BP_DantePawn_C|SetIsHiding _as_bp_dante_pawn true)
  (Variables|/Game/Dante/Blueprint/BP_DantePawn.BP_DantePawn_C|SetCurrentHidingSpot _as_bp_dante_pawn _self)
  (Game|Player|SetViewTargetwithBlend (Game|GetPlayerController 0) _self 0.0 "VTBlend_Linear" 0.0 false)
  (if (not (Variables|/Game/Dante/Blueprint/BP_DantePawn.BP_DantePawn_C|GetisSpotted _as_bp_dante_pawn))
    (Class|AIPerceptionStimuliSourceComponent|UnregisterfromPerceptionSystem (Variables|/Game/Dante/Blueprint/BP_DantePawn.BP_DantePawn_C|GetAIPerceptionStimuliSource _as_bp_dante_pawn))
    (Default|TeleporttoSafeZone _as_bp_dante_pawn)))

(event Input|KeyboardEvents|F
  (params (Key :type Key%20Structure :default "None"))
  (bind _as_bp_dante_pawn (Variables|Default|GetAs%20BP%20Dante%20Pawn))
  ;[0 0.6928 1] Interaction Logic
  ;;[1 1 1] Exit Hiding Place
  (:Pressed
    (Variables|/Game/Dante/Blueprint/BP_DantePawn.BP_DantePawn_C|SetIsHiding _as_bp_dante_pawn false)
    (Transformation|Teleport _as_bp_dante_pawn (Transformation|GetWorldLocation (Variables|Default|GetExitDirection)) (Transformation|GetWorldRotation (Variables|Default|GetDefaultSceneRoot)))
    (Class|AIPerceptionStimuliSourceComponent|RegisterwithPerceptionSystem (Variables|/Game/Dante/Blueprint/BP_DantePawn.BP_DantePawn_C|GetAIPerceptionStimuliSource _as_bp_dante_pawn))
    (Game|Player|SetViewTargetwithBlend (Game|GetPlayerController 0) _as_bp_dante_pawn 0.0 "VTBlend_Linear" 0.0 false)
    (Variables|/Game/Dante/Blueprint/BP_DantePawn.BP_DantePawn_C|SetCurrentHidingSpot _as_bp_dante_pawn 0)))

(event Input|KeyboardEvents|F
  (params (Key :type Key%20Structure :default "None"))
  (bind _returnvalue (Game|GetPlayerController 0))
  (bind _as_bp_dante_pawn (Variables|Default|GetAs%20BP%20Dante%20Pawn))
  ;[0 0.6928 1] Interaction Logic
  ;;[1 1 1] Exit Hiding Place
  (:Pressed
    (Variables|/Game/Dante/Blueprint/BP_DantePawn.BP_DantePawn_C|SetIsHiding _as_bp_dante_pawn false)
    (Pawn|UnPossess _returnvalue)
    (Transformation|Teleport _as_bp_dante_pawn (Transformation|GetWorldLocation (Variables|Default|GetExitDirection)) (Transformation|GetWorldRotation (Variables|Default|GetDefaultSceneRoot)))
    (Pawn|Possess _returnvalue _as_bp_dante_pawn)
    (Class|AIPerceptionStimuliSourceComponent|RegisterwithPerceptionSystem (Variables|/Game/Dante/Blueprint/BP_DantePawn.BP_DantePawn_C|GetAIPerceptionStimuliSource _as_bp_dante_pawn))))

(fn ConstructionScript
  (|CallParentFunction))