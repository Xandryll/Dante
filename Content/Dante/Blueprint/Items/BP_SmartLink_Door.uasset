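; Nav link proxy that wraps a child BP_Door so AI agents can path through and open it.
; On BeginPlay it registers itself with the door, then either enables the smart link or, if locked, disables it and passes its lock settings to the door.
; When an agent reaches a closed door, it plays a timed knock, spawns a wood-smash sound, destroys both audio components, then calls AIOpenDoor.
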(event EventBeginPlay
  (bind _asbp_door (Utilities|Casting|CastToBP_Door (Variables|/Script/Engine.ChildActorComponent|GetChildActor (Variables|Default|GetChildActor))))
  (bind _output_get (Variables|Default|SetAs%20BP%20Door _asbp_door))
  (Variables|/Game/Dante/Blueprint/Items/BP_Door.BP_Door_C|SetSmartLink _output_get self)
  (if (Variables|Default|GetLocked)
    (Class|NavLinkProxy|SetSmartLinkEnabled false)
    (Variables|/Game/Dante/Blueprint/Items/BP_Door.BP_Door_C|SetLocked (Variables|Default|GetAs%20BP%20Door) (Variables|Default|GetLocked))
    (Variables|/Game/Dante/Blueprint/Items/BP_Door.BP_Door_C|SetLockedKey (Variables|Default|GetAs%20BP%20Door) (Variables|Default|GetLockedKey))
    (Variables|/Game/Dante/Blueprint/Items/BP_Door.BP_Door_C|SetOpenAtDiveLevel (Variables|Default|GetAs%20BP%20Door) (Variables|Default|GetOpenedAtDiveLevel))
    (else
      (Class|NavLinkProxy|SetSmartLinkEnabled true))))

(event Collision|EventActorBeginOverlap
  (params (OtherActor :type Actor%20Object%20Reference)))

(event EventTick
  (params (DeltaSeconds :type Float%20%28single-precision%29)))

(event EventSmartLinkReached
  (params (Agent :type Actor%20Object%20Reference) (Destination :type Vector%20%28by%20ref%29 :default "0, 0, 0"))
  (bind _returnvalue (Transformation|GetActorLocation))
  (if (not (Variables|/Game/Dante/Blueprint/Items/BP_Door.BP_Door_C|GetDoorOpen (Variables|Default|GetAs%20BP%20Door)))
    (bind _returnvalue_2 (Audio|SpawnSoundatLocation (Variables|Default|GetKnockSound) _returnvalue "0, 0, 0" 1.0 1.0 0.0 0 0))
    (Utilities|FlowControl|Delay 3.0)
    (Audio|Components|Audio|Stop _returnvalue_2)
    (bind _returnvalue_3 (Audio|SpawnSoundatLocation "/Game/Dante/Blueprint/Audio/wood-smash-2-170417_Cue.wood-smash-2-170417_Cue" _returnvalue "0, 0, 0" 1.0 1.0 0.0 0 0))
    (Components|DestroyComponent _returnvalue_2)
    (Default|AIOpenDoor (Variables|Default|GetAs%20BP%20Door) Agent self)))

(fn ConstructionScript)