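; BP_ReadableObject is an interactable item that displays readable text on the Dante pawn's HUD.
; ShowReadable can first show a non-persistent spoken phrase as a HUD message, gated by SpeakBeforeInteraction, and wait briefly.
; It then passes ReadableText to the HUD's readable panel and immediately calls InteractionFinished, without waiting for the panel to close.
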(event EventBeginPlay
  (|CallParentFunction) ; This node is disabled and will not be called.\nDrag off pins to build functionality.
)

(event Collision|EventActorBeginOverlap
  (params (OtherActor :type Actor%20Object%20Reference))
  (|CallParentFunction OtherActor) ; This node is disabled and will not be called.\nDrag off pins to build functionality.
)

(event EventTick
  (params (DeltaSeconds :type Float%20%28single-precision%29))
  (|CallParentFunction DeltaSeconds) ; This node is disabled and will not be called.\nDrag off pins to build functionality.
)

(event EventShowReadable
  (params (Item :type BP%20Base%20Item%20Object%20Reference))
  (bind _as_bp_dante_pawn (Variables|Default|GetAs%20BP%20Dante%20Pawn))
  (bind _wb_hud (Variables|/Game/Dante/Blueprint/BP_DantePawn.BP_DantePawn_C|GetWB_Hud _as_bp_dante_pawn))
  (if (Variables|Parameters|Readable|GetSpeakBeforeInteraction)
    (Default|ShowMessage _wb_hud (Utilities|String|ToString(Text) (Variables|Parameters|Readable|GetPhraseBeforeInteraction)) false)
    (Utilities|FlowControl|Delay 3.0))
  (Default|ShowReadable _wb_hud (Variables|Parameters|Readable|GetReadableText) true)
  (CallFunction|InteractionFinished))

(fn ConstructionScript
  (|CallParentFunction))