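; BP_PointlessBook is an interactable flavor item in the Dante game, a book with no shown gameplay effect.
; On BeginPlay it applies a random material from its Materials array to the static mesh, varying the look of each instance.
; On Interact it shows a non-persistent message on the Dante pawn's HUD widget saying the book is pointless.
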(event EventBeginPlay
  (|CallParentFunction)
  (Rendering|Material|SetMaterial (Variables|Default|GetStaticMesh) 0 (.OutItem (Utilities|Array|Random (Variables|Default|GetMaterials)))))

(event Collision|EventActorBeginOverlap
  (params (OtherActor :type Actor%20Object%20Reference)))

(event EventTick
  (params (DeltaSeconds :type Float%20%28single-precision%29))
  (|CallParentFunction DeltaSeconds) ; This node is disabled and will not be called.\nDrag off pins to build functionality.
)

(event EventInteract
  (Default|ShowMessage (Variables|/Game/Dante/Blueprint/BP_DantePawn.BP_DantePawn_C|GetWB_Hud (Variables|Default|GetAs%20BP%20Dante%20Pawn)) "This is just another pointless book..." false))

(fn ConstructionScript
  (|CallParentFunction))