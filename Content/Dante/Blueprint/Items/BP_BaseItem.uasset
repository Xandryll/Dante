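; Base Blueprint for interactable items, with empty valid and invalid interaction events as hooks.
; Interact can be gated by a required active equipped item, optionally consumed with HUD feedback, or by a condition object, which keeps the box's collision off until its activation event fires.
; ChangeLevel toggles visibility and collision by the game mode's dive level unless persistent.
; InteractionFinished updates game-mode quests for quest finishers.
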(event Custom|InteractionFinished
  (if (Variables|Parameters|GetIsQuestFinisher)
    (Default|UpdateQuests (Variables|Logic|GetAs%20BP%20Dante%20Game%20Mode) (Variables|Parameters|GetQuestFinisherType))))

(event Custom|InvalidInteraction)

(event Custom|ValidInteraction)

(event Custom|FinishQuest)

(event Custom|CondtionActivation_Event
  (Variables|Logic|SetIsConditionSatisfied true)
  (Collision|SetCollisionEnabled (Variables|Default|GetBox) "QueryOnly"))

(event Custom|ChangeLevel
  (bind _self self)
  (bind _staticmesh (Variables|Default|GetStaticMesh))
  (if (or (== (Variables|/Game/Dante/Blueprint/BP_DanteGameMode.BP_DanteGameMode_C|GetDive_Level (Variables|Logic|GetAs%20BP%20Dante%20Game%20Mode)) (Variables|Parameters|Dive|GetVisible%20in%20level)) (Variables|Parameters|Dive|GetisPersistent))
    (Rendering|SetActorHiddenInGame _self false)
    (Collision|SetCollisionEnabled _staticmesh "QueryAndPhysics")
    (else
      (Rendering|SetActorHiddenInGame _self true)
      (Collision|SetCollisionEnabled _staticmesh "NoCollision"))))

(event EventBeginPlay
  (bind _box (Variables|Default|GetBox))
  (bind _preinteractioncondition (Variables|Parameters|Base|GetPreInteractionCondition))
  (bind _asbp_dante_game_mode (Utilities|Casting|CastToBP_DanteGameMode (Game|GetGameMode)))
  (Variables|Logic|SetAs%20BP%20Dante%20Game%20Mode _asbp_dante_game_mode)
  (bind _asbp_dante_pawn (Utilities|Casting|CastToBP_DantePawn (Game|Player|GetPlayerPawn 0)))
  (Variables|Logic|SetAs%20BP%20Dante%20Pawn _asbp_dante_pawn)
  (Utilities|IsValid _preinteractioncondition
    (:Is%20Valid
      (Collision|SetCollisionEnabled _box "NoCollision")
      (EventDispatchers|AssignCondtionActivation _preinteractioncondition (delegate Custom|CondtionActivation_Event)))
    (:Is%20Not%20Valid
      (if (Utilities|IsValidClass (Variables|Parameters|Base|GetPreInteractionObject))
        (Variables|Logic|SetIsConditionSatisfied false)
        (else
          (Variables|Logic|SetIsConditionSatisfied true)))
      (Collision|SetCollisionEnabled _box "QueryOnly"))))

(event EventTick
  (params (DeltaSeconds :type Float%20%28single-precision%29)))

(event EventInteract
  (bind _preinteractioncondition (Variables|Parameters|Base|GetPreInteractionCondition))
  (bind _preinteractionincorrectobjectphrase (Variables|Parameters|Base|GetPreInteractionIncorrectObjectPhrase))
  (bind _preinteractioncorrectobjectphrase (Variables|Parameters|Base|GetPreInteractionCorrectObjectPhrase))
  (bind _as_bp_dante_pawn (Variables|Logic|GetAs%20BP%20Dante%20Pawn))
  (bind _preinteractionobject (Variables|Parameters|Base|GetPreInteractionObject))
  (bind _wb_hud (Variables|/Game/Dante/Blueprint/BP_DantePawn.BP_DantePawn_C|GetWB_Hud _as_bp_dante_pawn))
  (if (Variables|Logic|GetIsConditionSatisfied)
    (CallFunction|ValidInteraction :!label _label)
    (elif (Utilities|IsValidClass _preinteractionobject)
      (if (and (== _preinteractionobject (Utilities|GetClass (Variables|/Game/Dante/Blueprint/BP_DantePawn.BP_DantePawn_C|GetItemEquipped _as_bp_dante_pawn))) (Variables|/Game/Dante/Blueprint/BP_DantePawn.BP_DantePawn_C|GetItemActive _as_bp_dante_pawn))
        (if (> (Utilities|String|Len _preinteractioncorrectobjectphrase) 0)
          (Default|ShowMessage _wb_hud _preinteractioncorrectobjectphrase false))
        (CallFunction|ValidInteraction)
        (Variables|Logic|SetIsConditionSatisfied true)
        (if (Variables|Parameters|Base|GetConsumeObject)
          (Actor|DestroyActor (Variables|/Game/Dante/Blueprint/BP_DantePawn.BP_DantePawn_C|GetItemEquipped _as_bp_dante_pawn))
          (Variables|/Game/Dante/Blueprint/BP_DantePawn.BP_DantePawn_C|SetItemEquipped _as_bp_dante_pawn 0))
        (else
          (if (> (Utilities|String|Len _preinteractionincorrectobjectphrase) 0)
            (Default|ShowMessage _wb_hud _preinteractionincorrectobjectphrase false))
          (CallFunction|InvalidInteraction)))
      (else
        (Utilities|IsValid _preinteractioncondition
          (:Is%20Valid
            (if (Variables|BP_BaseItem_C|GetQuestActivatorCondition _preinteractioncondition)
              (CallFunction|ValidInteraction)
              (else
                (CallFunction|InvalidInteraction))))
          (:Is%20Not%20Valid
            (goto _label)))))))

(fn ConstructionScript)

(fn IteminRange
  (params (Item :type BP%20Base%20Item%20Object%20Reference) (InteractionString :type String) (Name :type String)))