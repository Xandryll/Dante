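; BP_Door is a swinging door that the player and AI characters can open, with a stuck state for the player.
; Timelines rotate it away from whoever opens it, and ForceChangeState can drive it with a set direction and speed.
; MagicLock makes it glow temporarily, delaying approaching AI, who knock and smash before opening.
; While opened through a timeline, it keeps a spawned nav modifier, destroyed on closing.
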(event OnComponentBeginOverlap(ApproachOpponentBox)
  (params (OverlappedComponent :type Primitive%20Component%20Object%20Reference) (OtherActor :type Actor%20Object%20Reference) (OtherComp :type Primitive%20Component%20Object%20Reference) (OtherBodyIndex :type Integer) (bFromSweep :type Boolean) (SweepResult :type Hit%20Result%20Structure%20%28by%20ref%29))
  ;[1 1 1] Approach enemy box collision logic
  (if (== (Utilities|GetClass OtherActor) "/Game/XanWorld/BP_BaseCharacter.BP_BaseCharacter_C")
    (CallFunction|ApproachDoor OtherActor)))

(event Custom|ForceChangeState
  (params (OpenAlongNormal :type Boolean) (OpeningSpeedFactor :type Float%20%28single-precision%29) (PlaySoundEffect :type Boolean) (Sound :type Sound%20Base%20Object%20Reference))
  (bind _door (Variables|Default|GetDoor))
  (bind _door_2 (Variables|Default|GetDoor))
  (bind _returnvalue (Transformation|GetWorldTransform _door_2))
  ;[1 1 1] Player interaction
  (Components|Timeline|SetPlayRate (Variables|Default|GetTimeline_2) OpeningSpeedFactor)
  (if PlaySoundEffect
    (Audio|PlaySoundatLocation Sound (Transformation|GetActorLocation) "0, 0, 0" 1.0 1.0 0.0 0 0 0 0))
  (bind _output_get (Variables|Default|SetForcedActivation true))
  (if (not (Variables|Default|GetisBusy))
    (Variables|Default|SetisBusy true)
    (bind _output_get_2 (Variables|Default|SetTempDirection (Math|Float|SelectFloat (Math|Float|SelectFloat -9e+01 9e+01 OpenAlongNormal) (Math|Float|SelectFloat 9e+01 -9e+01 (>= (Math|Vector|DotProduct (Math|Vector|GetForwardVector (Variables|/Game/Dante/Blueprint/BP_DantePawn.BP_DantePawn_C|GetFirstPersonCamera (Variables|Default|GetAs%20BP%20Dante%20Pawn))) (* (Math|Vector|GetRightVector (Variables|Default|GetDoor)) -1.0)) 0.0)) _output_get)))
    (bind _newtrack_0 (Timeline|Timeline_2 PlayFromStart)
      (:Update
        (Transformation|SetRelativeRotation _door (Math|Rotator|MakeRotator 0.0 0.0 (Math|Float|Lerp (Math|Float|SelectFloat (.yaw (Variables|/Script/Engine.SceneComponent|GetRelativeRotation _door)) 0.0 (Variables|Default|GetDoorOpen)) (Math|Float|SelectFloat 0.0 _output_get_2 (Variables|Default|GetDoorOpen)) _newtrack_0)) false false))
      (:Finished
        (if (Variables|Default|GetDoorOpen)
          (Variables|Default|SetDoorOpen false)
          (Actor|DestroyActor (Variables|Default|GetDoorNavMod))
          (else
            (Variables|Default|SetDoorOpen true)
            (Variables|Default|SetMagicLocked false)
            (Rendering|Material|SetScalarParameterValue (Variables|Default|GetDoorMaterial) "Glow" 0.0 :!class /Script/Engine.MaterialInstanceDynamic)
            (Utilities|Time|ClearandInvalidateTimerbyHandle (Variables|Default|GetMagiLockTimer))
            (bind _returnvalue_2 (Game|SpawnActorfromClass "/Game/Dante/Blueprint/BP_DoorNavModifier.BP_DoorNavModifier_C" (Math|Transform|MakeTransform (.location _returnvalue) (.rotation _returnvalue) "1.000000,1.000000,1.000000") "AlwaysSpawn" "MultiplyWithRoot" 0 0))
            (Variables|Default|SetDoorNavMod _returnvalue_2)))
        (Variables|Default|SetisBusy false)))))

(event Custom|ApproachDoor
  (params (Actor :type Actor%20Object%20Reference))
  (bind _returnvalue (Transformation|GetActorLocation))
  (bind _self self)
  ;[1 1 1] Enemy opening door sequence
  (if (not (Variables|BP_Door_C|GetDoorOpen _self))
    (if (Variables|Default|GetMagicLocked)
      (bind _returnvalue_2 (Audio|SpawnSoundatLocation (Variables|Default|GetKnockSound) _returnvalue "0, 0, 0" 1.0 1.0 0.0 0 0))
      (Utilities|FlowControl|Delay 5.0)
      (Audio|Components|Audio|Stop _returnvalue_2)
      (bind _returnvalue_3 (Audio|SpawnSoundatLocation "/Game/Dante/Blueprint/Audio/wood-smash-2-170417_Cue.wood-smash-2-170417_Cue" _returnvalue "0, 0, 0" 1.0 1.0 0.0 0 0))
      (Components|DestroyComponent _returnvalue_2)
      (Variables|Default|SetMagicLocked false)
      (Rendering|Material|SetScalarParameterValue (Variables|Default|GetDoorMaterial) "Glow" 0.0 :!class /Script/Engine.MaterialInstanceDynamic)
      (else
        (Utilities|FlowControl|Delay 2.0)))
    (CallFunction|AIOpenDoor _self Actor _self)))

(event Custom|RemoveMagic
  (Variables|Default|SetMagicLocked false)
  (Rendering|Material|SetScalarParameterValue (Variables|Default|GetDoorMaterial) "Glow" 0.0 :!class /Script/Engine.MaterialInstanceDynamic)
  (Utilities|Time|ClearandInvalidateTimerbyHandle (Variables|Default|GetMagiLockTimer)))

(event Custom|AIOpenDoor
  (params (Actor :type Actor%20Object%20Reference) (SmartDoor :type Actor%20Object%20Reference))
  (bind _door (Variables|Default|GetDoor))
  (bind _approachopponentbox (Variables|Default|GetApproachOpponentBox))
  (bind _returnvalue (Transformation|GetWorldTransform _door))
  ;[1 1 1] AI opening door
  (if (not (Variables|Default|GetisBusy))
    (bind _output_get (Variables|Default|SetTmpActorLoc (Transformation|GetActorForwardVector Actor)))
    (Variables|Default|SetisBusy true)
    (bind _newtrack_0 (Timeline|Timeline_1 PlayFromStart)
      (:Update
        (Transformation|SetRelativeRotation (Variables|Default|GetDoor) (Math|Rotator|MakeRotator 0.0 0.0 (Math|Float|Lerp 0.0 (Math|Float|SelectFloat 9e+01 -9e+01 (>= (Math|Vector|DotProduct _output_get (* (Math|Vector|GetRightVector (Variables|Default|GetDoor)) -1.0)) 0.0)) _newtrack_0)) false false))
      (:Finished
        (if (Variables|Default|GetDoorOpen)
          (Variables|Default|SetDoorOpen false)
          (Collision|SetCollisionEnabled _approachopponentbox "QueryOnly")
          (Actor|DestroyActor (Variables|Default|GetDoorNavMod))
          (else
            (Variables|Default|SetDoorOpen true)
            (Collision|SetCollisionEnabled _approachopponentbox "NoCollision")
            (bind _returnvalue_2 (Game|SpawnActorfromClass "/Game/Dante/Blueprint/BP_DoorNavModifier.BP_DoorNavModifier_C" (Math|Transform|MakeTransform (.location _returnvalue) (.rotation _returnvalue) "1.000000,1.000000,1.000000") "AlwaysSpawn" "MultiplyWithRoot" 0 0))
            (Variables|Default|SetDoorNavMod _returnvalue_2)))
        (Variables|Default|SetisBusy false)
        (Variables|Default|SetMagicLocked false)
        (Rendering|Material|SetScalarParameterValue (Variables|Default|GetDoorMaterial) "Glow" 0.0 :!class /Script/Engine.MaterialInstanceDynamic)
        (Utilities|Time|ClearandInvalidateTimerbyHandle (Variables|Default|GetMagiLockTimer))))))

(event Custom|MagicLock
  (Variables|Default|SetMagicLocked true)
  (Rendering|Material|SetScalarParameterValue (Variables|Default|GetDoorMaterial) "Glow" 1.0 :!class /Script/Engine.MaterialInstanceDynamic)
  (bind _returnvalue (Utilities|Time|SetTimerbyEvent (delegate Custom|RemoveMagic) 2e+01))
  (Variables|Default|SetMagiLockTimer _returnvalue))

(event EventBeginPlay
  (bind _door (Variables|Default|GetDoor))
  (|CallParentFunction)
  (Collision|SetCollisionEnabled (Variables|Default|GetBox) "NoCollision")
  (bind _returnvalue (Rendering|Material|CreateDynamicMaterialInstance _door 0 "/Game/Dante/Meshes/Materials/M_DoorWood_Inst.M_DoorWood_Inst" "None" :!class /Script/Engine.PrimitiveComponent))
  (bind _output_get (Variables|Default|SetDoorMaterial _returnvalue))
  (Rendering|Material|SetMaterial _door 0 _output_get)
  (if (Variables|Default|GetStartsOpen)
    (Transformation|SetRelativeRotation (Variables|Default|GetDoor) (Math|Rotator|MakeRotator 0.0 0.0 9e+01) false false)
    (Variables|Default|SetDoorOpen true)))

(event EventTick
  (params (DeltaSeconds :type Float%20%28single-precision%29))
  (|CallParentFunction DeltaSeconds))

(event EventValidInteraction
  (bind _door (Variables|Default|GetDoor))
  (bind _door_2 (Variables|Default|GetDoor))
  (bind _returnvalue (Transformation|GetWorldTransform _door_2))
  ;[1 1 1] Player interaction
  (if (Variables|Default|GetLocked)
    (Default|ShowMessage (Variables|/Game/Dante/Blueprint/BP_DantePawn.BP_DantePawn_C|GetWB_Hud (Variables|Default|GetAs%20BP%20Dante%20Pawn)) "The door is stuck !" false)
    (else
      (Components|Timeline|SetPlayRate (Variables|Default|GetTimeline_2) 1.0)
      (if (not (Variables|Default|GetisBusy))
        (Variables|Default|SetisBusy true)
        (bind _output_get (Variables|Default|SetTempDirection (Math|Float|SelectFloat (Math|Float|SelectFloat -9e+01 9e+01 (stale Custom|ForceChangeState OpenAlongNormal)) (Math|Float|SelectFloat 9e+01 -9e+01 (>= (Math|Vector|DotProduct (Math|Vector|GetForwardVector (Variables|/Game/Dante/Blueprint/BP_DantePawn.BP_DantePawn_C|GetFirstPersonCamera (Variables|Default|GetAs%20BP%20Dante%20Pawn))) (* (Math|Vector|GetRightVector (Variables|Default|GetDoor)) -1.0)) 0.0)) (stale Custom|ForceChangeState _output_get))))
        (bind _newtrack_0 (Timeline|Timeline_2 PlayFromStart)
          (:Update
            (Transformation|SetRelativeRotation _door (Math|Rotator|MakeRotator 0.0 0.0 (Math|Float|Lerp (Math|Float|SelectFloat (.yaw (Variables|/Script/Engine.SceneComponent|GetRelativeRotation _door)) 0.0 (Variables|Default|GetDoorOpen)) (Math|Float|SelectFloat 0.0 _output_get (Variables|Default|GetDoorOpen)) _newtrack_0)) false false))
          (:Finished
            (if (Variables|Default|GetDoorOpen)
              (Variables|Default|SetDoorOpen false)
              (Actor|DestroyActor (Variables|Default|GetDoorNavMod))
              (else
                (Variables|Default|SetDoorOpen true)
                (Variables|Default|SetMagicLocked false)
                (Rendering|Material|SetScalarParameterValue (Variables|Default|GetDoorMaterial) "Glow" 0.0 :!class /Script/Engine.MaterialInstanceDynamic)
                (Utilities|Time|ClearandInvalidateTimerbyHandle (Variables|Default|GetMagiLockTimer))
                (bind _returnvalue_2 (Game|SpawnActorfromClass "/Game/Dante/Blueprint/BP_DoorNavModifier.BP_DoorNavModifier_C" (Math|Transform|MakeTransform (.location _returnvalue) (.rotation _returnvalue) "1.000000,1.000000,1.000000") "AlwaysSpawn" "MultiplyWithRoot" 0 0))
                (Variables|Default|SetDoorNavMod _returnvalue_2)))
            (Variables|Default|SetisBusy false)))))))

(fn ConstructionScript
  (|CallParentFunction))