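; Interactable object, such as a sliding door or drawer, that toggles between closed and open when it receives a valid interaction.
; A timeline lerps the actor between its BeginPlay position and an offset along its selected local axis, scaled by an opening distance.
; IsOpen picks the direction of travel and flips on finish, while IsActive blocks retriggering during movement.
; Invalid interactions do nothing.
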(event EventBeginPlay
  (|CallParentFunction)
  (Variables|Logic|SetOriginalPosition (Transformation|GetActorLocation)))

(event Collision|EventActorBeginOverlap
  (params (OtherActor :type Actor%20Object%20Reference))
  (|CallParentFunction OtherActor) ; This node is disabled and will not be called.\nDrag off pins to build functionality.
)

(event EventTick
  (params (DeltaSeconds :type Float%20%28single-precision%29))
  (|CallParentFunction DeltaSeconds) ; This node is disabled and will not be called.\nDrag off pins to build functionality.
)

(event EventInvalidInteraction)

(event EventValidInteraction
  (bind _returnvalue (Transformation|GetActorUpVector))
  (bind _returnvalue_2 (Transformation|GetActorRightVector))
  (bind _returnvalue_3 (Transformation|GetActorForwardVector))
  (bind _openingaxis (Variables|Parameters|Openable|GetOpeningAxis))
  (bind _openingdistance (Variables|Parameters|Openable|GetOpeningDistance))
  (bind _originalposition (Variables|Logic|GetOriginalPosition))
  (bind _returnvalue_4 (Utilities|Select :Index _openingaxis :NewEnumerator0 _returnvalue_3 :NewEnumerator1 _returnvalue_2 :NewEnumerator2 _returnvalue))
  (bind _returnvalue_5 (* _returnvalue_4 _openingdistance))
  (bind _returnvalue_6 (+ _originalposition _returnvalue_5))
  (if (not (Variables|Logic|GetIsActive))
    (bind _newtrack_0 (Timeline|Timeline PlayFromStart)
      (:Update
        (Transformation|SetActorLocation (Math|Vector|Lerp(Vector) (Math|Vector|SelectVector _originalposition _returnvalue_6 (not (Variables|Logic|GetisOpen))) (Math|Vector|SelectVector _returnvalue_6 _originalposition (not (Variables|Logic|GetisOpen))) _newtrack_0) false false)
        (Variables|Logic|SetIsActive true))
      (:Finished
        (Variables|Logic|SetisOpen (not (Variables|Logic|GetisOpen)))
        (Variables|Logic|SetIsActive false)))))

(fn ConstructionScript
  (|CallParentFunction))