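; BP_Soul is an interactable soul that acts as a quest giver, asking the player for a specific item.
; On Interact, it compares the class of the Dante pawn's active equipped item to WantedItem, removing it and setting QuestEnded on a match.
; Each outcome shows a non-persistent message on the pawn's HUD widget: a request, wrong item, correct item, or thanks once the quest has ended.
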(event EventBeginPlay
  (|CallParentFunction) ; This node is disabled and will not be called.\nDrag off pins to build functionality.
)

(event Collision|EventActorBeginOverlap
  (params (OtherActor :type Actor%20Object%20Reference))
  (|CallParentFunction OtherActor) ; This node is disabled and will not be called.\nDrag off pins to build functionality.
)

(event EventTick
  (params (DeltaSeconds :type Float%20%28single-precision%29))
  (|CallParentFunction DeltaSeconds) ; This node is disabled and will not be called.\nDrag off pins to build functionality.
)

(event EventInteract
  (bind _as_bp_dante_pawn (Variables|Default|GetAs%20BP%20Dante%20Pawn))
  (bind _wb_hud (Variables|/Game/Dante/Blueprint/BP_DantePawn.BP_DantePawn_C|GetWB_Hud _as_bp_dante_pawn))
  (if (Variables|Default|GetQuestEnded)
    (Default|ShowMessage _wb_hud "Thank you for your help..." false)
    (elif (Variables|/Game/Dante/Blueprint/BP_DantePawn.BP_DantePawn_C|GetItemActive _as_bp_dante_pawn)
      (if (== (Utilities|GetClass (Variables|/Game/Dante/Blueprint/BP_DantePawn.BP_DantePawn_C|GetItemEquipped _as_bp_dante_pawn)) (Variables|Default|GetWantedItem))
        (Default|ShowMessage _wb_hud "This is the item i was looking for !" false)
        (Default|RemoveItem _as_bp_dante_pawn)
        (Variables|Default|SetQuestEnded true)
        (else
          (Default|ShowMessage _wb_hud "This is the WRONG item" false)))
      (else
        (Default|ShowMessage _wb_hud "Give me knowledge..." false)))))

(fn ConstructionScript
  (|CallParentFunction))