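; BP_CombinationDoor is a puzzle door that slides its mesh down when every gear in the combination is correct.
; CheckGears scans all BP_DoorGear actors in the level and clears the Solved flag if any is not Correct.
; On success it fires OpenDoor, whose timeline drives the mesh's relative Z, then destroys all gears.
; On failure it resets Solved to true for the next check.
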(event Custom|OpenDoor
  (bind _newtrack_0 (Timeline|Timeline Play)
    (:Update
      (Transformation|SetRelativeLocation (Variables|Default|GetStaticMesh) (Math|Vector|MakeVector 0.0 0.0 (* _newtrack_0 -4e+02)) false false))))

(event Custom|CheckGears
  (bind _outactors (Actor|GetAllActorsOfClass "/Game/Dante/Blueprint/Items/BP_DoorGear.BP_DoorGear_C"))
  (for _array_element _outactors
    (if (not (Variables|/Game/Dante/Blueprint/Items/BP_DoorGear.BP_DoorGear_C|GetCorrect _array_element))
      (Variables|Default|SetSolved false)))
  (if (Variables|Default|GetSolved)
    (CallFunction|OpenDoor)
    (for _array_element_2 _outactors
      (Actor|DestroyActor _array_element_2))
    (else
      (Variables|Default|SetSolved true))))

(event EventBeginPlay
  (|CallParentFunction))

(event Collision|EventActorBeginOverlap
  (params (OtherActor :type Actor%20Object%20Reference))
  (|CallParentFunction OtherActor) ; This node is disabled and will not be called.\nDrag off pins to build functionality.
)

(event EventTick
  (params (DeltaSeconds :type Float%20%28single-precision%29))
  (|CallParentFunction DeltaSeconds) ; This node is disabled and will not be called.\nDrag off pins to build functionality.
)

(fn ConstructionScript
  (|CallParentFunction))