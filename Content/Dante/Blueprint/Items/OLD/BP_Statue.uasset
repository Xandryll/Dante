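; Statue actor whose eye material changes to show whether it has been activated.
; On BeginPlay it creates a dynamic instance of MI_Eyes on mesh slot 0 and tints it orange.
; ActivateStatue turns the color green, raises the emissive power and sets the Active flag.
; The Interact event is empty, and nothing in this Blueprint calls ActivateStatue.
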(event Custom|ActivateStatue
  (bind _materialinstance (Variables|Default|GetMaterialInstance))
  (Rendering|Material|SetScalarParameterValue _materialinstance "EmissivePower" 1e+01 :!class /Script/Engine.MaterialInstanceDynamic)
  (Rendering|Material|SetVectorParameterValue _materialinstance "Color" "(R=0.173600,G=1.000000,B=0.000000,A=1.000000)" :!class /Script/Engine.MaterialInstanceDynamic)
  (Variables|Default|SetActive true))

(event EventBeginPlay
  (bind _staticmesh (Variables|Default|GetStaticMesh))
  (|CallParentFunction)
  (bind _returnvalue (Rendering|Material|CreateDynamicMaterialInstance _staticmesh 0 "/Game/Dante/Meshes/MI_Eyes.MI_Eyes" "None" :!class /Script/Engine.PrimitiveComponent))
  (bind _output_get (Variables|Default|SetMaterialInstance _returnvalue))
  (Rendering|Material|SetMaterial _staticmesh 0 _output_get)
  (Rendering|Material|SetVectorParameterValue (Variables|Default|GetMaterialInstance) "Color" "(R=0.979167,G=0.575735,B=0.325593,A=1.000000)" :!class /Script/Engine.MaterialInstanceDynamic))

(event Collision|EventActorBeginOverlap
  (params (OtherActor :type Actor%20Object%20Reference))
  (|CallParentFunction OtherActor) ; This node is disabled and will not be called.\nDrag off pins to build functionality.
)

(event EventTick
  (params (DeltaSeconds :type Float%20%28single-precision%29))
  (|CallParentFunction DeltaSeconds) ; This node is disabled and will not be called.\nDrag off pins to build functionality.
)

(event EventInteract)

(fn ConstructionScript
  (|CallParentFunction))