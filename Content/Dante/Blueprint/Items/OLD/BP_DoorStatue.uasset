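; BP_DoorStatue is an interactable rotating statue that forms part of a combination puzzle linked to a door.
; On interact, if the game mode's dive level matches the statue's visible level, it adds a fixed yaw step to its mesh and flags whether it matches the wanted rotation.
; It then asks the linked door to check the combination.
; Otherwise, the HUD shows a message that the statue cannot rotate.
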(event EventBeginPlay
  (|CallParentFunction) ; This node is disabled and will not be called.\nDrag off pins to build functionality.
)

(event Collision|EventActorBeginOverlap
  (params (OtherActor :type Actor%20Object%20Reference))
  (|CallParentFunction OtherActor) ; This node is disabled and will not be called.\nDrag off pins to build functionality.
)

(event EventTick
  (params (DeltaSeconds :type Float%20%28single-precision%29))
  (|CallParentFunction DeltaSeconds) ; This node is disabled and will not be called.\nDrag off pins to build functionality.
)

(event EventInteract
  (if (== (Variables|Default|GetVisible%20in%20level) (Variables|/Game/Dante/Blueprint/BP_DanteGameMode.BP_DanteGameMode_C|GetDive_Level (Variables|Default|GetAs%20BP%20Dante%20Game%20Mode)))
    (bind _output_get (Variables|Default|SetCurrentRotation (+ (Variables|Default|GetCurrentRotation) 45)))
    (Transformation|SetRelativeRotation (Variables|Default|GetStaticMesh) (Math|Rotator|MakeRotator 0.0 0.0 (Math|Conversions|ToFloat(Integer) _output_get)) false false)
    (Variables|Default|SetisRotationCorrect (== (Variables|Default|GetWantedRotation) (Variables|Default|GetCurrentRotation)))
    (Default|CheckCombination (Variables|Default|GetDoor))
    (else
      (Default|ShowMessage (Variables|/Game/Dante/Blueprint/BP_DantePawn.BP_DantePawn_C|GetWB_Hud (Variables|Default|GetAs%20BP%20Dante%20Pawn)) "The basement of the statue appears to be broken, it can't rotate." false))))

(fn ConstructionScript
  (|CallParentFunction))