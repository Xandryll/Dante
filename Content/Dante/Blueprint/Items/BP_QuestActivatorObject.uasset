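; BP_QuestActivatorObject is an interactable item that activates a quest condition when the player uses it.
; On the first valid interaction it sets IsActive and QuestActivatorCondition, then, only if a pre-activation phrase exists, shows it on the Dante pawn's HUD and calls CallCondtionActivation.
; Later interactions only show the post-activation phrase, if set, as a non-persistent message.
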(event EventBeginPlay
  (|CallParentFunction) ; This node is disabled and will not be called.\nDrag off pins to build functionality.
)

(event Collision|EventActorBeginOverlap
  (params (OtherActor :type Actor%20Object%20Reference))
  (|CallParentFunction OtherActor) ; This node is disabled and will not be called.\nDrag off pins to build functionality.
)

(event EventTick
  (params (DeltaSeconds :type Float%20%28single-precision%29))
  (|CallParentFunction DeltaSeconds) ; This node is disabled and will not be called.\nDrag off pins to build functionality.
)

(event EventValidInteraction
  (bind _preactivationphrase (Variables|Parameters|QuestInteractor|GetPreActivationPhrase))
  (bind _as_bp_dante_pawn (Variables|Default|GetAs%20BP%20Dante%20Pawn))
  (bind _postactivationphrase (Variables|Parameters|QuestInteractor|GetPostActivationPhrase))
  (bind _wb_hud (Variables|/Game/Dante/Blueprint/BP_DantePawn.BP_DantePawn_C|GetWB_Hud _as_bp_dante_pawn))
  (if (Variables|Logic|GetIsActive)
    (if (> (Utilities|String|Len _postactivationphrase) 0)
      (Default|ShowMessage _wb_hud _postactivationphrase false))
    (else
      (Variables|Logic|SetIsActive true)
      (Variables|Default|SetQuestActivatorCondition true)
      (if (> (Utilities|String|Len _preactivationphrase) 0)
        (Default|ShowMessage _wb_hud _preactivationphrase false)
        (Default|CallCondtionActivation)))))

(fn ConstructionScript
  (|CallParentFunction))