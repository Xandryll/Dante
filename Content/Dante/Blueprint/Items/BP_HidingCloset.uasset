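; BP_HidingCloset is an interactable closet the player pawn can hide in, with an interaction prompt driven by box overlap.
; Interact switches view to the closet camera and, if unspotted, unregisters the pawn from AI perception, teleports it to a safe zone and enables clamped look input on Tick.
; Exit restores the pawn, view and perception at the exit point.
; Destroy swaps in a broken mesh, disables interaction and plays a smash sound.
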(event OnComponentEndOverlap(Box)
  (params (OverlappedComponent :type Primitive%20Component%20Object%20Reference) (OtherActor :type Actor%20Object%20Reference) (OtherComp :type Primitive%20Component%20Object%20Reference) (OtherBodyIndex :type Integer))
  (bind _returnvalue (Utilities|GetClass OtherActor))
  ;[1 1 1] Show Interaction Logic
  (if (or (== _returnvalue "/Game/Dante/Blueprint/BP_DantePawn.BP_DantePawn_C") (== _returnvalue "/Game/XanWorld/HideNSeek/BP_HideNSeekPAwn.BP_HideNSeekPAwn_C"))
    (Default|ItemOutOfRange (Variables|Default|GetAs%20BP%20Dante%20Pawn))))

(event OnComponentBeginOverlap(Box)
  (params (OverlappedComponent :type Primitive%20Component%20Object%20Reference) (OtherActor :type Actor%20Object%20Reference) (OtherComp :type Primitive%20Component%20Object%20Reference) (OtherBodyIndex :type Integer) (bFromSweep :type Boolean) (SweepResult :type Hit%20Result%20Structure%20%28by%20ref%29))
  (bind _returnvalue (Utilities|GetClass OtherActor))
  (bind _pda_item (Variables|Default|GetPDA_Item))
  ;[1 1 1] Show Interaction Logic
  (if (or (== _returnvalue "/Game/Dante/Blueprint/BP_DantePawn.BP_DantePawn_C") (== _returnvalue "/Game/XanWorld/HideNSeek/BP_HideNSeekPAwn.BP_HideNSeekPAwn_C"))
    (Default|IteminRange (Variables|Default|GetAs%20BP%20Dante%20Pawn) self (Variables|/Game/Dante/Blueprint/PDAs/PDA_Items.PDA_Items_C|GetInteractionString _pda_item) (Variables|/Game/Dante/Blueprint/PDAs/PDA_Items.PDA_Items_C|GetName _pda_item))))

(event Custom|Exit
  (bind _as_bp_dante_pawn (Variables|Default|GetAs%20BP%20Dante%20Pawn))
  ;[0 0.6928 1] Interaction Logic
  ;;[1 1 1] Exit Hiding Place
  (Variables|/Game/Dante/Blueprint/BP_DantePawn.BP_DantePawn_C|SetIsHiding _as_bp_dante_pawn false)
  (Variables|Default|SetisActive false)
  (Input|DisableInput (Game|GetPlayerController 0))
  (Transformation|Teleport _as_bp_dante_pawn (Transformation|GetWorldLocation (Variables|Default|GetExitDirection)) "0, 0, 0")
  (Class|AIPerceptionStimuliSourceComponent|RegisterwithPerceptionSystem (Variables|/Game/Dante/Blueprint/BP_DantePawn.BP_DantePawn_C|GetAIPerceptionStimuliSource _as_bp_dante_pawn))
  (Transformation|SetWorldRotation (Variables|/Game/Dante/Blueprint/BP_DantePawn.BP_DantePawn_C|GetTorchDirection _as_bp_dante_pawn) (Math|Rotator|MakeRotator 0.0 0.0 0.0) false true)
  (Transformation|SetWorldRotation (Variables|/Game/Dante/Blueprint/BP_DantePawn.BP_DantePawn_C|GetFirstPersonCamera _as_bp_dante_pawn) (Math|Rotator|MakeRotator 0.0 0.0 0.0) false true)
  (Transformation|SetActorRotation _as_bp_dante_pawn (Math|Rotator|MakeRotator 0.0 0.0 (- (.yaw (Transformation|GetActorRotation)) (.yaw (Transformation|GetActorRotation _as_bp_dante_pawn)))) true)
  (Game|Player|SetViewTargetwithBlend (Game|GetPlayerController 0) _as_bp_dante_pawn 0.0 "VTBlend_Linear" 0.0 false)
  (Variables|/Game/Dante/Blueprint/BP_DantePawn.BP_DantePawn_C|SetCurrentHidingSpot _as_bp_dante_pawn 0)
  (Transformation|SetRelativeRotation (Variables|Default|GetHidingCamera) (Transformation|GetActorRotation) false false)
  (Variables|Default|SetX 0.0)
  (Variables|Default|SetY 0.0)
  (Input|DisableInput (Game|GetPlayerController 0))
  (Variables|/Game/Dante/Blueprint/BP_DantePawn.BP_DantePawn_C|SetCanMove _as_bp_dante_pawn true))

(event Custom|Destroy
  (Components|StaticMesh|SetStaticMesh (Variables|Default|GetStaticMesh) "/Game/Dante/Meshes/SM_HidingClosetDestroyed.SM_HidingClosetDestroyed")
  (Collision|SetCollisionEnabled (Variables|Default|GetBox) "NoCollision")
  (Class|AIPerceptionStimuliSourceComponent|UnregisterfromPerceptionSystem (Variables|Default|GetAIPerceptionStimuliSource))
  (Audio|PlaySoundatLocation "/Game/Dante/Blueprint/Audio/wood-smash-2-170417.wood-smash-2-170417" (Transformation|GetActorLocation) "0, 0, 0" 1.0 1.0 0.0 "/Game/Dante/Blueprint/Audio/GenericSoundAttenuation.GenericSoundAttenuation" 0 0 0))

(event EventBeginPlay
  (|CallParentFunction) ; This node is disabled and will not be called.\nDrag off pins to build functionality.
)

(event Collision|EventActorBeginOverlap
  (params (OtherActor :type Actor%20Object%20Reference)))

(event EventTick
  (params (DeltaSeconds :type Float%20%28single-precision%29))
  (|CallParentFunction DeltaSeconds)
  (if (Variables|Default|GetisActive)
    (bind _output_get (Variables|Default|SetX (Math|Float|Clamp(Float) (+ (Variables|Default|GetX) (Class|Actor|GetInputAxisKeyValue)) -3e+01 3e+01)))
    (bind _output_get_2 (Variables|Default|SetY (Math|Float|Clamp(Float) (+ (Variables|Default|GetY) (Class|Actor|GetInputAxisKeyValue)) -2e+01 2e+01)))
    (Transformation|SetRelativeRotation (Variables|Default|GetHidingCamera) (Math|Rotator|MakeRotator 0.0 _output_get_2 _output_get) false false)))

(event EventInteract
  (bind _self self)
  (bind _as_bp_dante_pawn (Variables|Default|GetAs%20BP%20Dante%20Pawn))
  ;[1 1 1] Enter Hiding Place
  ;[0 0.6928 1] Interaction Logic
  (Variables|/Game/Dante/Blueprint/BP_DantePawn.BP_DantePawn_C|SetCanMove _as_bp_dante_pawn false)
  (Variables|Default|SetisActive true)
  (Variables|/Game/Dante/Blueprint/BP_DantePawn.BP_DantePawn_C|SetIsHiding _as_bp_dante_pawn true)
  (Variables|/Game/Dante/Blueprint/BP_DantePawn.BP_DantePawn_C|SetCurrentHidingSpot _as_bp_dante_pawn _self)
  (Game|Player|SetViewTargetwithBlend (Game|GetPlayerController 0) _self 0.0 "VTBlend_Linear" 0.0 false)
  (if (not (Variables|/Game/Dante/Blueprint/BP_DantePawn.BP_DantePawn_C|GetisSpotted _as_bp_dante_pawn))
    (Class|AIPerceptionStimuliSourceComponent|UnregisterfromPerceptionSystem (Variables|/Game/Dante/Blueprint/BP_DantePawn.BP_DantePawn_C|GetAIPerceptionStimuliSource _as_bp_dante_pawn))
    (Default|TeleporttoSafeZone _as_bp_dante_pawn "0, 0, 0")
    (Transformation|SetActorRotation _as_bp_dante_pawn "0, 0, 0" true)
    (Input|EnableInput (Game|GetPlayerController 0))))

(event Input|KeyboardEvents|F
  (params (Key :type Key%20Structure :default "None"))
  ;[0 0.6928 1] Interaction Logic
  ;;[1 1 1] Exit Hiding Place
)

(fn ConstructionScript
  (|CallParentFunction))