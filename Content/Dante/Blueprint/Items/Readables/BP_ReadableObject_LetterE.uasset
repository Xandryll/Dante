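; Readable item Blueprint (LetterE) that tints its book-material mesh when play begins.
; After the parent BeginPlay, it creates a dynamic instance of M_Book_Inst on material slot 0 of StaticMesh.
; The instance's Color parameter gets a random RGB value when RandomColor is set, otherwise BookColor.
; The construction script only calls its parent, and no reading logic is defined here.
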(event EventBeginPlay
  (bind _staticmesh (Variables|Default|GetStaticMesh))
  (|CallParentFunction)
  (bind _returnvalue (Rendering|Material|CreateDynamicMaterialInstance _staticmesh 0 "/Game/Dante/Meshes/M_Book_Inst.M_Book_Inst" "None" :!class /Script/Engine.PrimitiveComponent))
  (Rendering|Material|SetMaterial _staticmesh 0 _returnvalue)
  (Rendering|Material|SetVectorParameterValue _returnvalue "Color" (select (Variables|Parameters|Readable|GetRandomColor) (Utilities|Struct|MakeLinearColor (Math|Random|RandomFloatinRange 0.0 1.0) (Math|Random|RandomFloatinRange 0.0 1.0) (Math|Random|RandomFloatinRange 0.0 1.0) 1.0) (Math|Conversions|ToLinearColor(Color) (Variables|Parameters|Readable|GetBookColor))) :!class /Script/Engine.MaterialInstanceDynamic))

(event Collision|EventActorBeginOverlap
  (params (OtherActor :type Actor%20Object%20Reference))
  (|CallParentFunction OtherActor) ; This node is disabled and will not be called.\nDrag off pins to build functionality.
)

(event EventTick
  (params (DeltaSeconds :type Float%20%28single-precision%29))
  (|CallParentFunction DeltaSeconds) ; This node is disabled and will not be called.\nDrag off pins to build functionality.
)

(fn ConstructionScript
  (|CallParentFunction))