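; BP_DiveUpItem is an interactable pickup that adds its item amount to the first-person character's DiveUp item count.
; BeginPlay caches the player character, and box overlaps send it in-range and out-of-range messages with debug prints, without checking which actor overlapped.
; Interact calls DestroyActor, then increments the count and writes it directly to the character's HUD text.
; The ItemInRange function is an empty stub.
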(event OnComponentBeginOverlap(Box)
  (params (OverlappedComponent :type Primitive%20Component%20Object%20Reference) (OtherActor :type Actor%20Object%20Reference) (OtherComp :type Primitive%20Component%20Object%20Reference) (OtherBodyIndex :type Integer) (bFromSweep :type Boolean) (SweepResult :type Hit%20Result%20Structure%20%28by%20ref%29))
  (if true
    (Class|BPIDante|IteminRange(Message) (Variables|Default|GetAs%20BP%20First%20Person%20Character) self (Variables|Default|GetItemName))
    (Development|PrintString "In")))

(event OnComponentEndOverlap(Box)
  (params (OverlappedComponent :type Primitive%20Component%20Object%20Reference) (OtherActor :type Actor%20Object%20Reference) (OtherComp :type Primitive%20Component%20Object%20Reference) (OtherBodyIndex :type Integer))
  (if true
    (Class|BPIDante|ItemOutOfRange(Message) (Variables|Default|GetAs%20BP%20First%20Person%20Character))
    (Development|PrintString "Out")))

(event EventBeginPlay
  (bind _asbp_first_person_character (Utilities|Casting|CastToBP_FirstPersonCharacter (Game|Player|GetPlayerPawn 0)))
  (Variables|Default|SetAs%20BP%20First%20Person%20Character _asbp_first_person_character))

(event Collision|EventActorBeginOverlap
  (params (OtherActor :type Actor%20Object%20Reference)))

(event EventTick
  (params (DeltaSeconds :type Float%20%28single-precision%29)))

(event EventInteract
  (bind _as_bp_first_person_character (Variables|Default|GetAs%20BP%20First%20Person%20Character))
  (Actor|DestroyActor)
  (bind _output_get (Variables|/Game/FirstPerson/Blueprints/BP_FirstPersonCharacter.BP_FirstPersonCharacter_C|SetItem_DiveUp _as_bp_first_person_character (+ (Variables|/Game/FirstPerson/Blueprints/BP_FirstPersonCharacter.BP_FirstPersonCharacter_C|GetItem_DiveUp _as_bp_first_person_character) (Variables|Default|GetItemAmount))))
  (Variables|/Script/UMG.EditableText|SetText (Variables|/Game/Dante/Blueprint/WB_Hud.WB_Hud_C|Gettxt_DiveUpItems (Variables|/Game/FirstPerson/Blueprints/BP_FirstPersonCharacter.BP_FirstPersonCharacter_C|GetWB_Hud _as_bp_first_person_character)) (Utilities|Text|ToText(Integer) _output_get)))

(fn ConstructionScript)

(fn IteminRange
  (params (Item :type Actor%20Object%20Reference) (Name :type String)))