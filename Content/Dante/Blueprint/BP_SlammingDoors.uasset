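; Door actor for the Dante game that swings and slams with a sound until the player dives.
; SlamDoors binds to the Dante pawn's OnDive event and plays a timeline fed a random value.
; The timeline drives the pivot's yaw across a quarter turn, with an event track playing the closing sound at the actor.
; On dive, the timeline stops, has its time set, and the pivot snaps back to zero rotation.
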(event Custom|SlamDoors
  (bind _asbp_dante_pawn (Utilities|Casting|CastToBP_DantePawn (Game|Player|GetPlayerPawn 0)))
  (EventDispatchers|BindEventtoOnDive _asbp_dante_pawn (delegate Custom|CustomEvent))
  (bind _output_get (Variables|Default|SetNewVar (Math|Random|RandomFloatinRange 0.0 1.0)))
  (bind _newtrack_0 (Timeline|Timeline Play)
    (:Update
      (Transformation|SetRelativeRotation (Variables|Default|GetDoorPivot) (Math|Rotator|MakeRotator 0.0 0.0 (Math|Float|Lerp 0.0 9e+01 _newtrack_0)) false false))
    (:Event
      (Audio|PlaySoundatLocation "/Game/Dante/Audio/closedoor.closedoor" (Transformation|GetActorLocation) "0, 0, 0" 1.0 1.0 0.0 0 0 0 0))))

(event Custom|CustomEvent
  (Utilities|FlowControl|Sequence
    (:then_0
      (bind _newtrack_0 (Timeline|Timeline Stop)
        (:Update
          (Transformation|SetRelativeRotation (Variables|Default|GetDoorPivot) (Math|Rotator|MakeRotator 0.0 0.0 (Math|Float|Lerp 0.0 9e+01 _newtrack_0)) false false))
        (:Event
          (Audio|PlaySoundatLocation "/Game/Dante/Audio/closedoor.closedoor" (Transformation|GetActorLocation) "0, 0, 0" 1.0 1.0 0.0 0 0 0 0))))
    (:then_1
      (Timeline|Timeline SetNewTime))
    (:then_2
      (Transformation|SetRelativeRotation (Variables|Default|GetDoorPivot) (Math|Rotator|MakeRotator 0.0 0.0 0.0) false false))))

(event EventBeginPlay)

(event Collision|EventActorBeginOverlap
  (params (OtherActor :type Actor%20Object%20Reference)))

(event EventTick
  (params (DeltaSeconds :type Float%20%28single-precision%29)))

(fn ConstructionScript)