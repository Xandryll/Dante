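; BP_Enemy is a patrolling AI enemy configured by a data asset for mesh, animation, speeds and dialogue.
; BeginPlay caches spline waypoints and starts a StateTree; one enemy type disables sight and periodically speaks to a nearby player.
; AI Perception tracks the sighted player and last sound, while a polling timer triggers Engage on target-count changes.
; An overlap box reports range to other actors; GrabandDive stuns the enemy and tags it "Caller".
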(event OnComponentBeginOverlap(Box)
  (params (OverlappedComponent :type Primitive%20Component%20Object%20Reference) (OtherActor :type Actor%20Object%20Reference) (OtherComp :type Primitive%20Component%20Object%20Reference) (OtherBodyIndex :type Integer) (bFromSweep :type Boolean) (SweepResult :type Hit%20Result%20Structure%20%28by%20ref%29))
  ;[1 1 1] GrabAndDive Logic
  (Class|BPIDante|EnemyinRange(Message) OtherActor self true))

(event OnComponentEndOverlap(Box)
  (params (OverlappedComponent :type Primitive%20Component%20Object%20Reference) (OtherActor :type Actor%20Object%20Reference) (OtherComp :type Primitive%20Component%20Object%20Reference) (OtherBodyIndex :type Integer))
  ;[1 1 1] GrabAndDive Logic
  (Class|BPIDante|EnemyinRange(Message) OtherActor self false))

(event OnTargetPerceptionUpdated(AIPerception)
  (params (Actor :type Actor%20Object%20Reference) (Stimulus :type AI%20Stimulus%20Structure))
  ;[1 1 1] Perception system
  (CallFunction|AIPerceptionUpdateTargets Actor Stimulus))

(event OnTargetPerceptionForgotten(AIPerception)
  (params (Actor :type Actor%20Object%20Reference))
  ;[1 1 1] Perception system
  (CallFunction|AIPerceptionRemoveLostTargets Actor))

(event Custom|Speak
  (bind _returnvalue (Game|Player|GetPlayerPawn 0))
  (bind _enemyda (Variables|Setup|GetEnemyDA))
  ;[1 1 1] Initialize
  (if (<= (Math|Vector|Distance(Vector) (Transformation|GetActorLocation) (Transformation|GetActorLocation _returnvalue)) 1e+03)
    (Class|BPIDante|ShowDialogue(Message) _returnvalue (Variables|/Game/Dante/Blueprint/PDAs/PDA_Enemy.PDA_Enemy_C|GetName _enemyda) (Utilities|Array|Get(acopy) (Variables|/Game/Dante/Blueprint/PDAs/PDA_Enemy.PDA_Enemy_C|GetPhrase _enemyda) (Variables|/Game/Dante/Blueprint/BP_DanteGameMode.BP_DanteGameMode_C|GetDive_Level (Variables|Internal|GetAs%20BP%20Dante%20Game%20Mode))))))

(event Custom|Alert
  (params (Value :type Text%20%28by%20ref%29))
  (Rendering|Components|TextRender|SetText (Variables|Default|GetAlertText self) Value))

(event Custom|Engage
  ;[1 1 1] Engage
  (bind (_actor _stimulus _issight) (CallFunction|GetCurrentTarget))
  (if _issight
    (if (== (Utilities|GetClass _actor) "/Game/Dante/Blueprint/BP_DantePawn.BP_DantePawn_C")
      (Class|BPIDante|SpottedonSight(Message) _actor self true)
      (Variables|Internal|SetisPlayerSpotted true)
      (Variables|Internal|SetTargetActor _actor :!label _label)
      (elif (Actor|ActorHasTag _actor "Caller")
        (goto _label)))
    (else
      (CallFunction|AIPerceptionRemoveLostTargets _actor)
      (Variables|Internal|SetStimulus%20Location (.StimulusLocation (Utilities|Struct|BreakAIStimulus _stimulus))))))

(event Custom|Opponents%20Handeling
  (bind _targetactors (Variables|Default|GetTargetActors))
  (bind _returnvalue (Utilities|Array|Length _targetactors))
  ;[1 1 1] Initialize
  (if (!= (Variables|Default|GetOpponentsAmount) _returnvalue)
    (bind _output_get (Variables|Default|SetOpponentsAmount _returnvalue))
    (if (!= _output_get 0)
      (CallFunction|Engage))))

(event Custom|Investigate
  (AI|AIMoveTo self (Variables|Internal|GetStimulus%20Location) 0 5e+01 false))

(event EventBeginPlay
  (bind _mesh (Variables|Character|GetMesh))
  (bind _patrolspline (Variables|Default|GetPatrolSpline))
  (bind _enemyda (Variables|Setup|GetEnemyDA))
  (bind _animinstance (Variables|/Game/Dante/Blueprint/PDAs/PDA_Enemy.PDA_Enemy_C|GetAnimInstance _enemyda))
  (bind _skeletalmesh (Variables|/Game/Dante/Blueprint/PDAs/PDA_Enemy.PDA_Enemy_C|GetSkeletalMesh _enemyda))
  ;[1 1 1] Initialize
  (Utilities|FlowControl|Sequence
    (:then_0
      (bind _asbp_dante_game_mode (Utilities|Casting|CastToBP_DanteGameMode (Game|GetGameMode)))
      (Variables|Internal|SetAs%20BP%20Dante%20Game%20Mode _asbp_dante_game_mode)
      (bind _asbp_dante_pawn (Utilities|Casting|CastToBP_DantePawn (Game|Player|GetPlayerPawn 0)))
      (Variables|Default|SetAs%20BP%20Dante%20Pawn _asbp_dante_pawn)
      (Utilities|FlowControl|Delay 1.0)
      (for _index (range 0 (- (Spline|GetNumberOfSplinePoints _patrolspline) 1))
        (Utilities|Array|Add (Variables|Internal|GetWaypoints) (Spline|GetLocationatSplinePoint _patrolspline _index "World")))
      (if (not (or (Utilities|IsValid _skeletalmesh) (Utilities|IsValidClass _animinstance)))
        (Components|SkeletalMesh|SetSkeletalMeshAsset _mesh "/Game/Characters/Mannequins/Meshes/SKM_Quinn.SKM_Quinn")
        (Class|SkeletalMeshComponent|SetAnimClass _mesh "/Game/Characters/Mannequins/Animations/ABP_Quinn.ABP_Quinn_C")
        (else
          (Components|SkeletalMesh|SetSkeletalMeshAsset _mesh _skeletalmesh)
          (Class|SkeletalMeshComponent|SetAnimClass _mesh _animinstance)))
      (if (Utilities|Enum|Equal(Enum) (Variables|/Game/Dante/Blueprint/PDAs/PDA_Enemy.PDA_Enemy_C|GetEnemyType (Variables|Setup|GetEnemyDA)) "NewEnumerator2")
        (Class|AIPerceptionComponent|SetSenseEnabled (Variables|Default|GetAIPerception) "/Script/AIModule.AISense_Sight" false)
        (Utilities|Time|SetTimerbyEvent (delegate Custom|Speak) 1e+01 true))
      (CallFunction|ChangeSpeed)
      (AI|Logic|StartLogic (Variables|Default|GetStateTree))
      (Utilities|Time|SetTimerbyEvent (delegate Custom|Opponents%20Handeling) 0.1 true))))

(event EventTick
  (params (DeltaSeconds :type Float%20%28single-precision%29))
  (bind _returnvalue (Game|Player|GetPlayerPawn 0))
  (bind _debugtext (Variables|Default|GetDebugText))
  (bind _targetactors (Variables|Default|GetTargetActors))
  (bind _returnvalue_2 (Utilities|Array|Length _targetactors))
  (bind _returnvalue_3 (Transformation|GetWorldTransform _debugtext))
  (bind _returnvalue_4 (Transformation|GetActorLocation _returnvalue))
  (bind _returnvalue_5 (Class|KismetAnimationLibrary|Lookat _returnvalue_3 _returnvalue_4 "1.000000,0.000000,0.000000" false "0.000000,0.000000,1.000000" 0.0))
  ;[1 1 1] Tick Logic
  (Utilities|FlowControl|Sequence
    (:then_0
      (Transformation|SetWorldTransform _debugtext (Math|Transform|MakeTransform (.location _returnvalue_5) (Math|Rotator|MakeRotator 0.0 0.0 (.yaw (.rotation _returnvalue_5))) (.scale _returnvalue_5)) false false))
    (:then_1
      ;[1 1 1] PerceptionDebug
      (if (Variables|Default|GetDebugAiPerception)
        (Development|PrintString (Utilities|String|Append "ActorsNum: " (Utilities|String|ToString(Integer) _returnvalue_2) " - StimulusNum: " (Utilities|String|ToString(Integer) (Utilities|Array|Length (Variables|Default|GetTargetStimulus)))))
        (for _array_element _targetactors
          (Development|PrintString (Utilities|String|Append "Actor: " (Utilities|GetDisplayName _array_element))))
        (Utilities|FlowControl|Sequence
          (:then_0
            (if (!= _returnvalue_2 0)
              (Development|PrintString (Utilities|String|Append "Priority: " (Utilities|GetDisplayName (Utilities|Array|Get(acopy) _targetactors))))))
          (:then_1
            (Development|PrintString "--------------------")))))))

(event EventGrabandDive
  (Variables|Default|SetgotDived true)
  (Variables|Internal|SetisStunned true)
  (Variables|Default|SetTags (Utilities|Array|MakeArray "Caller")))

(event EventAttackTarget
  (Variables|Default|SetTags (Utilities|Array|MakeArray "None"))
  (Actor|DestroyActor))

(fn ConstructionScript)

(fn ChangeSpeed
  (bind _enemyda (Variables|Setup|GetEnemyDA))
  (bind _charactermovement (Variables|Character|GetCharacterMovement))
  (switch Utilities|FlowControl|Switch|SwitchonEn_EnemyStates (Variables|Internal|GetEnemyState)
    (:NewEnumerator0
      (Variables|/Script/Engine.CharacterMovementComponent|SetMaxWalkSpeed _charactermovement (Variables|/Game/Dante/Blueprint/PDAs/PDA_Enemy.PDA_Enemy_C|GetPatrolSpeed _enemyda)))
    (:NewEnumerator1
      (Variables|/Script/Engine.CharacterMovementComponent|SetMaxWalkSpeed _charactermovement (Variables|/Game/Dante/Blueprint/PDAs/PDA_Enemy.PDA_Enemy_C|GetEngageSpeed _enemyda)))))

(fn AIPerceptionUpdateTargets
  (params (Actor :type Actor%20Object%20Reference%20%28by%20ref%29) (Stimulus :type AI%20Stimulus%20Structure%20%28by%20ref%29))
  (bind (_age _expirationage _strength _stimuluslocation _receiverlocation _tag _bsuccessfullysensed) (Utilities|Struct|BreakAIStimulus Stimulus))
  (bind _returnvalue (Class|AIPerceptionSystem|GetSenseClassforStimulus Stimulus))
  (if (== _returnvalue "/Script/AIModule.AISense_Sight")
    (if (Math|Boolean|ANDBoolean (!= Actor self) _bsuccessfullysensed (not (Utilities|Array|ContainsItem (Variables|Default|GetTargetActors) Actor)) (== (Utilities|GetClass Actor) "/Game/Dante/Blueprint/BP_DantePawn.BP_DantePawn_C"))
      (Development|PrintString (Utilities|String|Append "Sensed Actor:" (Utilities|GetDisplayName Actor) " - Stimulus: " (Utilities|String|ToString(Vector) _stimuluslocation) " - Tag: " (Utilities|String|ToString(Name) _tag) (Utilities|String|ToString(Boolean) _bsuccessfullysensed)))
      (LocalVariables|SetTempActor Actor)
      (LocalVariables|SetTempStimulus Stimulus)
      (Utilities|Array|Add (Variables|Default|GetTargetActors) (LocalVariables|GetTempActor))
      (Utilities|Array|Add (Variables|Default|GetTargetStimulus) (LocalVariables|GetTempStimulus))
      (Rendering|Components|TextRender|SetText (Variables|Default|GetAlertText) (Utilities|Text|MakeLiteralText "!"))
      (return))
    (else
      (Variables|Default|SetTargetAudioLocation (.StimulusLocation (Utilities|Struct|BreakAIStimulus Stimulus)))
      (Variables|Default|SetTargetAudioActor Actor))))

(fn AIPerceptionRemoveLostTargets
  (params (Actor :type Actor%20Object%20Reference%20%28by%20ref%29))
  (bind _returnvalue (Utilities|GetClass Actor))
  (bind _targetactors (Variables|Default|GetTargetActors))
  (bind _returnvalue_2 (== _returnvalue "/Game/Dante/Blueprint/BP_DantePawn.BP_DantePawn_C"))
  (if (or _returnvalue_2 (== _returnvalue "BP_Enemy_C"))
    (if _returnvalue_2
      (Default|SpottedonSight (Variables|Default|GetAs%20BP%20Dante%20Pawn) self false))
    (Utilities|Array|RemoveIndex (Variables|Default|GetTargetStimulus) (Utilities|Array|FindItem _targetactors Actor))
    (Utilities|Array|RemoveItem _targetactors Actor)
    (Variables|Default|SetTauntPerformed false)
    (Rendering|Components|TextRender|SetText (Variables|Default|GetAlertText) (Utilities|Text|MakeLiteralText " "))
    (Development|PrintString "LOST")
    (return)
    (else
      (Variables|Default|SetTargetAudioLocation "0, 0, 0")
      (Variables|Default|SetTargetAudioActor 0)
      (Development|PrintString "Audio deleted"))))

(fn CheckOpponents
  (bind _targetactors (Variables|Default|GetTargetActors))
  (bind _returnvalue (Utilities|Array|Length _targetactors))
  (if (!= (Variables|Default|GetOpponentsAmount) _returnvalue)
    (bind _output_get (Variables|Default|SetOpponentsAmount _returnvalue))
    (CallFunction|Engage)
    (return _output_get)))

(fn GetCurrentTarget
  (bind _targetactors (Variables|Default|GetTargetActors))
  (bind _targetstimulus (Variables|Default|GetTargetStimulus))
  (bind _output (Utilities|Array|Get(acopy) _targetstimulus))
  (if (> (Utilities|Array|Length _targetactors) 0)
    (bind _returnvalue (Class|AIPerceptionSystem|GetSenseClassforStimulus _output))
    (return (Utilities|Array|Get(acopy) _targetactors) _output (== _returnvalue "/Script/AIModule.AISense_Sight"))))

(fn OnBoolChangeTick
  (params (Condition :type Boolean))
  (if (not (== Condition (LocalVariables|GetTempBool)))
    (bind _output_get (LocalVariables|SetTempBool Condition))
    (Development|PrintString (Utilities|String|Append "Changed state to: " (Utilities|String|ToString(Boolean) _output_get)))
    (return)))