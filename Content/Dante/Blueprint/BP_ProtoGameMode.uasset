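; Prototype game mode that manages stacked dive levels and a global countdown for the Dante pawn.
; On BeginPlay it copies streamed levels, per-level settings and the timer from the first BP_HoldingZone's PDALevel data, then loads the first level.
; A looping timer drains the clock by the current level's time dilation, updating the HUD and killing the pawn at zero.
; ChangeLevel swaps streamed levels, ends the dive, broadcasts the change and updates dive limits.
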(event Custom|ChangeLevel
  (params (DiveDown? :type Boolean))
  (bind _as_bp_dante_pawn (Variables|Internal|GetAs%20BP%20Dante%20Pawn))
  (bind _levels (Variables|Internal|GetLevels))
  ;[1 1 1] Change Dive Lvels Logic
  (Utilities|FlowControl|Sequence
    (:then_0
      (if DiveDown?
        (Variables|Internal|SetDive_PrevLevel (Variables|Internal|GetDive_Level))
        (bind _result (Math|Integer|IncrementInt (Variables|Internal|GetDive_Level))
          (:%20%20
            (if (> _result (Utilities|Array|LastIndex (Variables|Internal|GetLevels)))
              (Variables|Internal|SetDive_Level 0))))
        (else
          (Variables|Internal|SetDive_PrevLevel (Variables|Internal|GetDive_Level))
          (bind _result_2 (Math|Integer|DecrementInt (Variables|Internal|GetDive_Level))
            (:%20%20
              (if (< _result_2 0)
                (Variables|Internal|SetDive_Level (Utilities|Array|LastIndex (Variables|Internal|GetLevels))))))))
      (Class|GameplayStatics|UnloadStreamLevelbySoftObjectPtr (Utilities|Array|Get(acopy) _levels (Variables|Internal|GetDive_PrevLevel)) false)
      (Class|GameplayStatics|LoadStreamLevelbySoftObjectPtr (Utilities|Array|Get(acopy) _levels (Variables|Internal|GetDive_Level)) true false)
      (Default|EndDive (Variables|Internal|GetAs%20BP%20Dante%20Pawn))
      (Default|CallDiveChangeLevel))
    (:then_1
      (Utilities|FlowControl|Sequence
        (:then_0
          (if (== (Variables|Internal|GetDive_Level) (Utilities|Array|LastIndex (Variables|Internal|GetLevels)))
            (Variables|/Game/Dante/Blueprint/BP_DantePawn.BP_DantePawn_C|SetCanDiveDown _as_bp_dante_pawn false)
            (else
              (Variables|/Game/Dante/Blueprint/BP_DantePawn.BP_DantePawn_C|SetCanDiveDown _as_bp_dante_pawn true))))
        (:then_1
          (if (== 0 (Variables|Internal|GetDive_Level))
            (Variables|/Game/Dante/Blueprint/BP_DantePawn.BP_DantePawn_C|SetCanDiveUp _as_bp_dante_pawn false)))))))

(event Custom|UpdateClock
  ;[1 1 1] Global timer
  (bind _output_get (Variables|Internal|SetGlobalTimer (- (Variables|Internal|GetGlobalTimer) (* (Utilities|Array|Get(acopy) (Variables|Internal|GetDive_LevelsTimeDilatation) (Variables|Internal|GetDive_Level)) (Variables|Setup|GetTimeTimerTick)))))
  (if (<= _output_get 0.0)
    (Class|BPIDante|KillActor(Message) (Variables|Internal|GetAs%20BP%20Dante%20Pawn))
    (else
      (Variables|/Script/UMG.EditableText|SetText (Variables|/Game/Dante/Blueprint/HUD/WB_Hud.WB_Hud_C|Gettxt_globalTimer (Variables|Internal|GetWB%20Hud)) (Class|KismetTextLibrary|AsTimespanTimespan (Math|Timespan|FromSeconds _output_get))))))

(event EventBeginPlay
  ;[1 1 1] Initialize
  (Utilities|FlowControl|Sequence
    (:then_0
      (Utilities|Array|Clear (Variables|Internal|GetLevels))
      (Utilities|Array|Clear (Variables|Internal|GetDive_LevelsTimerDuration))
      (Utilities|Array|Clear (Variables|Internal|GetDive_LevelsTimeDilatation))
      (bind _asbp_dante_pawn (Utilities|Casting|CastToBP_DantePawn (Game|Player|GetPlayerPawn 0)))
      (Variables|Internal|SetAs%20BP%20Dante%20Pawn _asbp_dante_pawn)
      (bind _outactors (Actor|GetAllActorsOfClass "/Game/Dante/Blueprint/Items/BP_HoldingZone.BP_HoldingZone_C"))
      (Variables|Setup|SetPDA_Levels (Variables|/Game/Dante/Blueprint/Items/BP_HoldingZone.BP_HoldingZone_C|GetPDA_Level (Utilities|Array|Get(acopy) _outactors))))
    (:then_1
      (bind (_array_element _array_index) (Utilities|Array|ForEachLoopwithBreak (Variables|/Game/Dante/Blueprint/PDAs/PDA_Levels.PDA_Levels_C|GetLevels (Variables|Setup|GetPDA_Levels)))
        (:LoopBody
          (Utilities|Array|Add (Variables|Internal|GetLevels) (Utilities|Struct|BreakSoftWorldReference _array_element))
          (Utilities|Array|Add (Variables|Internal|GetDive_LevelsTimerDuration) (Utilities|Array|Get(acopy) (Variables|/Game/Dante/Blueprint/PDAs/PDA_Levels.PDA_Levels_C|GetDive_LevelsTimerDuration (Variables|Setup|GetPDA_Levels)) _array_index))
          (Utilities|Array|Add (Variables|Internal|GetDive_LevelsTimeDilatation) (Utilities|Array|Get(acopy) (Variables|/Game/Dante/Blueprint/PDAs/PDA_Levels.PDA_Levels_C|GetDive_LevelsTimeDilatation (Variables|Setup|GetPDA_Levels)) _array_index))
          (Variables|Internal|SetGlobalTimer (Variables|/Game/Dante/Blueprint/PDAs/PDA_Levels.PDA_Levels_C|GetGlobalTimer (Variables|Setup|GetPDA_Levels))))
        (:Completed
          (Class|GameplayStatics|LoadStreamLevelbySoftObjectPtr (Utilities|Array|Get(acopy) (Variables|Internal|GetLevels)) true false)
          (Variables|Internal|SetWB%20Hud (Variables|/Game/Dante/Blueprint/BP_DantePawn.BP_DantePawn_C|GetWB_Hud (Variables|Internal|GetAs%20BP%20Dante%20Pawn)))
          (Utilities|Time|SetTimerbyEvent (delegate Custom|UpdateClock) (Variables|Setup|GetTimeTimerTick) true))))))

(fn ConstructionScript)