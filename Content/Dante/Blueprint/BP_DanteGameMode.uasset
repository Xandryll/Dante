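; Game mode for Dante that runs a timed loop across streamed dive levels with persistent quests and threat.
; BeginPlay reads level data from the holding zone's PDA, spawns the pawn, then restores the save and randomly places powerups, or shows the tutorial.
; A looping timer drains global time at each depth's dilation rate, while diving swaps streamed levels.
; Loop end raises capped threat and saves; five completed quests trigger the end screen.
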(event Custom|ChangeLevel
  (params (DiveDown? :type Boolean))
  (bind _as_bp_dante_pawn (Variables|Internal|GetAs%20BP%20Dante%20Pawn))
  (bind _levels (Variables|Internal|GetLevels))
  ;[1 1 1] Change Dive Levels Logic
  (Utilities|FlowControl|Sequence
    (:then_0
      (if DiveDown?
        (Variables|Internal|SetDive_PrevLevel (Variables|Internal|GetDive_Level))
        (bind _result (Math|Integer|IncrementInt (Variables|Internal|GetDive_Level))
          (:%20%20
            (if (> _result (Utilities|Array|LastIndex (Variables|Internal|GetLevels)))
              (Variables|Internal|SetDive_Level 0))))
        (else
          (Variables|Internal|SetDive_PrevLevel (Variables|Internal|GetDive_Level))
          (bind _result_2 (Math|Integer|DecrementInt (Variables|Internal|GetDive_Level))
            (:%20%20
              (if (< _result_2 0)
                (Variables|Internal|SetDive_Level (Utilities|Array|LastIndex (Variables|Internal|GetLevels))))))))
      (Class|GameplayStatics|UnloadStreamLevelbySoftObjectPtr (Utilities|Array|Get(acopy) _levels (Variables|Internal|GetDive_PrevLevel)) false)
      (Class|GameplayStatics|LoadStreamLevelbySoftObjectPtr (Utilities|Array|Get(acopy) _levels (Variables|Internal|GetDive_Level)) true false)
      (Default|EndDive (Variables|Internal|GetAs%20BP%20Dante%20Pawn))
      (Default|CallDiveChangeLevel))
    (:then_1
      (Utilities|FlowControl|Sequence
        (:then_0
          (if (== (Variables|Internal|GetDive_Level) (Utilities|Array|LastIndex (Variables|Internal|GetLevels)))
            (Variables|/Game/Dante/Blueprint/BP_DantePawn.BP_DantePawn_C|SetCanDiveDown _as_bp_dante_pawn false)
            (else
              (Variables|/Game/Dante/Blueprint/BP_DantePawn.BP_DantePawn_C|SetCanDiveDown _as_bp_dante_pawn true))))
        (:then_1
          (if (== 0 (Variables|Internal|GetDive_Level))
            (Variables|/Game/Dante/Blueprint/BP_DantePawn.BP_DantePawn_C|SetCanDiveUp _as_bp_dante_pawn false)
            (else
              (Variables|/Game/Dante/Blueprint/BP_DantePawn.BP_DantePawn_C|SetCanDiveUp _as_bp_dante_pawn true))))))))

(event Custom|UpdateQuests
  (params (Quest :type En_Quests%20Enum :default "NewEnumerator0"))
  (bind _as_bp_dante_pawn (Variables|Internal|GetAs%20BP%20Dante%20Pawn))
  (bind _completedquests (Variables|Default|GetCompletedQuests))
  (bind _wb_hud (Variables|Internal|GetWB%20Hud))
  (Utilities|Array|AddUnique _completedquests Quest)
  (Variables|Default|SetTempString "")
  (for _array_element _completedquests
    (Variables|Default|SetTempString (Utilities|String|Append (Utilities|String|Append (Variables|Default|GetTempString) (Utilities|String|EnumtoString _array_element)) " 
")))
  (Variables|/Script/UMG.MultiLineEditableText|SetText (Variables|/Game/Dante/Blueprint/HUD/WB_Hud.WB_Hud_C|Gettxt_QuestList _wb_hud) (Utilities|Text|ToText(String) (Variables|Default|GetTempString)))
  (if (== (Utilities|Array|Length _completedquests) 5)
    (Utilities|FlowControl|Delay 3.0)
    (Variables|/Script/UMG.Widget|SetRenderOpacity (Variables|/Game/Dante/Blueprint/HUD/WB_Hud.WB_Hud_C|GetHudBox _wb_hud) 0.0)
    (Variables|/Script/UMG.Widget|SetRenderOpacity (Variables|/Game/Dante/Blueprint/HUD/WB_Hud.WB_Hud_C|GetEndScreen _wb_hud) 1.0)
    (Input|DisableInput _as_bp_dante_pawn (Game|GetPlayerController 0))
    (Utilities|Time|ClearandInvalidateTimerbyHandle (Variables|Default|GetClockTimerHandle))
    (Default|TeleporttoSafeZone _as_bp_dante_pawn "0, 0, 0")))

(event Custom|StartGame
  (Pawn|Possess (Game|GetPlayerController 0) (stale EventBeginPlay _output_get))
  (bind _returnvalue (Utilities|Time|SetTimerbyEvent (delegate Custom|UpdateClock) (Variables|Setup|GetTimeTimerTick) true))
  (Variables|Default|SetClockTimerHandle _returnvalue)
  (Default|CallGameStarted))

(event Custom|UpdateClock
  ;[1 1 1] Global timer
  (bind _output_get (Variables|Internal|SetGlobalTimer (- (Variables|Internal|GetGlobalTimer) (* (Utilities|Array|Get(acopy) (Variables|Internal|GetDive_LevelsTimeDilatation) (Variables|Internal|GetDive_Level)) (Variables|Setup|GetTimeTimerTick)))))
  (if (<= _output_get 0.0)
    (CallFunction|EndLoop false)
    (else
      (Variables|/Script/UMG.EditableText|SetText (Variables|/Game/Dante/Blueprint/HUD/WB_Hud.WB_Hud_C|Gettxt_globalTimer (Variables|Internal|GetWB%20Hud)) (Class|KismetTextLibrary|AsTimespanTimespan (Math|Timespan|FromSeconds _output_get))))))

(event Custom|SavedQuests
  (bind _as_bp_dante_pawn (Variables|Internal|GetAs%20BP%20Dante%20Pawn))
  (bind _completedquests (Variables|Default|GetCompletedQuests))
  (bind _wb_hud (Variables|Internal|GetWB%20Hud))
  (for _array_element _completedquests
    (Variables|Default|SetTempString (Utilities|String|Append (Utilities|String|Append (Variables|Default|GetTempString) (Utilities|String|EnumtoString _array_element)) " 
")))
  (Variables|/Script/UMG.MultiLineEditableText|SetText (Variables|/Game/Dante/Blueprint/HUD/WB_Hud.WB_Hud_C|Gettxt_QuestList _wb_hud) (Utilities|Text|ToText(String) (Variables|Default|GetTempString)))
  (if (== (Utilities|Array|Length _completedquests) 5)
    (Utilities|FlowControl|Delay 3.0)
    (Variables|/Script/UMG.Widget|SetRenderOpacity (Variables|/Game/Dante/Blueprint/HUD/WB_Hud.WB_Hud_C|GetHudBox _wb_hud) 0.0)
    (Variables|/Script/UMG.Widget|SetRenderOpacity (Variables|/Game/Dante/Blueprint/HUD/WB_Hud.WB_Hud_C|GetEndScreen _wb_hud) 1.0)
    (Input|DisableInput _as_bp_dante_pawn (Game|GetPlayerController 0))
    (Utilities|Time|ClearandInvalidateTimerbyHandle (Variables|Default|GetClockTimerHandle))
    (Default|TeleporttoSafeZone _as_bp_dante_pawn "0, 0, 0")))

(event Custom|EndLoop
  (params (DeathByEnemy :type Boolean))
  ;[1 1 1] End loop
  (Default|CallLoopEnd)
  (Utilities|Time|ClearandInvalidateTimerbyHandle (Variables|Default|GetClockTimerHandle))
  (if (< (Variables|Default|GetThreat) (* (Variables|Default|GetThreatPerLevel) (Utilities|Array|LastIndex (.general_timebeforespawning (Variables|/Game/XanWorld/DataAssets/PDA_xEnemy.PDA_xEnemy_C|GetxEnemyConfiguration (Variables|/Game/Dante2/Blueprints/BP_Coordinator.BP_Coordinator_C|GetDA (Variables|Default|GetCoordinatorReference)))))))
    (Math|Integer|IncrementInt (Variables|Default|GetThreat)
      (:%20%20
        _)))
  (bind _returnvalue (SaveGame|CreateSaveGameObject "/Game/Dante/BP_Savegame.BP_Savegame_C"))
  (Variables|/Game/Dante/BP_Savegame.BP_Savegame_C|SetQuests _returnvalue (Variables|Default|GetCompletedQuests))
  (Variables|/Game/Dante/BP_Savegame.BP_Savegame_C|SetThreatLevel _returnvalue (/ (Variables|Default|GetThreat) (Variables|Default|GetThreatPerLevel)))
  (Variables|/Game/Dante/BP_Savegame.BP_Savegame_C|SetThreat _returnvalue (Variables|Default|GetThreat))
  (|AsyncSaveGametoSlot _returnvalue _returnvalue "Dante"
    (:Completed
      (Class|BPIDante|KillActor(Message) (Variables|Internal|GetAs%20BP%20Dante%20Pawn) DeathByEnemy))))

(event Custom|SpawnPowerups
  (bind _itemsto_spawn (Variables|Default|GetItemsTo%20Spawn))
  (for _array_element (Variables|Default|GetItemSpawned)
    (Actor|DestroyActor _array_element))
  (Variables|Default|SetItemSpawnerLocationsTemp (Variables|Default|GetItemSpawnerLocations))
  (for _index (range 0 (Utilities|Array|LastIndex _itemsto_spawn))
    (bind _output_get (Variables|Default|SetTempItemToSpawnLocation (.OutItem (Utilities|Array|Random (Variables|Default|GetItemSpawnerLocationsTemp)))))
    (bind _returnvalue (Game|SpawnActorfromClass (Utilities|Array|Get(acopy) _itemsto_spawn _index) (Math|Conversions|ToTransform(Vector) (Transformation|GetActorLocation _output_get)) "Undefined" "MultiplyWithRoot" 0 0))
    (Utilities|Array|Add (Variables|Default|GetItemSpawned) _returnvalue)
    (Utilities|Array|RemoveItem (Variables|Default|GetItemSpawnerLocationsTemp) _output_get)))

(event EventBeginPlay
  ;[1 1 1] Initialize
  (Utilities|FlowControl|Sequence
    (:then_0
      (Utilities|Array|Clear (Variables|Internal|GetLevels))
      (Utilities|Array|Clear (Variables|Internal|GetDive_LevelsTimerDuration))
      (Utilities|Array|Clear (Variables|Internal|GetDive_LevelsTimeDilatation))
      (bind _outactors (Actor|GetAllActorsOfClass "/Game/Dante/Blueprint/Items/BP_HoldingZone.BP_HoldingZone_C"))
      (Variables|Setup|SetPDA_Levels (Variables|/Game/Dante/Blueprint/Items/BP_HoldingZone.BP_HoldingZone_C|GetPDA_Level (Utilities|Array|Get(acopy) _outactors)))
      (bind _outactors_2 (Actor|GetAllActorsOfClass "/Game/Dante/Blueprint/BP_ItemSpawnerLocation.BP_ItemSpawnerLocation_C"))
      (Variables|Default|SetItemSpawnerLocations _outactors_2))
    (:then_1
      (bind (_array_element _array_index) (Utilities|Array|ForEachLoopwithBreak (Variables|/Game/Dante/Blueprint/PDAs/PDA_Levels.PDA_Levels_C|GetLevels (Variables|Setup|GetPDA_Levels)))
        (:LoopBody
          (Utilities|Array|Add (Variables|Internal|GetLevels) (Utilities|Struct|BreakSoftWorldReference _array_element))
          (Utilities|Array|Add (Variables|Internal|GetDive_LevelsTimerDuration) (Utilities|Array|Get(acopy) (Variables|/Game/Dante/Blueprint/PDAs/PDA_Levels.PDA_Levels_C|GetDive_LevelsTimerDuration (Variables|Setup|GetPDA_Levels)) _array_index))
          (Utilities|Array|Add (Variables|Internal|GetDive_LevelsTimeDilatation) (Utilities|Array|Get(acopy) (Variables|/Game/Dante/Blueprint/PDAs/PDA_Levels.PDA_Levels_C|GetDive_LevelsTimeDilatation (Variables|Setup|GetPDA_Levels)) _array_index))
          (Variables|Internal|SetGlobalTimer (Variables|/Game/Dante/Blueprint/PDAs/PDA_Levels.PDA_Levels_C|GetGlobalTimer (Variables|Setup|GetPDA_Levels))))
        (:Completed
          (Class|GameplayStatics|LoadStreamLevelbySoftObjectPtr (Utilities|Array|Get(acopy) (Variables|Internal|GetLevels)) true true)
          (bind _outactors_3 (Actor|GetAllActorsOfClass "/Game/Dante2/Blueprints/BP_Coordinator.BP_Coordinator_C"))
          (Variables|Default|SetCoordinatorReference (Utilities|Array|Get(acopy) _outactors_3))
          (bind _outactors_4 (Actor|GetAllActorsOfClass "/Game/Dante/Blueprint/Items/BP_BaseItem.BP_BaseItem_C"))
          (for _array_element_2 _outactors_4
            (if (Variables|/Game/Dante/Blueprint/Items/BP_BaseItem.BP_BaseItem_C|GetIsClue _array_element_2)
              (Utilities|Array|AddUnique (Variables|Default|GetCluesList) _array_element_2)))
          (bind _outactors_5 (Actor|GetAllActorsOfClass "/Script/Engine.PlayerStart"))
          (bind _returnvalue (Game|SpawnActorfromClass "/Game/Dante/Blueprint/BP_DantePawn.BP_DantePawn_C" (Math|Conversions|ToTransform(Vector) (Transformation|GetActorLocation (Utilities|Array|Get(acopy) _outactors_5))) "Undefined" "MultiplyWithRoot" 0 0))
          (bind _output_get (Variables|Internal|SetAs%20BP%20Dante%20Pawn _returnvalue))
          (Variables|Internal|SetWB%20Hud (Variables|/Game/Dante/Blueprint/BP_DantePawn.BP_DantePawn_C|GetWB_Hud _output_get))
          (bind _returnvalue_2 (SaveGame|DoesSaveGameExist "Dante"))
          (if _returnvalue_2
            (bind _savegame (|AsyncLoadGamefromSlot "Dante")
              (:Completed
                (bind _asbp_savegame (Utilities|Casting|CastToBP_Savegame _savegame)
                  (:then
                    (Variables|Default|SetCompletedQuests (Variables|/Game/Dante/BP_Savegame.BP_Savegame_C|GetQuests _asbp_savegame))
                    (Variables|Default|SetThreatLevel (Variables|/Game/Dante/BP_Savegame.BP_Savegame_C|GetThreatLevel _asbp_savegame))
                    (Variables|Default|SetThreat (Variables|/Game/Dante/BP_Savegame.BP_Savegame_C|GetThreat _asbp_savegame))
                    (CallFunction|SavedQuests)
                    (CallFunction|SpawnPowerups)
                    (CallFunction|StartGame))
                  (:CastFailed
                    (Development|PrintString "save failed")))))
            (else
              (Default|ShowTutorial (Variables|Internal|GetWB%20Hud) true)
              (Variables|Default|SetThreatLevel 0)
              (Variables|Default|SetThreat 0)
              (bind _returnvalue_3 (SaveGame|CreateSaveGameObject "/Game/Dante/BP_Savegame.BP_Savegame_C"))
              (Variables|/Game/Dante/BP_Savegame.BP_Savegame_C|SetFirstStart _returnvalue_3 true)
              (|AsyncSaveGametoSlot _returnvalue_3 _returnvalue_3 "Dante"))))))))

(fn ConstructionScript)