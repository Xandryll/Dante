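; BP_PhysicItem is a prop the player can knock over, creating noise on landing.
; Box overlap rolls a drop chance indexed by the Dante pawn's movement type (walk, run, crouch), then enables mesh physics and applies an impulse at the arrow.
; The mesh's first hit on a Floor-tagged actor reports a range-limited noise event at the impact point.
; BeginPlay caches the pawn and fires a delayed debug noise at a hardcoded location.
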(event OnComponentBeginOverlap(Box)
  (params (OverlappedComponent :type Primitive%20Component%20Object%20Reference) (OtherActor :type Actor%20Object%20Reference) (OtherComp :type Primitive%20Component%20Object%20Reference) (OtherBodyIndex :type Integer) (bFromSweep :type Boolean) (SweepResult :type Hit%20Result%20Structure%20%28by%20ref%29))
  (bind _as_bp_dante_pawn (Variables|Default|GetAs%20BP%20Dante%20Pawn))
  (bind _staticmesh (Variables|Default|GetStaticMesh))
  (if (< (Math|Random|RandomFloatinRange 0.0 1e+02) (Utilities|Array|Get(acopy) (Variables|Default|GetDropChance) (Math|Conversions|ToInteger(Byte) (Variables|/Game/Dante/Blueprint/BP_DantePawn.BP_DantePawn_C|GetMovementType _as_bp_dante_pawn))))
    (Development|PrintString "ItemDropped")
    (Physics|SetSimulatePhysics _staticmesh true)
    (Physics|AddImpulseatLocation _staticmesh (* (.location (Class|KismetAnimationLibrary|Lookat (Transformation|GetActorTransform _as_bp_dante_pawn) (Transformation|GetActorLocation) "1.000000,0.000000,0.000000" false "0.000000,0.000000,1.000000" 0.0)) 2.0) (Transformation|GetWorldLocation (Variables|Default|GetArrow)) "None")
    (else
      (Development|PrintString "Phew"))))

(event OnComponentHit(StaticMesh)
  (params (HitComponent :type Primitive%20Component%20Object%20Reference) (OtherActor :type Actor%20Object%20Reference) (OtherComp :type Primitive%20Component%20Object%20Reference) (NormalImpulse :type Vector :default "0, 0, 0") (Hit :type Hit%20Result%20Structure%20%28by%20ref%29))
  (if (not (Variables|Default|GetSoundEmitted))
    (if (Actor|ActorHasTag OtherActor "Floor")
      (Variables|Default|SetSoundEmitted true)
      (Class|AISenseHearing|ReportNoiseEvent (.Location (Collision|BreakHitResult Hit)) 1.0 self (Variables|Default|GetNoiseMaxRange) "None"))))

(event EventBeginPlay
  (bind _asbp_dante_pawn (Utilities|Casting|CastToBP_DantePawn (Game|Player|GetPlayerPawn 0)))
  (Variables|Default|SetAs%20BP%20Dante%20Pawn _asbp_dante_pawn)
  (Utilities|FlowControl|Delay 5.0)
  (Class|AISenseHearing|ReportNoiseEvent "1980.000000,1084.000000,97.000000" 1.0 self 0.0 "None")
  (Development|PrintString "NOISE!"))

(event EventTick
  (params (DeltaSeconds :type Float%20%28single-precision%29)))

(fn ConstructionScript)