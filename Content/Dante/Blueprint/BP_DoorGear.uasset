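; BP_DoorGear is a lettered, rotatable gear that forms part of a combination door puzzle.
; On BeginPlay it displays its letter and snaps its mesh to a random one of eight 45-degree pitch positions.
; Each Interact advances it one step with wraparound, updates its Correct flag against CorrectRotation, and tells every BP_CombinationDoor in the level to run CheckGears.
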(event EventBeginPlay
  (|CallParentFunction)
  (Rendering|Components|TextRender|SetText (Variables|Default|GetText) (Variables|Default|GetLetter))
  (bind _output_get (Variables|Default|SetRotationIndex (Math|Random|RandomIntegerinRange 0 7)))
  (Transformation|SetRelativeRotation (Variables|Default|GetStaticMesh) (Math|Rotator|MakeRotator 0.0 (* _output_get 45.0) 0.0) false false))

(event Collision|EventActorBeginOverlap
  (params (OtherActor :type Actor%20Object%20Reference))
  (|CallParentFunction OtherActor) ; This node is disabled and will not be called.\nDrag off pins to build functionality.
)

(event EventTick
  (params (DeltaSeconds :type Float%20%28single-precision%29))
  (|CallParentFunction DeltaSeconds) ; This node is disabled and will not be called.\nDrag off pins to build functionality.
)

(event EventInteract
  (Math|Integer|IncrementInt (Variables|Default|GetRotationIndex)
    (:%20%20
      (if (> (Variables|Default|GetRotationIndex) 7)
        (bind _output_get (Variables|Default|SetRotationIndex 0)))
      (Transformation|SetRelativeRotation (Variables|Default|GetStaticMesh) (Math|Rotator|MakeRotator 0.0 (* _output_get 45.0) 0.0) false false)
      (Variables|Default|SetCorrect (== (Variables|Default|GetCorrectRotation) (Variables|Default|GetRotationIndex)))
      (bind _outactors (Actor|GetAllActorsOfClass "/Game/Dante/Blueprint/BP_CombinationDoor.BP_CombinationDoor_C"))
      (for _array_element _outactors
        (Default|CheckGears _array_element)))))

(fn ConstructionScript
  (|CallParentFunction))