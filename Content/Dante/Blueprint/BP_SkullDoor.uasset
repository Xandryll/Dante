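; BP_SkullDoor is a door that opens once enough coins have been added to it.
; On BeginPlay it creates a dynamic eye material for its static mesh.
; Each CoinAdded call increments an activated-statue counter.
; When the count equals CoinsAmount, the Cube drops by a relative offset and the eye material switches to a bright green glow.
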(event Custom|CoinAdded
  (bind _materialinstance (Variables|Default|GetMaterialInstance))
  (bind _result (Math|Integer|IncrementInt (Variables|Default|GetActivatedStatues))
    (:%20%20
      (if (== _result (Variables|Default|GetCoinsAmount))
        (Transformation|AddRelativeLocation (Variables|Default|GetCube) "0.000000,0.000000,-200.000000" false false)
        (Rendering|Material|SetScalarParameterValue _materialinstance "EmissivePower" 1e+01 :!class /Script/Engine.MaterialInstanceDynamic)
        (Rendering|Material|SetVectorParameterValue _materialinstance "Color" "(R=0.131763,G=1.000000,B=0.000000,A=1.000000)" :!class /Script/Engine.MaterialInstanceDynamic)))))

(event EventBeginPlay
  (bind _staticmesh (Variables|Default|GetStaticMesh))
  (|CallParentFunction)
  (bind _returnvalue (Rendering|Material|CreateDynamicMaterialInstance _staticmesh 0 "/Game/Dante/Meshes/MI_Eyes.MI_Eyes" "None" :!class /Script/Engine.PrimitiveComponent))
  (bind _output_get (Variables|Default|SetMaterialInstance _returnvalue))
  (Rendering|Material|SetMaterial _staticmesh 0 _output_get))

(event Collision|EventActorBeginOverlap
  (params (OtherActor :type Actor%20Object%20Reference)))

(event EventTick
  (params (DeltaSeconds :type Float%20%28single-precision%29)))

(fn ConstructionScript
  (|CallParentFunction))