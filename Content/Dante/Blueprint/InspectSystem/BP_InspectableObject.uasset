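; BP_InspectableObject is an inspectable jewel box puzzle with a secret compartment, driven by an ActivateArea event that switches on the selected area.
; Area A shifts a cylinder and the box cube, then disables its own collision and enables B's, chaining the steps.
; Area B slides the cube further to reveal the compartment and disables itself, while C only describes the Alighieri insignia.
; Each area shows dialogue through the Room's InspectHUD.
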(event Custom|Activate%20Area
  (params (Selection :type String))
  (bind _room (Variables|Default|GetRoom))
  (bind _inspecthud (Variables|/Game/Dante/Blueprint/InspectSystem/BP_InspectRoom.BP_InspectRoom_C|GetInspectHUD _room))
  (switch string Selection
    (:A
      (Transformation|AddLocalOffset (Variables|Default|GetCylinder3) "0.000000,0.000000,5.000000" false false)
      (Collision|SetCollisionEnabled (Variables|Default|GetA) "NoCollision")
      (Transformation|AddLocalOffset (Variables|Default|GetJewelBox_Cube_001) "10.000000,0.000000,0.000000" false false)
      (Collision|SetCollisionEnabled (Variables|Default|GetB) "QueryAndProbe")
      (Default|ShowDialogue _inspecthud "Something clicked inside..."))
    (:B
      (Transformation|AddLocalOffset (Variables|Default|GetJewelBox_Cube_001) "140.000000,0.000000,0.000000" false false)
      (Collision|SetCollisionEnabled (Variables|Default|GetB) "NoCollision")
      (Default|ShowDialogue _inspecthud "A secret compartment ! How clever..."))
    (:C
      (Default|ShowDialogue _inspecthud "This is the Alighieri insignia."))))

(event EventBeginPlay)

(event Collision|EventActorBeginOverlap
  (params (OtherActor :type Actor%20Object%20Reference)))

(event EventTick
  (params (DeltaSeconds :type Float%20%28single-precision%29)))

(fn ConstructionScript)