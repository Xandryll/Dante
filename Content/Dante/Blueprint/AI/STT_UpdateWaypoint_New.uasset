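; StateTree task that advances an enemy's current waypoint index for patrol-style movement.
; On entering the state, it increments the Enemy's CurrentWaypoint, wrapping to zero after the last entry in its Waypoints array.
; It then finishes immediately as succeeded, leaving an unused UpdateWaypoint call disconnected.
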(event EventLatentEnterState
  (params (Transition :type State%20Tree%20Transition%20Result%20Structure%20%28by%20ref%29))
  (bind _enemy (Variables|Default|GetEnemy))
  (if (== (Variables|/Game/Dante/BP_Enemy.BP_Enemy_C|GetCurrentWaypoint _enemy) (Utilities|Array|LastIndex (Variables|/Game/Dante/BP_Enemy.BP_Enemy_C|GetWaypoints _enemy)))
    (Variables|/Game/Dante/BP_Enemy.BP_Enemy_C|SetCurrentWaypoint _enemy 0)
    (else
      (bind _result (Math|Integer|IncrementInt (Variables|/Game/Dante/BP_Enemy.BP_Enemy_C|GetCurrentWaypoint _enemy))
        (:%20%20
          (Variables|/Game/Dante/BP_Enemy.BP_Enemy_C|SetCurrentWaypoint _enemy _result)))))
  (StateTree|FinishTask true))