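; StateTree task that keeps an enemy stunned, blind to sight for its stun duration.
; On state entry it disables the AI sight sense and waits out the delay.
; If the enemy was dived on, it then plays a scream, reports a noise event within its data asset's calling range, and clears that flag.
; Finally it restores sight, clears the stunned flag and finishes successfully.
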(event EventLatentEnterState
  (params (Transition :type State%20Tree%20Transition%20Result%20Structure%20%28by%20ref%29))
  (bind _enemy (Variables|Default|GetEnemy))
  (bind _returnvalue (Transformation|GetActorLocation _enemy))
  (bind _aiperception (Variables|/Game/Dante/BP_Enemy.BP_Enemy_C|GetAIPerception _enemy))
  (Class|AIPerceptionComponent|SetSenseEnabled _aiperception "/Script/AIModule.AISense_Sight" false)
  (Utilities|FlowControl|Delay (Variables|/Game/Dante/BP_Enemy.BP_Enemy_C|GetStunDuration _enemy))
  (if (Variables|/Game/Dante/BP_Enemy.BP_Enemy_C|GetgotDived _enemy)
    (Audio|PlaySoundatLocation "/Game/Dante/Blueprint/Audio/mixkit-male-falling-scream-392_Cue.mixkit-male-falling-scream-392_Cue" _returnvalue "0, 0, 0" 1.0 1.0 0.0 0 0 0 0)
    (Class|AISenseHearing|ReportNoiseEvent _returnvalue 1.0 _enemy (Variables|/Game/Dante/Blueprint/PDAs/PDA_Enemy.PDA_Enemy_C|GetCallingMaxDistance (Variables|/Game/Dante/BP_Enemy.BP_Enemy_C|GetEnemyDA _enemy)) "None")
    (Variables|/Game/Dante/BP_Enemy.BP_Enemy_C|SetgotDived _enemy false))
  (Class|AIPerceptionComponent|SetSenseEnabled _aiperception "/Script/AIModule.AISense_Sight" true)
  (Variables|/Game/Dante/BP_Enemy.BP_Enemy_C|SetisStunned _enemy false)
  (StateTree|FinishTask true))