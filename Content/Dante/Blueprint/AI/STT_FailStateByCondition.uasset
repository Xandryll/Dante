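; StateTree task that fails its state when selected conditions on the AI Enemy are met.
; Each latent tick runs flag-gated checks on opponent count, stun and a valid target audio actor for investigation, calling FinishTask as failed on a match.
; The same AbortByOpponents0 flag gates both the above-zero and equals-zero opponent checks, so enabling it fails the task in either case.
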(event EventLatentTick
  (params (DeltaTime :type Float%20%28single-precision%29))
  (Utilities|FlowControl|Sequence
    (:then_0
      (if (Variables|Default|GetAbortByOpponents>0)
        (if (> (Variables|/Game/Dante/BP_Enemy.BP_Enemy_C|GetOpponentsAmount (Variables|Input|GetEnemy)) 0)
          (StateTree|FinishTask false))))
    (:then_1
      (if (Variables|Default|GetAbortByOpponents=0)
        (if (== (Variables|/Game/Dante/BP_Enemy.BP_Enemy_C|GetOpponentsAmount (Variables|Input|GetEnemy)) 0)
          (StateTree|FinishTask false))))
    (:then_2
      (if (Variables|Default|GetAbortByStun)
        (if (Variables|/Game/Dante/BP_Enemy.BP_Enemy_C|GetisStunned (Variables|Input|GetEnemy))
          (StateTree|FinishTask false))))
    (:then_3
      (if (Variables|Default|GetAbortByInvestigate)
        (if (Utilities|IsValid (Variables|/Game/Dante/BP_Enemy.BP_Enemy_C|GetTargetAudioActor (Variables|Input|GetEnemy)))
          (StateTree|FinishTask false))))))