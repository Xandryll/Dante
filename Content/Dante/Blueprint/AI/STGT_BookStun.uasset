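; StateTree task that stuns an Enemy while Dante's book is active and the player is nearby.
; On state entry it caches the player pawn as BP_DantePawn.
; Each tick with BookActive true, it sets the enemy's IsStunned from a fixed distance check between enemy and player.
; IsStunned is left unchanged while the book is inactive, so this task does not clear a stun then.
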(event EventLatentTick
  (params (DeltaTime :type Float%20%28single-precision%29))
  (bind _enemy (Variables|Input|GetEnemy))
  (bind _as_bp_dante_pawn (Variables|Default|GetAs%20BP%20Dante%20Pawn))
  (if (Variables|/Game/Dante/Blueprint/BP_DantePawn.BP_DantePawn_C|GetBookActive _as_bp_dante_pawn)
    (if (< (Math|Vector|Distance(Vector) (Transformation|GetActorLocation _enemy) (Transformation|GetActorLocation _as_bp_dante_pawn)) 1.5e+03)
      (Variables|/Game/Dante/BP_Enemy.BP_Enemy_C|SetisStunned _enemy true)
      (else
        (Variables|/Game/Dante/BP_Enemy.BP_Enemy_C|SetisStunned _enemy false)))))

(event EventLatentEnterState
  (params (Transition :type State%20Tree%20Transition%20Result%20Structure%20%28by%20ref%29))
  (bind _asbp_dante_pawn (Utilities|Casting|CastToBP_DantePawn (Game|Player|GetPlayerPawn 0)))
  (Variables|Default|SetAs%20BP%20Dante%20Pawn _asbp_dante_pawn))