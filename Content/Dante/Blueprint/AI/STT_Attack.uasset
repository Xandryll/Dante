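; StateTree task that carries out an enemy's attack on its target when the state is entered.
; Enemy targets and Killer-type attackers send an attack message to the target, then drop it from AI perception's lost targets.
; Against other targets, Divers send a force-dive message instead, falling back to a plain attack when the game mode's dive level is the last one.
; Each of these branches finishes the task as succeeded.
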(event EventLatentEnterState
  (params (Transition :type State%20Tree%20Transition%20Result%20Structure%20%28by%20ref%29))
  (bind _enemy (Variables|Input|GetEnemy))
  (bind _enemy_2 (Variables|Input|GetEnemy))
  (bind _targetactor (Variables|/Game/Dante/BP_Enemy.BP_Enemy_C|GetTargetActor _enemy))
  (bind _as_bp_dante_game_mode (Variables|/Game/Dante/BP_Enemy.BP_Enemy_C|GetAs%20BP%20Dante%20Game%20Mode _enemy_2))
  (if (== (Utilities|GetClass (Variables|/Game/Dante/BP_Enemy.BP_Enemy_C|GetTargetActor _enemy_2)) "/Game/Dante/BP_Enemy.BP_Enemy_C")
    (Class|BPIDante|AttackTarget(Message) _targetactor :!label _label)
    (Default|AIPerceptionRemoveLostTargets _enemy_2 _targetactor)
    (else
      (switch Utilities|FlowControl|Switch|SwitchonEn_EnemyType (Variables|/Game/Dante/Blueprint/PDA_Enemy.PDA_Enemy_C|GetEnemyType (Variables|/Game/Dante/BP_Enemy.BP_Enemy_C|GetEnemyDA _enemy_2))
        (:NewEnumerator0
          (goto _label))
        (:NewEnumerator1
          (if (== (Variables|/Game/Dante/Blueprint/BP_DanteGameMode.BP_DanteGameMode_C|GetDive_Level _as_bp_dante_game_mode) (Utilities|Array|LastIndex (Variables|/Game/Dante/Blueprint/BP_DanteGameMode.BP_DanteGameMode_C|GetLevels _as_bp_dante_game_mode)))
            (Class|BPIDante|AttackTarget(Message) _targetactor)
            (Development|PrintString "Last level")
            (else
              (Class|BPIDante|ForceDive(Message) _targetactor _enemy)
              (Development|PrintString "Force dive")))))))
  (StateTree|FinishTask true))