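; BP_HidingPlace is a possessable hiding spot that lets the Dante player hide from AI.
; Box overlap shows or clears the pawn's interaction prompt, and Interact moves possession from Dante to the hiding place.
; If Dante is unspotted, entering also unregisters its perception stimuli and teleports it to a safe zone.
; Pressing F teleports Dante to the exit, repossesses it and re-registers perception; ForceDive is an empty stub.
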(event OnComponentEndOverlap(Box)
  (params (OverlappedComponent :type Primitive%20Component%20Object%20Reference) (OtherActor :type Actor%20Object%20Reference) (OtherComp :type Primitive%20Component%20Object%20Reference) (OtherBodyIndex :type Integer))
  (bind _as_bp_dante_pawn (Variables|Default|GetAs%20BP%20Dante%20Pawn))
  ;[1 1 1] Show Interaction Logic
  ;[1 1 1] Overlap system
  (if (== OtherActor _as_bp_dante_pawn)
    (Default|ObjectOutOfRange _as_bp_dante_pawn)))

(event OnComponentBeginOverlap(Box)
  (params (OverlappedComponent :type Primitive%20Component%20Object%20Reference) (OtherActor :type Actor%20Object%20Reference) (OtherComp :type Primitive%20Component%20Object%20Reference) (OtherBodyIndex :type Integer) (bFromSweep :type Boolean) (SweepResult :type Hit%20Result%20Structure%20%28by%20ref%29))
  (bind _as_bp_dante_pawn (Variables|Default|GetAs%20BP%20Dante%20Pawn))
  (bind _pda_item (Variables|Default|GetPDA_Item))
  ;[1 1 1] Show Interaction Logic
  ;[1 1 1] Overlap system
  (if (== OtherActor _as_bp_dante_pawn)
    (Default|ObjectinRange _as_bp_dante_pawn self (Variables|/Game/Dante/Blueprint/PDAs/PDA_Items.PDA_Items_C|GetInteractionString _pda_item) (Variables|/Game/Dante/Blueprint/PDAs/PDA_Items.PDA_Items_C|GetName _pda_item))))

(event EventBeginPlay
  ;[1 1 1] Initialize
  (bind _asbp_dante_pawn (Utilities|Casting|CastToBP_DantePawn (Game|Player|GetPlayerPawn 0)))
  (Variables|Default|SetAs%20BP%20Dante%20Pawn _asbp_dante_pawn))

(event EventInteract
  (bind _returnvalue (Game|GetPlayerController 0))
  (bind _self self)
  (bind _as_bp_dante_pawn (Variables|Default|GetAs%20BP%20Dante%20Pawn))
  ;[0 0.6928 1] Interaction Logic
  ;;[1 1 1] Enter Hiding Place
  (Variables|/Game/Dante/Blueprint/BP_DantePawn.BP_DantePawn_C|SetIsHiding _as_bp_dante_pawn true)
  (Pawn|UnPossess _returnvalue)
  (Pawn|Possess _returnvalue _self)
  (Variables|/Game/Dante/Blueprint/BP_DantePawn.BP_DantePawn_C|SetTemporaryPawn _as_bp_dante_pawn _self)
  (if (not (Variables|/Game/Dante/Blueprint/BP_DantePawn.BP_DantePawn_C|GetisSpotted _as_bp_dante_pawn))
    (Class|AIPerceptionStimuliSourceComponent|UnregisterfromPerceptionSystem (Variables|/Game/Dante/Blueprint/BP_DantePawn.BP_DantePawn_C|GetAIPerceptionStimuliSource _as_bp_dante_pawn))
    (Default|TeleporttoSafeZone _as_bp_dante_pawn)))

(event Input|KeyboardEvents|F
  (params (Key :type Key%20Structure :default "None"))
  (bind _returnvalue (Game|GetPlayerController 0))
  (bind _as_bp_dante_pawn (Variables|Default|GetAs%20BP%20Dante%20Pawn))
  ;[0 0.6928 1] Interaction Logic
  ;;[1 1 1] Exit Hiding Place
  (:Pressed
    (Variables|/Game/Dante/Blueprint/BP_DantePawn.BP_DantePawn_C|SetIsHiding _as_bp_dante_pawn false)
    (Pawn|UnPossess _returnvalue)
    (Transformation|Teleport _as_bp_dante_pawn (Transformation|GetWorldLocation (Variables|Default|GetExitDirection)) (Transformation|GetWorldRotation (Variables|Default|GetDefaultSceneRoot)))
    (Pawn|Possess _returnvalue _as_bp_dante_pawn)
    (Class|AIPerceptionStimuliSourceComponent|RegisterwithPerceptionSystem (Variables|/Game/Dante/Blueprint/BP_DantePawn.BP_DantePawn_C|GetAIPerceptionStimuliSource _as_bp_dante_pawn))))

(fn ConstructionScript)

(fn ForceDive
  (params (Enemy :type BP%20Enemy%20Object%20Reference))
  (return))