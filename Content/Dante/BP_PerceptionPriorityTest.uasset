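; Test Blueprint for AI perception target priority that keeps an ordered list of perceived actors and prints it for debugging.
; Perception updates add unseen actors to TargetActors, putting BP_DantePawn instances at the front and others at the back.
; Actors leave the list only when perception forgets them.
; Tick prints the count, each actor's name and the first entry as the current priority.
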(event OnTargetPerceptionUpdated(AIPerception)
  (params (Actor :type Actor%20Object%20Reference) (Stimulus :type AI%20Stimulus%20Structure))
  (bind _targetactors (Variables|Default|GetTargetActors))
  (if (not (Utilities|Array|ContainsItem _targetactors Actor))
    (if (== (Utilities|GetClass Actor) "/Game/Dante/Blueprint/BP_DantePawn.BP_DantePawn_C")
      (Utilities|Array|Insert _targetactors Actor)
      (else
        (Utilities|Array|Add _targetactors Actor)))))

(event OnTargetPerceptionInfoUpdated(AIPerception)
  (params (UpdateInfo :type Actor%20Perception%20Update%20Info%20Structure%20%28by%20ref%29)))

(event OnTargetPerceptionForgotten(AIPerception)
  (params (Actor :type Actor%20Object%20Reference))
  (Utilities|Array|RemoveItem (Variables|Default|GetTargetActors) Actor))

(event EventBeginPlay)

(event Collision|EventActorBeginOverlap
  (params (OtherActor :type Actor%20Object%20Reference)))

(event EventTick
  (params (DeltaSeconds :type Float%20%28single-precision%29))
  (bind _targetactors (Variables|Default|GetTargetActors))
  (Development|PrintString (Utilities|String|Append "ActorsNum: " (Utilities|String|ToString(Integer) (Utilities|Array|Length _targetactors))))
  (for _array_element _targetactors
    (Development|PrintString (Utilities|String|Append "Actor: " (Utilities|GetDisplayName _array_element))))
  (Development|PrintString (Utilities|String|Append "Priority: " (Utilities|GetDisplayName (Utilities|Array|Get(acopy) _targetactors))))
  (Development|PrintString "--------------------"))

(fn ConstructionScript)