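; BP_Talker is a talking character that periodically shows dialogue to the player.
; On BeginPlay it runs the parent logic, sets an inherited-style EnemyState and starts a looping five-second timer.
; Each timer tick calls ShowDialogueMessage on the player pawn with its Name and a Text entry indexed by the Dante game mode's DiveLevel, so lines vary with dive level.
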(event Custom|Speak
  (Class|BPIDante|ShowDialogue(Message) (Game|Player|GetPlayerPawn 0) (Variables|Default|GetName) (Utilities|Array|Get(acopy) (Variables|Default|GetText) (Variables|/Game/Dante/Blueprint/BP_DanteGameMode.BP_DanteGameMode_C|GetDive_Level (Variables|Default|GetAs%20BP%20Dante%20Game%20Mode)))))

(event EventBeginPlay
  (|CallParentFunction)
  (Variables|Default|SetEnemyState "NewEnumerator0")
  (Utilities|Time|SetTimerbyEvent (delegate Custom|Speak) 5.0 true))

(event Collision|EventActorBeginOverlap
  (params (OtherActor :type Actor%20Object%20Reference)))

(event EventTick
  (params (DeltaSeconds :type Float%20%28single-precision%29))
  (|CallParentFunction DeltaSeconds) ; This node is disabled and will not be called.\nDrag off pins to build functionality.
)

(fn ConstructionScript
  (|CallParentFunction))